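; Change_Scene_BP is a trigger volume that loads another level when a Character_Gameplay overlaps its box.
; The overlap calls FadeWidget, waits for the duration it returns, then opens the level named by LevelName.
; FadeWidget contains no fade logic and returns zero, so the delay has no set duration.
; The construction script applies SizeBoxTrigger to the box extent and DebugHiddenCollision to its in-game visibility.
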(event `self.Box.OnComponentBeginOverlap`
  (params (OverlappedComponent :type "PrimitiveComponent Object Reference") (OtherActor :type "Actor Object Reference") (OtherComp :type "PrimitiveComponent Object Reference") (OtherBodyIndex :type Integer) (bFromSweep :type Boolean) (SweepResult :type "HitResult Structure (by ref)"))
  (cast `/Game/Blueprints/Gameplay/Character_Gameplay` OtherActor)
  (bind _delay_fade (`self.FadeWidget`))
  (`KismetSystemLibrary.Delay` _delay_fade)
  (`GameplayStatics.OpenLevel` (`self.Level Name`)))

(fn `FadeWidget`
  (returns (`Delay Fade` :type "Float (double-precision)"))
  (return 0.0))

(fn `UserConstructionScript`
  (`BoxComponent.SetBoxExtent` (`self.Box`) (`self.Size Box Trigger`) true)
  (`SceneComponent.SetHiddenInGame` (`self.Box`) (`self.Debug Hidden Collision`) false))