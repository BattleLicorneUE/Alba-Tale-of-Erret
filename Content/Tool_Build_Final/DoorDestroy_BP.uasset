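; Destructible door actor that shatters when a single hit deals damage at least equal to its Health.
; AnyDamage prints the damage and, if CanDestructible is set and the threshold is met, applies radius damage with impulse to its Destructible component.
; A DoOnce then spawns a smoke effect and sound, and destroys the actor after a short delay.
; Health is never decremented, so weaker hits do not accumulate.
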(event `self.ReceiveAnyDamage`
  (params (Damage :type "Float (single-precision)") (DamageType :type "DamageType Object Reference") (InstigatedBy :type "Controller Object Reference") (DamageCauser :type "Actor Object Reference"))
  (bind _returnvalue (`self.K2_GetActorLocation`))
  (`KismetSystemLibrary.PrintString` (`KismetStringLibrary.Conv_DoubleToString` Damage))
  (if (and (`self.Can Destructible`) (>= Damage (`self.Health`)))
    (`DestructibleComponent.ApplyRadiusDamage` (`self.Destructible`) Damage (`self.K2_GetActorLocation` self) 200.0 10000.0 true)
    (`/Engine/EditorBlueprintResources/StandardMacros.DoOnce` false
      (:`Completed`
        (`NiagaraFunctionLibrary.SpawnSystemAtLocation` "/Game/Particles/Systems/VFX_Fumee.VFX_Fumee" _returnvalue)
        (`GameplayStatics.PlaySoundAtLocation` (`self.Sound `) _returnvalue (struct) 1.0 1.0 0.0 null null null)
        (`KismetSystemLibrary.Delay` 2.0)
        (`self.K2_DestroyActor`)))))

(fn `UserConstructionScript`)