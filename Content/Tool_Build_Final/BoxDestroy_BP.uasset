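; BoxDestroy_BP is a breakable box that drops money when damaged.
; If CanDestructible is set, any damage is forwarded to its Destructible component as radius damage with a strong impulse to fracture it.
; A DoOnce limits the reward to the first hit: it spawns Money_BP, a Niagara smoke effect and a sound, then destroys the actor after a short delay.
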(event `self.ReceiveAnyDamage`
  (params (Damage :type "Float (single-precision)") (DamageType :type "DamageType Object Reference") (InstigatedBy :type "Controller Object Reference") (DamageCauser :type "Actor Object Reference"))
  (bind _returnvalue (`self.K2_GetActorLocation`))
  (if (`self.Can Destructible`)
    (`DestructibleComponent.ApplyRadiusDamage` (`self.Destructible`) Damage (`self.K2_GetActorLocation` self) 200.0 10000.0 true)
    (`/Engine/EditorBlueprintResources/StandardMacros.DoOnce` false
      (:`Completed`
        (`|SpawnActorFromClass` "/Game/Blueprints/Gameplay/Actors/Interactables/Money_BP.Money_BP_C" (`KismetMathLibrary.MakeTransform` _returnvalue) "Undefined" "OverrideRootScale" null null)
        (`NiagaraFunctionLibrary.SpawnSystemAtLocation` "/Game/Particles/Systems/VFX_Fumee.VFX_Fumee" _returnvalue)
        (`GameplayStatics.PlaySoundAtLocation` (`self.Sound `) _returnvalue (struct) 1.0 1.0 0.0 null null null)
        (`KismetSystemLibrary.Delay` 2.0)
        (`self.K2_DestroyActor`)))))

(fn `UserConstructionScript`)