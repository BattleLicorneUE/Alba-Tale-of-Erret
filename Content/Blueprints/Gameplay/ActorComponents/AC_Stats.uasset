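; Actor component that holds a character's RPG attribute points (Int, For, End, Agi, Cha) and adds or removes them by selection.
; Each change writes back into the Stats struct, with removal blocked at zero.
; End and Agi changes also shift the owning Character_Master's health and stamina components, moving max and current by a fixed step and flooring both on decrease.
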(fn `AddStatPoint`
  (params (Selection :type "/Game/Blueprints/Gameplay/Datas/E_StatsNames Enum" :default "NewEnumerator0"))
  (bind _stats (`self.Stats`))
  (bind (_stats_name _stats_int _stats_for _stats_end _stats_agi _stats_cha) (break `/Game/Blueprints/Gameplay/Stat_struct` (`self.Stats`)))
  (switch `/Game/Blueprints/Gameplay/Datas/E_StatsNames` Selection
    (:`NewEnumerator0`
      (bind _result (`/Engine/EditorBlueprintResources/StandardMacros.IncrementInt` _stats_int)
        (:`  `
          (setmembers `/Game/Blueprints/Gameplay/Stat_struct` :`StructRef` _stats :`Int` _result))))
    (:`NewEnumerator1`
      (bind _result_2 (`/Engine/EditorBlueprintResources/StandardMacros.IncrementInt` _stats_for)
        (:`  `
          (setmembers `/Game/Blueprints/Gameplay/Stat_struct` :`StructRef` _stats :`For` _result_2))))
    (:`NewEnumerator2`
      (bind _result_3 (`/Engine/EditorBlueprintResources/StandardMacros.IncrementInt` _stats_end)
        (:`  `
          (setmembers `/Game/Blueprints/Gameplay/Stat_struct` :`StructRef` _stats :`End` _result_3)
          (`self.UpdateHealth` false))))
    (:`NewEnumerator3`
      (bind _result_4 (`/Engine/EditorBlueprintResources/StandardMacros.IncrementInt` _stats_agi)
        (:`  `
          (setmembers `/Game/Blueprints/Gameplay/Stat_struct` :`StructRef` _stats :`Agi` _result_4)
          (`self.UpdateStamina` false))))
    (:`NewEnumerator4`
      (bind _result_5 (`/Engine/EditorBlueprintResources/StandardMacros.IncrementInt` _stats_cha)
        (:`  `
          (setmembers `/Game/Blueprints/Gameplay/Stat_struct` :`StructRef` _stats :`Cha` _result_5))))))

(fn `RemoveStatPoint`
  (params (Selection :type "/Game/Blueprints/Gameplay/Datas/E_StatsNames Enum" :default "NewEnumerator0"))
  (bind (_stats_name _stats_int _stats_for _stats_end _stats_agi _stats_cha) (break `/Game/Blueprints/Gameplay/Stat_struct` (`self.Stats`)))
  (bind _stats (`self.Stats`))
  (switch `/Game/Blueprints/Gameplay/Datas/E_StatsNames` Selection
    (:`NewEnumerator0`
      ;[1 1 1] Int
      (if (not (<= _stats_int 0))
        (bind _result (`/Engine/EditorBlueprintResources/StandardMacros.DecrementInt` _stats_int)
          (:`  `
            (setmembers `/Game/Blueprints/Gameplay/Stat_struct` :`StructRef` _stats :`Int` (`KismetMathLibrary.Clamp` _result 0 99999))))))
    (:`NewEnumerator1`
      ;[1 1 1] For
      (if (not (<= _stats_for 0))
        (bind _result_2 (`/Engine/EditorBlueprintResources/StandardMacros.DecrementInt` _stats_for)
          (:`  `
            (setmembers `/Game/Blueprints/Gameplay/Stat_struct` :`StructRef` _stats :`For` (`KismetMathLibrary.Clamp` _result_2 0 99999))))))
    (:`NewEnumerator2`
      ;[1 1 1] End
      (if (not (<= _stats_end 0))
        (bind _result_3 (`/Engine/EditorBlueprintResources/StandardMacros.DecrementInt` _stats_end)
          (:`  `
            (setmembers `/Game/Blueprints/Gameplay/Stat_struct` :`StructRef` _stats :`End` (`KismetMathLibrary.Clamp` _result_3 0 99999))
            (`self.UpdateHealth` true)))))
    (:`NewEnumerator3`
      ;[1 1 1] Agi
      (if (not (<= _stats_agi 0))
        (bind _result_4 (`/Engine/EditorBlueprintResources/StandardMacros.DecrementInt` _stats_agi)
          (:`  `
            (setmembers `/Game/Blueprints/Gameplay/Stat_struct` :`StructRef` _stats :`Agi` (`KismetMathLibrary.Clamp` _result_4 0 99999))
            (`self.UpdateStamina` true)))))
    (:`NewEnumerator4`
      ;[1 1 1] Cha
      (if (not (<= _stats_cha 0))
        (bind _result_5 (`/Engine/EditorBlueprintResources/StandardMacros.DecrementInt` _stats_cha)
          (:`  `
            (setmembers `/Game/Blueprints/Gameplay/Stat_struct` :`StructRef` _stats :`Cha` (`KismetMathLibrary.Clamp` _result_5 0 99999))))))))

(fn `UpdateHealth`
  (params (`Negatif?` :type Boolean))
  (bind _returnvalue (`self.GetOwner`))
  (if `Negatif?`
    (bind _ascharacter_master (cast `/Game/Blueprints/Gameplay/Character_Master` _returnvalue))
    (bind _ac_health (`/Game/Blueprints/Gameplay/Character_Master.AC_Health` _ascharacter_master))
    (set `/Game/Blueprints/Gameplay/ActorComponents/AC_Health.Health_Max` (`KismetMathLibrary.FClamp` (- (`/Game/Blueprints/Gameplay/ActorComponents/AC_Health.Health_Max` _ac_health) 10.0) 100.0 7.766279436516721e+18) _ac_health)
    (set `/Game/Blueprints/Gameplay/ActorComponents/AC_Health.Health_Current` (`KismetMathLibrary.FClamp` (- (`/Game/Blueprints/Gameplay/ActorComponents/AC_Health.Health_Current` _ac_health) 10.0) 100.0 7.766279436516721e+18) _ac_health)
    (else
      (bind _ascharacter_master_2 (cast `/Game/Blueprints/Gameplay/Character_Master` _returnvalue))
      (bind _ac_health_2 (`/Game/Blueprints/Gameplay/Character_Master.AC_Health` _ascharacter_master_2))
      (set `/Game/Blueprints/Gameplay/ActorComponents/AC_Health.Health_Max` (+ (`/Game/Blueprints/Gameplay/ActorComponents/AC_Health.Health_Max` _ac_health_2) 10.0) _ac_health_2)
      (set `/Game/Blueprints/Gameplay/ActorComponents/AC_Health.Health_Current` (+ (`/Game/Blueprints/Gameplay/ActorComponents/AC_Health.Health_Current` _ac_health_2) 10.0) _ac_health_2))))

(fn `UpdateStamina`
  (params (`Negatif?` :type Boolean))
  (bind _returnvalue (`self.GetOwner`))
  (if `Negatif?`
    (bind _ascharacter_master (cast `/Game/Blueprints/Gameplay/Character_Master` _returnvalue))
    (bind _ac_stamina (`/Game/Blueprints/Gameplay/Character_Master.AC_Stamina` _ascharacter_master))
    (set `/Game/Blueprints/Gameplay/ActorComponents/AC_Stamina.Stamina_Max` (`KismetMathLibrary.FClamp` (- (`/Game/Blueprints/Gameplay/ActorComponents/AC_Stamina.Stamina_Max` _ac_stamina) 10.0) 100.0 7.766279436516721e+18) _ac_stamina)
    (set `/Game/Blueprints/Gameplay/ActorComponents/AC_Stamina.Stamina_Current` (`KismetMathLibrary.FClamp` (- (`/Game/Blueprints/Gameplay/ActorComponents/AC_Stamina.Stamina_Current` _ac_stamina) 10.0) 100.0 7.766279436516721e+18) _ac_stamina)
    (else
      (bind _ascharacter_master_2 (cast `/Game/Blueprints/Gameplay/Character_Master` _returnvalue))
      (bind _ac_stamina_2 (`/Game/Blueprints/Gameplay/Character_Master.AC_Stamina` _ascharacter_master_2))
      (set `/Game/Blueprints/Gameplay/ActorComponents/AC_Stamina.Stamina_Max` (+ (`/Game/Blueprints/Gameplay/ActorComponents/AC_Stamina.Stamina_Max` _ac_stamina_2) 10.0) _ac_stamina_2)
      (set `/Game/Blueprints/Gameplay/ActorComponents/AC_Stamina.Stamina_Current` (+ (`/Game/Blueprints/Gameplay/ActorComponents/AC_Stamina.Stamina_Current` _ac_stamina_2) 10.0) _ac_stamina_2))))