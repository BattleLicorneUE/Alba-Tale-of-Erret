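; Actor component that tracks the owning gameplay character's current element (Fire, Water, Metal or Air) for skill-set switching.
; Four switch events set the element, then share a path that colors the character's switch VFX to match and refreshes it.
; A flag and delay throttle that VFX update, though the element itself still changes during the cooldown.
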(event `SwitchToWater`
  (bind _ascharacter_gameplay (cast `/Game/Blueprints/Gameplay/Character_Gameplay` (`self.GetOwner`) :!pure true))
  (set `self.CurrentElement` "NewEnumerator1")
  (if (not (`self.bChangingSkillSet`)) :!label _label
    (set `self.bChangingSkillSet` true)
    (switch `/Game/Blueprints/Gameplay/Datas/E_ElementTypes` (`self.CurrentElement`)
      (:`NewEnumerator0`
        (set `/Game/Blueprints/Gameplay/Character_Gameplay.Color VFX Switch Element` (struct :`R` 1.0 :`B` 0.006586 :`A` 1.0) _ascharacter_gameplay))
      (:`NewEnumerator1`
        (set `/Game/Blueprints/Gameplay/Character_Gameplay.Color VFX Switch Element` (struct :`R` 0.05725 :`B` 1.0 :`A` 1.0) _ascharacter_gameplay))
      (:`NewEnumerator2`
        (set `/Game/Blueprints/Gameplay/Character_Gameplay.Color VFX Switch Element` (struct :`R` 0.677083 :`G` 0.677083 :`B` 0.677083 :`A` 1.0) _ascharacter_gameplay))
      (:`NewEnumerator3`
        (set `/Game/Blueprints/Gameplay/Character_Gameplay.Color VFX Switch Element` (struct :`R` 0.307292 :`G` 1.0 :`B` 0.494847 :`A` 1.0) _ascharacter_gameplay)))
    (`/Game/Blueprints/Gameplay/Character_Gameplay.UpdateVFX_SwitchElement` _ascharacter_gameplay)
    (`KismetSystemLibrary.Delay` 1.5)
    (set `self.bChangingSkillSet` false)))

(event `SwitchToFire`
  (set `self.CurrentElement` "NewEnumerator0")
  (goto _label))

(event `SwitchToMetal`
  (set `self.CurrentElement` "NewEnumerator2")
  (goto _label))

(event `SwitchToAir`
  (set `self.CurrentElement` "NewEnumerator3")
  (goto _label))