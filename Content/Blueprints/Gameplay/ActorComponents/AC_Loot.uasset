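; Actor component for enemy characters that rolls and spawns loot drops when DropAll is called.
; DropAll walks every DataTable row, and each of the four rarity branches runs the same random-selection macro on that row's LootDrop array.
; Class and drop rate come from separate random indices, so they can mismatch.
; DropObject rolls that rate scaled by TauxChancePlayer, spawning at a random point inside the enemy's Box.
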(event `self.ReceiveBeginPlay`
  (bind _ascharacter_gameplay_child_enemy (cast `/Game/Blueprints/Gameplay/AI/Character_Gameplay_Child_Enemy` (`self.GetOwner`)))
  (set `self.Enemy` _ascharacter_gameplay_child_enemy))

(event `Drop All`
  (bind _data_table (`self.Data Table`))
  (bind _outrownames (`DataTableFunctionLibrary.GetDataTableRowNames` _data_table))
  (for _array_element _outrownames
    (bind _returnvalue (`|GetDataTableRow` _data_table _array_element)
      (:`then`
        (bind (`_typederareté` _lootdrop) (break `/Game/Blueprints/Gameplay/Actors/Other/Struct_Loot` _returnvalue))
        (set `self.Loot Drop` _lootdrop)
        (switch `/Game/Blueprints/Gameplay/Actors/Other/Type_Rareté` `_typederareté`
          (:`NewEnumerator0`
            (`self.RandomLootSeleted`))
          (:`NewEnumerator1`
            (`self.RandomLootSeleted`))
          (:`NewEnumerator2`
            (`self.RandomLootSeleted`))
          (:`NewEnumerator3`
            (`self.RandomLootSeleted`)))))))

(fn `DropObject`
  (bind _box (`/Game/Blueprints/Gameplay/AI/Character_Gameplay_Child_Enemy.Box` (`self.Enemy`)))
  (if (<= (`KismetMathLibrary.RandomFloat`) (/ (* (`self.Taux Drop `) (`self.Taux Chance Player`)) 100.0))
    (`|SpawnActorFromClass` (`self.Class Drop`) (`KismetMathLibrary.MakeTransform` (`KismetMathLibrary.RandomPointInBoundingBox` (`SceneComponent.K2_GetComponentLocation` _box) (`BoxComponent.GetScaledBoxExtent` _box))) "AlwaysSpawn" "OverrideRootScale" null null)))