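; Health component for a Character owner that handles damage, regeneration and a death flag.
; On BeginPlay it fills current and maximum health from the default and starts a looping one-second regeneration timer.
; Each hit lowers current health and also shrinks the regeneration cap by a separate amount, down to a minimum.
; Death is flagged at zero health, but regeneration does not check that flag.
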(event `self.ReceiveBeginPlay`
  (bind _ascharacter (cast `Character` (`self.GetOwner`)))
  (set `self.Owner` _ascharacter)
  (`self.INIT Health`)
  (`KismetSystemLibrary.K2_SetTimer` null "Regene Health" 1.0 true))

(fn `Apply Damage Simple`
  (params (Damage :type "Float (double-precision)"))
  (set `self.Health_Current` (`KismetMathLibrary.FClamp` (- (`self.Health_Current`) Damage) 0.0 (`self.Health_Default`)))
  (set `self.Health_Max` (`KismetMathLibrary.FClamp` (- (`self.Health_Max`) (`self.Health_Consume`)) (`self.Health_Min`) (`self.Health_Default`)))
  (if (<= (`self.Health_Current`) 0.0)
    (set `self.Death` true)))

(fn `INIT Health`
  (bind _health_default (`self.Health_Default`))
  (set `self.Health_Current` _health_default)
  (set `self.Health_Max` _health_default))

(fn `Regene Health`
  (if (< (`self.Health_Current`) (`self.Health_Max`))
    (set `self.Health_Current` (`KismetMathLibrary.FClamp` (+ (`self.Health_Current`) (`self.Health / S`)) 0.0 (`self.Health_Max`)))))