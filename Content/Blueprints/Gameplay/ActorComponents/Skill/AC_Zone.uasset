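; Player skill component for an aimed zone attack that costs stamina.
; Holding the input opens a Tick gate that, while stamina suffices, predicts a projectile arc from the eye view and places an aim decal on the impact, with two debug radius spheres.
; Controller yaw drives the character while aiming.
; Release closes the gate, spends stamina and spawns AC_Skill_Zone with the impact point, then hides the decal after a short delay.
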(event `self.ReceiveBeginPlay`
  (bind _ascharacter_gameplay (cast `/Game/Blueprints/Gameplay/Character_Gameplay` (`GameplayStatics.GetPlayerCharacter` 0)))
  (set `self.Owner` _ascharacter_gameplay)
  (bind _returnvalue (`NiagaraFunctionLibrary.SpawnSystemAtLocation` "/Game/Particles/Systems/Systems_SwitchElements/VFX_Decal_Aim.VFX_Decal_Aim" (`Actor.K2_GetActorLocation` (`self.Owner`)) (struct) (1.0 1.0 1.0) false false "None" false))
  (set `self.VFX Decal` _returnvalue))

(event `self.ReceiveTick`
  (params (DeltaSeconds :type "Float (single-precision)"))
  (`/Engine/EditorBlueprintResources/StandardMacros.Gate` true :!label _label
    (:`Exit`
      (bind _returnvalue (`/Game/Blueprints/Gameplay/ActorComponents/Players/AC_Stamina.Check Stamina` (`/Game/Blueprints/Gameplay/Character_Master.AC_Stamina` (`self.Owner`)) (`self.Consume Stamina`)))
      (if _returnvalue
        (`self.Raycast`)
        (else
          (`self.SetActive` (`self.VFX Decal`) false false))))))

(event `Pressed`
  (`self.SetActive` (`self.VFX Decal`) true false)
  (set `Pawn.bUseControllerRotationYaw` true (`self.Owner`))
  (`GameplayStatics.PlaySound2D` "/Game/Sounds/SFX/BombAttack/Bomb_Attack_Throw.Bomb_Attack_Throw" 1.0 1.0 0.0 null null)
  (goto _label :!via `Open`))

(event `Released`
  (bind (_returnvalue2 _returnvalue _owner) (`self.SpawnActorOffSet`))
  (set `Pawn.bUseControllerRotationYaw` false (`self.Owner`))
  (`|ExecutionSequence`
    (:`then_0`
      (goto _label :!via `Close`))
    (:`then_1`
      (bind _returnvalue_2 (`/Game/Blueprints/Gameplay/ActorComponents/Players/AC_Stamina.Use Stamina` (`/Game/Blueprints/Gameplay/Character_Master.AC_Stamina` (`self.Owner`)) (`self.Consume Stamina`)))
      (if _returnvalue_2
        (`GameplayStatics.PlaySoundAtLocation` "/Game/Sounds/SFX/BombAttack/Bomb_Attack_Spawner.Bomb_Attack_Spawner" (`Actor.K2_GetActorLocation` (`GameplayStatics.GetPlayerCharacter` 0)) (struct) 1.0 1.0 0.0 null null null)
        (`|SpawnActorFromClass` "/Game/Blueprints/Gameplay/Actors/Skills/AC_Skill_Zone.AC_Skill_Zone_C" (`KismetMathLibrary.MakeTransform` _returnvalue2 _returnvalue) "AlwaysSpawn" "OverrideRootScale" null (`self.Point Impact`) _owner)
        (`KismetSystemLibrary.Delay` 0.2)
        (`self.SetActive` (`self.VFX Decal`) false false)
        (else
          (goto _label :!via `Close`))))))

(fn `Raycast`
  (bind _vfx_decal (`self.VFX Decal`))
  (bind (_outlocation _outrotation) (`Actor.GetActorEyesViewPoint` (`self.Owner`)))
  (bind _outhit (`GameplayStatics.Blueprint_PredictProjectilePath_ByObjectType` _outlocation (* (`KismetMathLibrary.GetForwardVector` _outrotation) (`self.Launch Velocity`)) true 30.0 (`|MakeArray` "ObjectTypeQuery1" :!type "EObjectTypeQuery Enum")))
  (bind (_bblockinghit _binitialoverlap _time _distance _location _impactpoint _normal _impactnormal) (`GameplayStatics.BreakHitResult` _outhit))
  (bind _output_get (set `self.Point Impact` _location))
  (`SceneComponent.K2_SetWorldLocation` _vfx_decal _output_get true true)
  (`SceneComponent.K2_SetWorldRotation` _vfx_decal (`KismetMathLibrary.MakeRotFromZX` _impactnormal _impactnormal) true true)
  (`KismetSystemLibrary.DrawDebugSphere` _output_get 200.0 12 (struct :`R` 1.0 :`A` 1.0))
  (`KismetSystemLibrary.DrawDebugSphere` _output_get 400.0 12 (struct :`R` 1.0 :`G` 0.553216 :`A` 1.0)))