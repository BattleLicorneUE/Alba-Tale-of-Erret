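; Actor component for the fist (Poings) melee skill, playing punch combo montages on its owning character.
; Attack cycles through montages, with notifies timing the hit and combo window, and locks input for the player.
; Hits box-trace pawns ahead, dealing randomized damage typed by the player's current element and scaled by the upgrade level read from the HUD.
; Landed hits also restore stamina and trigger sound, force feedback and Niagara impact FX.
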(event `self.ReceiveBeginPlay`
  (bind _ascharacter_master (cast `/Game/Blueprints/Gameplay/Character_Master` (`self.GetOwner`)))
  (set `self.Owner` _ascharacter_master)
  (bind _output_get (set `self.AttackAnimIndexMax` (- (`KismetArrayLibrary.Array_Length` (`self.AttackAnimations`)) 1)))
  (`KismetSystemLibrary.PrintString` (`KismetStringLibrary.Conv_IntToString` _output_get))
  (set `self.HitAnimIndexMax` (`KismetArrayLibrary.Array_LastIndex` (`self.HitAnimations`))))

(event `Attack`
  (bind _attackanimindexcurrent (`self.AttackAnimIndexCurrent`))
  (bind _owner (`self.Owner`))
  (bind _owner_2 (`self.Owner`))
  (set `self.Element` (`/Game/Blueprints/Gameplay/ActorComponents/Players/AC_SkillManager.CurrentElement` (`/Game/Blueprints/Gameplay/Character_Master.AC_SkillManager` (cast `/Game/Blueprints/Gameplay/Character_Gameplay` (`GameplayStatics.GetPlayerCharacter` 0) :!pure true))))
  (if (== _owner_2 (`GameplayStatics.GetPlayerCharacter` 0))
    (set `/Game/Blueprints/Gameplay/Character_Gameplay.InputEnabled?` false (cast `/Game/Blueprints/Gameplay/Character_Gameplay` _owner_2 :!pure true)))
  (if (`self.bCanAttack`)
    (set `self.bCanAttack` false)
    (bind _notifyname (`|PlayMontage` (`Character.Mesh` (`self.Owner`)) (`|GetArrayItem` (`self.AttackAnimations`) (`self.AttackAnimIndexCurrent`)))
      (:`then`
        (set `self.AttackAnimIndexCurrent` (`KismetMathLibrary.SelectInt` (+ _attackanimindexcurrent 1) 0 (< _attackanimindexcurrent (`self.AttackAnimIndexMax`)))))
      (:`OnCompleted`
        (set `self.AttackAnimIndexCurrent` 0)
        (set `self.bCanAttack` true)
        (if (== _owner (`GameplayStatics.GetPlayerCharacter` 0))
          (set `/Game/Blueprints/Gameplay/Character_Gameplay.InputEnabled?` true (cast `/Game/Blueprints/Gameplay/Character_Gameplay` _owner :!pure true))))
      (:`OnInterrupted`
        (`KismetSystemLibrary.Delay` 0.5)
        (set `self.bCanAttack` true)
        (set `/Game/Blueprints/Gameplay/Character_Gameplay.InputEnabled?` true (cast `/Game/Blueprints/Gameplay/Character_Gameplay` (`self.Owner`) :!pure true)))
      (:`OnNotifyBegin`
        (switch `name` _notifyname
          (:`Hit`
            (`self.TriggerSimpleHit`))
          (:`CanCombo`
            (set `self.bCanAttack` true))
          (:`Recovery`
            (set `self.bCanAttack` false)))))))

(fn `Calcul Damage`
  (returns (`Base Damage` :type "Float (double-precision)"))
  (bind _base_damage (`self.Base Damage`))
  (return (* (`KismetMathLibrary.RandomFloatInRange` _base_damage (* _base_damage 1.3)) (`self.Damage Upgrade`))))

(fn `Check Upgrade`
  (switch `int` (`/Game/Blueprints/HUD/Player/Compétence/UpgradeSkill.Niveau Upgrade` (`/Game/Blueprints/HUD/Player/Compétence/Skill_MainPanel.Upgrade_Poings` (`/Game/Blueprints/Gameplay/PlayerController_Gameplay.HUD Skill` (cast `/Game/Blueprints/Gameplay/PlayerController_Gameplay` (`GameplayStatics.GetPlayerController` 0) :!pure true))))
    (:`0`
      (set `self.Damage Upgrade` 1.0))
    (:`1`
      (set `self.Damage Upgrade` 2.0))
    (:`2`
      (set `self.Damage Upgrade` 3.0))
    (:`3`
      (set `self.Damage Upgrade` 4.0)))
  (return))

(fn `TriggerSimpleHit`
  (bind _owner (`self.Owner`))
  (bind _returnvalue (`Actor.K2_GetActorRotation` _owner))
  (bind _returnvalue_2 (`Actor.K2_GetActorLocation` _owner))
  (bind _returnvalue_3 (`KismetMathLibrary.GetForwardVector` _returnvalue))
  (`self.Check Upgrade`)
  (bind (_outhit _returnvalue_4) (`KismetSystemLibrary.BoxTraceSingleForObjects` (+ _returnvalue_2 (* _returnvalue_3 (`self.SpellStartOffset`))) (+ _returnvalue_2 (* _returnvalue_3 (`self.SpellEndOffset`))) (`self.SpellHitSize`) _returnvalue (`|MakeArray` "ObjectTypeQuery3" :!type "EObjectTypeQuery Enum") false (`|MakeArray` (`GameplayStatics.GetPlayerCharacter` 0) :!type "Actor Object Reference")))
  (if _returnvalue_4
    (bind (_bblockinghit _binitialoverlap _time _distance _location _impactpoint _normal _impactnormal _physmat _hitactor) (`GameplayStatics.BreakHitResult` _outhit))
    (`GameplayStatics.ApplyDamage` _hitactor (`self.Calcul Damage`) null null (select `/Game/Blueprints/Gameplay/Datas/E_ElementTypes` (`/Game/Blueprints/Gameplay/ActorComponents/Players/AC_SkillManager.CurrentElement` (`/Game/Blueprints/Gameplay/Character_Master.AC_SkillManager` (`/Game/Blueprints/Gameplay/Library_Blueprints/FunctionLibrary.Get Player character`))) :`NewEnumerator0` "/Game/Blueprints/Gameplay/Datas/DamageTypes/DamageType_Fire.DamageType_Fire_C" :`NewEnumerator1` "/Game/Blueprints/Gameplay/Datas/DamageTypes/DamageType_Water.DamageType_Water_C" :`NewEnumerator2` "/Game/Blueprints/Gameplay/Datas/DamageTypes/DamageType_Metal.DamageType_Metal_C" :`NewEnumerator3` "/Game/Blueprints/Gameplay/Datas/DamageTypes/DamageType_Air.DamageType_Air_C" :!type "DamageType Class Reference"))
    (`GameplayStatics.PlaySoundAtLocation` "/Game/Sounds/SFX/Hits/Hit_Blob.Hit_Blob" _impactpoint (struct) 1.0 1.0 0.0 null null null)
    (`GameplayStatics.SpawnForceFeedbackAtLocation` "/Game/Feelback/Impact.Impact" _impactpoint (struct) false 1.0 0.0 null)
    (`/Game/Blueprints/Gameplay/ActorComponents/Players/AC_Stamina.Add Stamina` (`/Game/Blueprints/Gameplay/Character_Master.AC_Stamina` (`self.Owner`)) (`self.Add Stamina`))
    (switch `/Game/Blueprints/Gameplay/Datas/E_ElementTypes` (`self.Element`)
      (:`NewEnumerator0`
        _)
      (:`NewEnumerator1`
        _)
      (:`NewEnumerator2`
        _)
      (:`NewEnumerator3`
        _))
    (`NiagaraFunctionLibrary.SpawnSystemAtLocation` "/Game/Particles/Systems/FX_Impact.FX_Impact" _impactpoint (`KismetMathLibrary.Conv_VectorToRotator` _impactpoint))))