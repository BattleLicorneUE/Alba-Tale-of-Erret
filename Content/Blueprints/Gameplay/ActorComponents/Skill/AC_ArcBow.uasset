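; Actor component for a character's bow skill, handling cycling attack montages, hit reactions and a timed combo counter.
; Attack shows the bow and plays the next montage, whose notifies fire the shot and open or close the combo window, locking player input meanwhile.
; Despite its name, SpawnArrow is hitscan: it turns on controller yaw rotation and applies fixed damage to the camera raycast's hit actor.
; TakeDamage plays hit montages, blocking further damage until blend-out.
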(event `self.ReceiveBeginPlay`
  (bind _ascharacter_master (cast `/Game/Blueprints/Gameplay/Character_Master` (`self.GetOwner`)))
  (set `self.Owner` _ascharacter_master)
  (bind _output_get (set `self.AttackAnimIndexMax` (- (`KismetArrayLibrary.Array_Length` (`self.AttackAnimations`)) 1)))
  (`KismetSystemLibrary.PrintString` (`KismetStringLibrary.Conv_IntToString` _output_get))
  (set `self.HitAnimIndexMax` (`KismetArrayLibrary.Array_LastIndex` (`self.HitAnimations`))))

(event `Attack`
  (bind _attackanimindexcurrent (`self.AttackAnimIndexCurrent`))
  (bind _owner (`self.Owner`))
  (bind _owner_2 (`self.Owner`))
  (bind _ascharacter_gameplay (cast `/Game/Blueprints/Gameplay/Character_Gameplay` (`self.Owner`) :!pure true))
  (bind _ascharacter_gameplay_2 (cast `/Game/Blueprints/Gameplay/Character_Gameplay` _owner_2 :!pure true))
  (set `self.Element` (`/Game/Blueprints/Gameplay/ActorComponents/Players/AC_SkillManager.CurrentElement` (`/Game/Blueprints/Gameplay/Character_Master.AC_SkillManager` (cast `/Game/Blueprints/Gameplay/Character_Gameplay` (`GameplayStatics.GetPlayerCharacter` 0) :!pure true))))
  (if (== _owner_2 (`GameplayStatics.GetPlayerCharacter` 0))
    (set `/Game/Blueprints/Gameplay/Character_Gameplay.InputEnabled?` false _ascharacter_gameplay_2))
  (if (`self.bCanAttack`)
    (set `self.bCanAttack` false)
    (`/Game/Blueprints/Gameplay/Character_Gameplay.Set visibility Bow` _ascharacter_gameplay_2)
    (bind _notifyname (`|PlayMontage` (`Character.Mesh` (`self.Owner`)) (`|GetArrayItem` (`self.AttackAnimations`) (`self.AttackAnimIndexCurrent`)))
      (:`then`
        (set `self.AttackAnimIndexCurrent` (`KismetMathLibrary.SelectInt` (+ _attackanimindexcurrent 1) 0 (< _attackanimindexcurrent (`self.AttackAnimIndexMax`)))))
      (:`OnCompleted`
        (set `self.AttackAnimIndexCurrent` 0)
        (set `self.bCanAttack` true)
        (if (== _owner (`GameplayStatics.GetPlayerCharacter` 0))
          (set `/Game/Blueprints/Gameplay/Character_Gameplay.InputEnabled?` true (cast `/Game/Blueprints/Gameplay/Character_Gameplay` _owner :!pure true))
          (set `Pawn.bUseControllerRotationYaw` false _ascharacter_gameplay :!label _label)))
      (:`OnInterrupted`
        (`KismetSystemLibrary.Delay` 0.5)
        (set `self.bCanAttack` true)
        (set `/Game/Blueprints/Gameplay/Character_Gameplay.InputEnabled?` true _ascharacter_gameplay)
        (goto _label))
      (:`OnNotifyBegin`
        (switch `name` _notifyname
          (:`Hit`
            (`self.Spawn Arrow`))
          (:`CanCombo`
            (set `self.bCanAttack` true))
          (:`Recovery`
            (set `self.bCanAttack` false)))))))

(event `TakeDamage`
  (bind _hitanimindexcurrent (`self.HitAnimIndexCurrent`))
  (bind _owner (`self.Owner`))
  (if (`Actor.bCanBeDamaged` _owner)
    (set `Actor.bCanBeDamaged` false _owner)
    (`|PlayMontage` (`Character.Mesh` (`self.Owner`)) (`|GetArrayItem` (`self.HitAnimations`) (`self.HitAnimIndexCurrent`))
      (:`then`
        (set `self.HitAnimIndexCurrent` (`KismetMathLibrary.SelectInt` (+ _hitanimindexcurrent 1) 0 (< _hitanimindexcurrent (`self.HitAnimIndexMax`)))))
      (:`OnCompleted`
        (set `self.HitAnimIndexCurrent` 0))
      (:`OnBlendOut`
        (set `Actor.bCanBeDamaged` true _owner)))))

(event `IncrementCombo`
  (`/Engine/EditorBlueprintResources/StandardMacros.IncrementInt` (`self.ComboCount`)
    (:`  `
      (`KismetSystemLibrary.RetriggerableDelay` 2.0)
      (set `self.ComboCount` 0))))

(fn `Spawn Arrow`
  (bind _ascharacter_gameplay (cast `/Game/Blueprints/Gameplay/Character_Gameplay` (`self.Owner`) :!pure true))
  (set `Pawn.bUseControllerRotationYaw` true _ascharacter_gameplay)
  (bind (_returnvalue _hitactor) (`/Game/Blueprints/Gameplay/Character_Gameplay.Raycast to Camera` _ascharacter_gameplay))
  (if _returnvalue
    (`GameplayStatics.ApplyDamage` _hitactor 50.0)))