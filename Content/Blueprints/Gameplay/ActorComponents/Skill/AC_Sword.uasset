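; Sword skill component that runs a character's melee combo attacks, airborne attack and hit reactions.
; Attack cycles montages whose notifies open combo windows and trigger a forward box trace; the jump attack, used while flying, polls for ground to stop.
; Hits apply randomized damage, spawn impact feedback, add stamina and raise a timed combo counter.
; Element branches are empty, and the upgrade multiplier is fixed at base level.
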(event `self.ReceiveBeginPlay`
  (bind _ascharacter_master (cast `/Game/Blueprints/Gameplay/Character_Master` (`self.GetOwner`)))
  (set `self.Owner` _ascharacter_master)
  (set `self.AttackAnimIndexMax` (- (`KismetArrayLibrary.Array_Length` (`self.AttackAnimations`)) 1))
  (set `self.HitAnimIndexMax` (- (`KismetArrayLibrary.Array_Length` (`self.HitAnimations`)) 1)))

(event `Attack`
  (bind _attackanimindexcurrent (`self.AttackAnimIndexCurrent`))
  (bind _owner (`self.Owner`))
  (bind _owner_2 (`self.Owner`))
  (bind _owner_3 (`self.Owner`))
  (set `self.Element` (`/Game/Blueprints/Gameplay/ActorComponents/Players/AC_SkillManager.CurrentElement` (`/Game/Blueprints/Gameplay/Character_Master.AC_SkillManager` (cast `/Game/Blueprints/Gameplay/Character_Gameplay` (`GameplayStatics.GetPlayerCharacter` 0) :!pure true))))
  (`self.Check Upgrade`)
  (`/Game/Blueprints/Gameplay/Character_Gameplay.Show Sword` (cast `/Game/Blueprints/Gameplay/Character_Gameplay` (`self.Owner`) :!pure true))
  (if (== _owner_3 (`GameplayStatics.GetPlayerCharacter` 0))
    (set `/Game/Blueprints/Gameplay/Character_Gameplay.InputEnabled?` false (cast `/Game/Blueprints/Gameplay/Character_Gameplay` _owner_3 :!pure true)))
  (if (`self.bCanAttack`)
    (set `self.bCanAttack` false)
    (if (not (`NavMovementComponent.IsFlying` (`Character.CharacterMovement` (`self.Owner`))))
      (bind _notifyname (`|PlayMontage` (`Character.Mesh` (`self.Owner`)) (`|GetArrayItem` (`self.AttackAnimations`) (`self.AttackAnimIndexCurrent`)))
        (:`then`
          (set `self.AttackAnimIndexCurrent` (`KismetMathLibrary.SelectInt` (+ _attackanimindexcurrent 1) 0 (< _attackanimindexcurrent (`self.AttackAnimIndexMax`)))))
        (:`OnCompleted`
          (set `self.AttackAnimIndexCurrent` 0)
          (set `self.bCanAttack` true)
          (if (== _owner_2 (`GameplayStatics.GetPlayerCharacter` 0))
            (set `/Game/Blueprints/Gameplay/Character_Gameplay.InputEnabled?` true (cast `/Game/Blueprints/Gameplay/Character_Gameplay` _owner_2 :!pure true))))
        (:`OnInterrupted`
          (`KismetSystemLibrary.Delay` 0.5)
          (set `self.bCanAttack` true)
          (set `/Game/Blueprints/Gameplay/Character_Gameplay.InputEnabled?` true (cast `/Game/Blueprints/Gameplay/Character_Gameplay` (`self.Owner`) :!pure true)))
        (:`OnNotifyBegin`
          (switch `name` _notifyname
            (:`Hit`
              (`self.TriggerSimpleHit`))
            (:`CanCombo`
              (set `self.bCanAttack` true))
            (:`Recovery`
              (set `self.bCanAttack` false)))))
      (else
        (bind _notifyname_2 (`|PlayMontage` (`Character.Mesh` (`self.Owner`)) (`self.JumpAttackMontage`))
          (:`then`
            (bind _returnvalue (`KismetSystemLibrary.K2_SetTimerDelegate` (delegate `CheckForGround`) 0.016667 true))
            (set `self.CheckForGroundTimer` _returnvalue))
          (:`OnCompleted`
            (if (== _owner (`GameplayStatics.GetPlayerCharacter` 0))
              (set `/Game/Blueprints/Gameplay/Character_Gameplay.InputEnabled?` true (cast `/Game/Blueprints/Gameplay/Character_Gameplay` _owner :!pure true))))
          (:`OnNotifyBegin`
            (switch `name` _notifyname_2
              (:`Hit`
                (`self.TriggerSimpleHit`))
              (:`CanCombo`
                (set `self.bCanAttack` true)))))))))

(event `CheckForGround`
  (if (`NavMovementComponent.IsMovingOnGround` (`Character.CharacterMovement` (`self.Owner`)))
    (`Character.StopAnimMontage` (`self.Owner`) (`self.JumpAttackMontage`))
    (set `self.bCanAttack` true)
    (`KismetSystemLibrary.K2_ClearAndInvalidateTimerHandle` (`self.CheckForGroundTimer`))))

(event `TakeDamage`
  (bind _hitanimindexcurrent (`self.HitAnimIndexCurrent`))
  (bind _owner (`self.Owner`))
  (if (`Actor.bCanBeDamaged` _owner)
    (set `Actor.bCanBeDamaged` false _owner)
    (`|PlayMontage` (`Character.Mesh` (`self.Owner`)) (`|GetArrayItem` (`self.HitAnimations`) (`self.HitAnimIndexCurrent`))
      (:`then`
        (set `self.HitAnimIndexCurrent` (`KismetMathLibrary.SelectInt` (+ _hitanimindexcurrent 1) 0 (< _hitanimindexcurrent (`self.HitAnimIndexMax`)))))
      (:`OnCompleted`
        (set `self.HitAnimIndexCurrent` 0))
      (:`OnBlendOut`
        (set `Actor.bCanBeDamaged` true _owner)))))

(event `IncrementCombo`
  (`/Engine/EditorBlueprintResources/StandardMacros.IncrementInt` (`self.ComboCount`)
    (:`  `
      (`KismetSystemLibrary.RetriggerableDelay` 2.0)
      (set `self.ComboCount` 0))))

(fn `Calcul Damage`
  (returns (`Base Damage` :type "Float (double-precision)"))
  (bind _base_damage (`self.Base Damage`))
  (return (* (`KismetMathLibrary.RandomFloatInRange` _base_damage (* _base_damage 1.3)) (`self.Damage Upgrade`))))

(fn `Check Upgrade`
  (switch `int` 0
    (:`0`
      (set `self.Damage Upgrade` 1.0))
    (:`1`
      (set `self.Damage Upgrade` 1.5))
    (:`2`
      (set `self.Damage Upgrade` 2.0))
    (:`3`
      (set `self.Damage Upgrade` 3.0)))
  (return))

(fn `TriggerSimpleHit`
  (bind _owner (`self.Owner`))
  (bind _returnvalue (`Actor.K2_GetActorRotation` _owner))
  (bind _returnvalue_2 (`Actor.K2_GetActorLocation` _owner))
  (bind _returnvalue_3 (`KismetMathLibrary.GetForwardVector` _returnvalue))
  (bind (_outhit _returnvalue_4) (`KismetSystemLibrary.BoxTraceSingleForObjects` (+ _returnvalue_2 (* _returnvalue_3 (`self.SpellStartOffset`))) (+ _returnvalue_2 (* _returnvalue_3 (`self.SpellEndOffset`))) (`self.SpellHitSize`) _returnvalue (`|MakeArray` "ObjectTypeQuery3" :!type "EObjectTypeQuery Enum") false (`|MakeArray` (`GameplayStatics.GetPlayerCharacter` 0) :!type "Actor Object Reference")))
  (if _returnvalue_4
    (bind (_bblockinghit _binitialoverlap _time _distance _location _impactpoint _normal _impactnormal _physmat _hitactor) (`GameplayStatics.BreakHitResult` _outhit))
    (`GameplayStatics.ApplyDamage` _hitactor (`self.Calcul Damage`))
    (`GameplayStatics.PlaySoundAtLocation` "/Game/Sounds/SFX/Hits/Hit_Blob.Hit_Blob" _impactpoint (struct) 1.0 1.0 0.0 null null null)
    (`GameplayStatics.SpawnForceFeedbackAtLocation` "/Game/Feelback/Impact.Impact" _impactpoint (struct) false 1.0 0.0 null)
    (`self.IncrementCombo`)
    (`/Game/Blueprints/Gameplay/ActorComponents/Players/AC_Stamina.Add Stamina` (`/Game/Blueprints/Gameplay/Character_Master.AC_Stamina` (`self.Owner`)) (`self.Add Stamina`))
    (switch `/Game/Blueprints/Gameplay/Datas/E_ElementTypes` (`self.Element`)
      (:`NewEnumerator0`
        _)
      (:`NewEnumerator1`
        _)
      (:`NewEnumerator2`
        _)
      (:`NewEnumerator3`
        _))
    (`NiagaraFunctionLibrary.SpawnSystemAtLocation` "/Game/Particles/Systems/FX_Impact.FX_Impact" _impactpoint (`KismetMathLibrary.Conv_VectorToRotator` _impactpoint))))