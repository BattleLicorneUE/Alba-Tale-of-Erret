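; Actor component that gives a Character_Master ranged combo and beam attacks.
; DistanceAttack cycles montages, using notifies to open combo windows, pause while right mouse is held, and call CastDistanceSkill.
; That spawns a skill actor beside the owner, requiring a camera target for the player and targeting the player otherwise.
; The beam attack freezes its montage and starts a looping timer until ended; RayAttack only draws a debug line, and FireProjectileOnTarget is empty.
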(event `self.ReceiveBeginPlay`
  (bind _ascharacter_master (cast `/Game/Blueprints/Gameplay/Character_Master` (`self.GetOwner`)))
  (set `self.Owner` _ascharacter_master)
  (set `self.DistAttackIndexMax` (- (`KismetArrayLibrary.Array_Length` (`self.DistAttackAnims`)) 1)))

(event `DistanceAttack`
  (bind _distattackindex (`self.DistAttackIndex`))
  (bind _returnvalue (`SkeletalMeshComponent.GetAnimInstance` (`Character.Mesh` (`self.Owner`))))
  (bind _returnvalue_2 (`SkeletalMeshComponent.GetAnimInstance` (`Character.Mesh` (`self.Owner`))))
  (if (`self.bIsAnimPaused`)
    (`AnimInstance.Montage_Resume` _returnvalue_2 (`AnimInstance.GetCurrentActiveMontage` _returnvalue_2))
    (set `self.bIsAnimPaused` false)
    (elif (`PlayerController.IsInputKeyDown` (`GameplayStatics.GetPlayerController` 0) "RightMouseButton")
      (set `self.bIsAnimPaused` true)))
  (if (`self.bCanAttack`)
    (set `self.bCanAttack` false)
    (bind _notifyname (`|PlayMontage` (`Character.Mesh` (`self.Owner`)) (`|GetArrayItem` (`self.DistAttackAnims`) (`self.DistAttackIndex`)))
      (:`then`
        (set `self.DistAttackIndex` (`KismetMathLibrary.SelectInt` (+ _distattackindex 1) 0 (< _distattackindex (`self.DistAttackIndexMax`)))))
      (:`OnCompleted`
        (set `self.bCanAttack` true)
        (set `self.DistAttackIndex` 0))
      (:`OnNotifyBegin`
        (switch `name` _notifyname
          (:`Hit`
            (`self.CastDistanceSkill`))
          (:`CanCombo`
            (set `self.bCanAttack` true))
          (:`Recovery`
            (set `self.bCanAttack` false))
          (:`Pause`
            (if (`self.bIsAnimPaused`)
              (`AnimInstance.Montage_Pause` _returnvalue (`AnimInstance.GetCurrentActiveMontage` _returnvalue)))))))))

(event `StartRayAttack`
  (bind _mesh (`Character.Mesh` (`self.Owner`)))
  (bind _returnvalue (`SkeletalMeshComponent.GetAnimInstance` _mesh))
  (bind _notifyname (`|PlayMontage` _mesh "/Game/Resources/Animations/Animations_Selected/Animations_Magic/MG_BeamAttack_Montage.MG_BeamAttack_Montage")
    (:`OnNotifyBegin`
      (switch `name` _notifyname
        (:`Pause`
          (`AnimInstance.Montage_Pause` _returnvalue (`AnimInstance.GetCurrentActiveMontage` _returnvalue))
          (bind _returnvalue_2 (`KismetSystemLibrary.K2_SetTimerDelegate` (`|CreateDelegate` :!event `RayAttack`) 0.1 true))
          (set `self.RayAttackTimer` _returnvalue_2))))))

(event `RayAttack`
  (bind _owner (`self.Owner`))
  (`KismetSystemLibrary.DrawDebugLine` (`SceneComponent.GetSocketLocation` (`Character.Mesh` _owner) "RightHandSocket") (`Actor.K2_GetActorLocation` (`/Game/Blueprints/Gameplay/ActorComponents/AC_Camera.Target` (`/Game/Blueprints/Gameplay/Character_Gameplay.AC_Camera` (cast `/Game/Blueprints/Gameplay/Character_Gameplay` _owner :!pure true)))) (struct :`G` 0.14433 :`B` 1.0 :`A` 1.0) 0.1 3.0))

(event `EndRayAttack`
  (bind _returnvalue (`SkeletalMeshComponent.GetAnimInstance` (`Character.Mesh` (`self.Owner`))))
  (`KismetSystemLibrary.K2_ClearAndInvalidateTimerHandle` (`self.RayAttackTimer`))
  (`AnimInstance.Montage_Resume` _returnvalue (`AnimInstance.GetCurrentActiveMontage` _returnvalue)))

(fn `CastDistanceSkill`
  (bind _owner (`self.Owner`))
  (bind _capsulecomponent (`Character.CapsuleComponent` (`self.Owner`)))
  (bind _returnvalue (`SceneComponent.K2_GetComponentRotation` _capsulecomponent))
  (bind _returnvalue_2 (`KismetMathLibrary.MakeVector` (.x (+ (`SceneComponent.K2_GetComponentLocation` _capsulecomponent) (* (`KismetMathLibrary.GetRightVector` _returnvalue) 100.0))) (.y (+ (`SceneComponent.K2_GetComponentLocation` _capsulecomponent) (* (`KismetMathLibrary.GetRightVector` _returnvalue) 100.0))) (- (.z (+ (`SceneComponent.K2_GetComponentLocation` _capsulecomponent) (* (`KismetMathLibrary.GetRightVector` _returnvalue) 100.0))) (`CapsuleComponent.CapsuleHalfHeight` _capsulecomponent))))
  (if (== _owner (`GameplayStatics.GetPlayerCharacter` 0))
    (`/Engine/EditorBlueprintResources/StandardMacros.IsValid` (`/Game/Blueprints/Gameplay/ActorComponents/AC_Camera.Target` (`/Game/Blueprints/Gameplay/Character_Gameplay.AC_Camera` (cast `/Game/Blueprints/Gameplay/Character_Gameplay` _owner :!pure true)))
      (:`Is Valid`
        (`|SpawnActorFromClass` "/Game/Blueprints/Gameplay/Actors/Skills/AC_DistanceSkill.AC_DistanceSkill_C" (`KismetMathLibrary.MakeTransform` _returnvalue_2 _returnvalue) "Undefined" "OverrideRootScale" null null _owner)))
    (else
      (`|SpawnActorFromClass` "/Game/Blueprints/Gameplay/Actors/Skills/AC_DistanceSkill.AC_DistanceSkill_C" (`KismetMathLibrary.MakeTransform` _returnvalue_2 _returnvalue) "Undefined" "OverrideRootScale" null (cast `/Game/Blueprints/Gameplay/Character_Master` (`GameplayStatics.GetPlayerCharacter` 0) :!pure true) null))))

(fn `FireProjectileOnTarget`)