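; Actor component that tracks health for the character that owns it, with functions to damage, heal and reset it.
; On BeginPlay it stores the owning Character and sets current and max health from the default.
; For Character_Gameplay owners, a looping one-second timer regenerates health up to the max.
; All changes are clamped, though damage caps at the default health rather than the max.
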(event `Reset Health`
  ;[1 1 1] Reset Health
  (`self.INIT Health`))

(event `self.ReceiveBeginPlay`
  ;[1 1 1] Begin player, and Set Owner
  (bind _ascharacter (cast `Character` (`self.GetOwner`)))
  (set `self.Owner` _ascharacter)
  ;[1 1 1] Init Health
  (`self.INIT Health`)
  ;[1 1 1] Set Regene if Character gameplay
  (cast `/Game/Blueprints/Gameplay/Character_Gameplay` (`self.Owner`))
  (`KismetSystemLibrary.K2_SetTimer` null "Regene Health" 1.0 true))

(fn `Add Health`
  (params (`Add Health` :type "Float (double-precision)"))
  (set `self.Health_Current` (`KismetMathLibrary.FClamp` (+ (`self.Health_Current`) `Add Health`) (`self.Health_Min`) (`self.Health_Max`))))

(fn `Apply Damage Simple`
  (params (Damage :type "Float (double-precision)"))
  (set `self.Health_Current` (`KismetMathLibrary.FClamp` (- (`self.Health_Current`) Damage) 0.0 (`self.Health_Default`))))

(fn `INIT Health`
  (bind _health_default (`self.Health_Default`))
  (set `self.Health_Current` _health_default)
  (set `self.Health_Max` _health_default))

(fn `Regene Health`
  (if (< (`self.Health_Current`) (`self.Health_Max`))
    (set `self.Health_Current` (`KismetMathLibrary.FClamp` (+ (`self.Health_Current`) (`self.Health / S`)) 0.0 (`self.Health_Max`)))))