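; Actor component that tracks level and experience for its owning Character_Gameplay, whose reference it caches on BeginPlay.
; AddExp adds experience clamped to the current maximum, calls AddLevel when that is reached, then prints level and experience.
; AddLevel raises the level up to LevelMax, resets experience to zero, discarding any overflow, and multiplies the required experience by AmountExp, even at the level cap.
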(event `self.ReceiveBeginPlay`
  (bind _ascharacter_gameplay (cast `/Game/Blueprints/Gameplay/Character_Gameplay` (`self.GetOwner`)))
  (set `self.Ref Character Gameplay` _ascharacter_gameplay))

(fn `Add Exp`
  (params (`Add Exp` :type "Float (double-precision)"))
  (bind _output_get (set `self.Exp_Current` (`KismetMathLibrary.FClamp` (+ `Add Exp` (`self.Exp_Current`)) 0.0 (`self.Exp_Max`))))
  (if (>= _output_get (`self.Exp_Max`))
    (`self.Add Level`))
  (`KismetSystemLibrary.PrintString` (`KismetStringLibrary.Concat_StrStr` "Niveau  : " (`KismetStringLibrary.Conv_IntToString` (`self.Level`)) " Exp : " (`KismetStringLibrary.Conv_DoubleToString` (`self.Exp_Current`)))))

(fn `Add Level`
  (set `self.Level` (`KismetMathLibrary.Clamp` (+ (`self.Level`) 1) 1 (`self.Level_Max`)))
  (set `self.Exp_Current` 0.0)
  (set `self.Exp_Max` (* (`self.Exp_Max`) (`self.Amount Exp`))))