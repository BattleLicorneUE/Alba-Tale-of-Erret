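; Actor component that manages a player character's stamina pool as the cost of using skills.
; On BeginPlay it fills the pool to its default and, for Character_Gameplay owners, starts a looping timer that regenerates stamina.
; UseStamina checks affordability, then deducts the cost or prints a French out-of-stamina message.
; AddStamina grants clamped refills; logic that lowers maximum stamina is present but never runs.
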(event `self.ReceiveBeginPlay`
  (bind _ascharacter (cast `Character` (`self.GetOwner`)))
  (set `self.Owner` _ascharacter)
  (`self.INIT Stamina`)
  (cast `/Game/Blueprints/Gameplay/Character_Gameplay` (`self.Owner`))
  (`KismetSystemLibrary.K2_SetTimer` null "Regene Stamina" 0.5 true))

(fn `Add Stamina`
  (params (`Add Stamina` :type "Float (double-precision)"))
  (if (< `Add Stamina` (`self.Stamina_Max`))
    (set `self.Stamina_Current` (`KismetMathLibrary.FClamp` (+ (`self.Stamina_Current`) `Add Stamina`) (`self.Stamina_Min`) (`self.Stamina_Max`)))))

(fn `Check Stamina`
  (params (`Skill Consume` :type "Float (double-precision)"))
  (returns (ReturnValue :type Boolean))
  (return (<= `Skill Consume` (`self.Stamina_Current`))))

(fn `Consume Stamina`
  (params (Consume :type "Float (double-precision)"))
  (set `self.Stamina_Current` (`KismetMathLibrary.FClamp` (- (`self.Stamina_Current`) Consume) 0.0 (`self.Stamina_Default`))))

(fn `INIT Stamina`
  (bind _stamina_default (`self.Stamina_Default`))
  (set `self.Stamina_Current` _stamina_default)
  (set `self.Stamina_Max` _stamina_default))

(fn `Regene Stamina`
  (if (< (`self.Stamina_Current`) (`self.Stamina_Max`))
    (set `self.Stamina_Current` (`KismetMathLibrary.FClamp` (+ (`self.Stamina_Current`) (`self.Stamina/ S`)) 0.0 (`self.Stamina_Max`)))))

(fn `Use Stamina`
  (params (`Skill Consume` :type "Float (double-precision)"))
  (returns (ReturnValue :type Boolean))
  (bind _returnvalue (`self.Check Stamina` `Skill Consume`))
  (if _returnvalue
    (`self.Consume Stamina` `Skill Consume`)
    (return _returnvalue)
    (else
      (`KismetSystemLibrary.PrintString` "Le developpeur tiens a te signaler que tu n'as plus de stamina pour lancer ton skill."))))