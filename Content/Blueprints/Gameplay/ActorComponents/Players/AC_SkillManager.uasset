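; Player component that manages the four elemental skill sets (Fire, Water, Metal, Air) and the list of learned skills.
; Element switches copy three HUD-assigned skills to the player controller and update UI, character color and VFX.
; A 1.5-second lock gates that refresh, though element and sound change before it.
; LearnNewSkill registers skills and creates their HUD upgrade widgets, or restores upgrade levels for known skills when loading.
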(event `UpdateInputSkills`
  (switch `/Game/Blueprints/Gameplay/Datas/E_ElementTypes` (`self.CurrentElement`)
    (:`NewEnumerator0`
      (`self.Fire_Update_Skill`))
    (:`NewEnumerator1`
      (`self.Water_Update_Skill`))
    (:`NewEnumerator2`
      (`self.Metal_Update_Skill`))
    (:`NewEnumerator3`
      (`self.Air_Update_Skill`)))
  (`/Game/Blueprints/HUD/Player/Interface_Player.Update Element Select` (`/Game/Blueprints/Gameplay/PlayerController_Gameplay.InterfacePlayer` (`/Game/Blueprints/Gameplay/Library_Blueprints/FunctionLibrary.Get Player Controller`)) (`self.CurrentElement`)))

(event `self.ReceiveBeginPlay`
  (`self.UpdateInputSkills`))

(event `SwitchToWater`
  (bind _ascharacter_gameplay (cast `/Game/Blueprints/Gameplay/Character_Gameplay` (`self.GetOwner`) :!pure true))
  (set `self.CurrentElement` "NewEnumerator1")
  (`GameplayStatics.PlaySound2D` "/Game/Sounds/SFX/SwitchElements/E_Water.E_Water" 1.0 1.0 0.0 null null)
  (if (not (`self.bChangingSkillSet`)) :!label _label
    (set `self.bChangingSkillSet` true)
    (`/Game/Blueprints/HUD/Player/Interface_Player.Update Element Select` (`/Game/Blueprints/Gameplay/PlayerController_Gameplay.InterfacePlayer` (`/Game/Blueprints/Gameplay/Library_Blueprints/FunctionLibrary.Get Player Controller`)) (`self.CurrentElement`))
    (switch `/Game/Blueprints/Gameplay/Datas/E_ElementTypes` (`self.CurrentElement`)
      (:`NewEnumerator0`
        (`self.Fire_Update_Skill`)
        (set `/Game/Blueprints/Gameplay/Character_Gameplay.In Value` (struct :`R` 1.0 :`B` 0.006586 :`A` 1.0) _ascharacter_gameplay))
      (:`NewEnumerator1`
        (`self.Water_Update_Skill`)
        (set `/Game/Blueprints/Gameplay/Character_Gameplay.In Value` (struct :`R` 0.05725 :`B` 1.0 :`A` 1.0) _ascharacter_gameplay))
      (:`NewEnumerator2`
        (`self.Metal_Update_Skill`)
        (set `/Game/Blueprints/Gameplay/Character_Gameplay.In Value` (struct :`R` 0.677083 :`G` 0.677083 :`B` 0.677083 :`A` 1.0) _ascharacter_gameplay))
      (:`NewEnumerator3`
        (`self.Air_Update_Skill`)
        (set `/Game/Blueprints/Gameplay/Character_Gameplay.In Value` (struct :`R` 0.307292 :`G` 1.0 :`B` 0.494847 :`A` 1.0) _ascharacter_gameplay)))
    (`/Game/Blueprints/Gameplay/Character_Gameplay.UpdateVFX_SwitchElement` _ascharacter_gameplay)
    (`KismetSystemLibrary.Delay` 1.5)
    (set `self.bChangingSkillSet` false)))

(event `SwitchToFire`
  (set `self.CurrentElement` "NewEnumerator0")
  (`GameplayStatics.PlaySound2D` "/Game/Sounds/SFX/SwitchElements/E_Fire.E_Fire" 1.0 1.0 0.0 null null)
  (goto _label))

(event `SwitchToMetal`
  (set `self.CurrentElement` "NewEnumerator2")
  (`GameplayStatics.PlaySound2D` "/Game/Sounds/SFX/SwitchElements/E_Metal.E_Metal" 1.0 1.0 0.0 null null)
  (goto _label))

(event `SwitchToAir`
  (set `self.CurrentElement` "NewEnumerator3")
  (`GameplayStatics.PlaySound2D` "/Game/Sounds/SFX/SwitchElements/E_Wind.E_Wind" 1.0 1.0 0.0 null null)
  (goto _label))

(fn `Air_Update_Skill`
  (bind _asplayer_controller_gameplay (cast `/Game/Blueprints/Gameplay/PlayerController_Gameplay` (`GameplayStatics.GetPlayerController` 0) :!pure true))
  (bind _air (`/Game/Blueprints/HUD/Player/Compétence/Skill_MainPanel.Air` (`/Game/Blueprints/Gameplay/PlayerController_Gameplay.HUD Skill` _asplayer_controller_gameplay)))
  (set `/Game/Blueprints/Gameplay/PlayerController_Gameplay.Skill 1` (`/Game/Blueprints/HUD/Player/Compétence/SwitchSkill.Input_1` _air) _asplayer_controller_gameplay)
  (set `/Game/Blueprints/Gameplay/PlayerController_Gameplay.Skill 2` (`/Game/Blueprints/HUD/Player/Compétence/SwitchSkill.Input_2` _air) _asplayer_controller_gameplay)
  (set `/Game/Blueprints/Gameplay/PlayerController_Gameplay.Skill 3` (`/Game/Blueprints/HUD/Player/Compétence/SwitchSkill.Input_3` _air) _asplayer_controller_gameplay))

(fn `Fire_Update_Skill`
  (bind _asplayer_controller_gameplay (cast `/Game/Blueprints/Gameplay/PlayerController_Gameplay` (`GameplayStatics.GetPlayerController` 0) :!pure true))
  (bind _fire (`/Game/Blueprints/HUD/Player/Compétence/Skill_MainPanel.Fire` (`/Game/Blueprints/Gameplay/PlayerController_Gameplay.HUD Skill` _asplayer_controller_gameplay)))
  (set `/Game/Blueprints/Gameplay/PlayerController_Gameplay.Skill 1` (`/Game/Blueprints/HUD/Player/Compétence/SwitchSkill.Input_1` _fire) _asplayer_controller_gameplay)
  (set `/Game/Blueprints/Gameplay/PlayerController_Gameplay.Skill 2` (`/Game/Blueprints/HUD/Player/Compétence/SwitchSkill.Input_2` _fire) _asplayer_controller_gameplay)
  (set `/Game/Blueprints/Gameplay/PlayerController_Gameplay.Skill 3` (`/Game/Blueprints/HUD/Player/Compétence/SwitchSkill.Input_3` _fire) _asplayer_controller_gameplay))

(fn `LearnNewSkill`
  (params (SkillToLearn :type "/Game/Blueprints/Gameplay/Datas/E_SkillNames Enum" :default "NewEnumerator6") (`Niveau Upgrade` :type Integer) (`Loading?` :type Boolean))
  (locals (UpgradeSkills :type "Array of Widget Object Reference"))
  (bind _hud_skill (`/Game/Blueprints/Gameplay/PlayerController_Gameplay.HUD Skill` (`/Game/Blueprints/Gameplay/Library_Blueprints/FunctionLibrary.Get Player Controller`)))
  (bind _upgradeskillbox (`/Game/Blueprints/HUD/Player/Compétence/Skill_MainPanel.UpgradeSkillBox` _hud_skill))
  (bind _upgradeskillbox_2 (`/Game/Blueprints/HUD/Player/Compétence/Skill_MainPanel.UpgradeSkillBox` (`/Game/Blueprints/Gameplay/PlayerController_Gameplay.HUD Skill` (`/Game/Blueprints/Gameplay/Library_Blueprints/FunctionLibrary.Get Player Controller`))))
  (bind _returnvalue (`PanelWidget.GetAllChildren` _upgradeskillbox_2))
  (if (`KismetArrayLibrary.Array_Contains` (`self.LearnedSkills`) SkillToLearn)
    (if `Loading?`
      (for _array_element _returnvalue
        (bind _asupgrade_skill (cast `/Game/Blueprints/HUD/Player/Compétence/UpgradeSkill` _array_element))
        (if (`|EnumEquality` (`/Game/Blueprints/HUD/Player/Compétence/UpgradeSkill.SkillName` _asupgrade_skill) SkillToLearn)
          (set `/Game/Blueprints/HUD/Player/Compétence/UpgradeSkill.Niveau Upgrade` `Niveau Upgrade` _asupgrade_skill)))
      (bind _output_get (set `local.UpgradeSkills` _returnvalue))
      (`PanelWidget.ClearChildren` _upgradeskillbox_2)
      (for _array_element_2 _output_get
        (`VerticalBox.AddChildToVerticalBox` _upgradeskillbox_2 _array_element_2))
      (return))
    (else
      (`KismetArrayLibrary.Array_Add` (`self.LearnedSkills`) SkillToLearn)
      (`/Game/Blueprints/HUD/Player/Compétence/Skill_MainPanel.UpdateAllElements` _hud_skill)
      (bind _returnvalue_2 (`|CreateWidget` "/Game/Blueprints/HUD/Player/Compétence/UpgradeSkill.UpgradeSkill_C" null `Niveau Upgrade` SkillToLearn))
      (`KismetArrayLibrary.Array_Add` (`/Game/Blueprints/HUD/Player/Compétence/Skill_MainPanel.AllSkills` _hud_skill) _returnvalue_2)
      (`VerticalBox.AddChildToVerticalBox` _upgradeskillbox _returnvalue_2)
      (bind _output_get_2 (set `local.UpgradeSkills` (`PanelWidget.GetAllChildren` _upgradeskillbox)))
      (bind _returnvalue_3 (`KismetArrayLibrary.Array_Find` _output_get_2 _returnvalue_2))
      (`KismetArrayLibrary.Array_Swap` _output_get_2 _returnvalue_3 (- _returnvalue_3 1))
      (`PanelWidget.ClearChildren` _upgradeskillbox)
      (for _array_element_3 _output_get_2
        (`VerticalBox.AddChildToVerticalBox` _upgradeskillbox _array_element_3))
      (`KismetSystemLibrary.PrintString` (`KismetStringLibrary.Concat_StrStr` "Nouvelle compétence : " (`|GetEnumeratorNameAsString` SkillToLearn) "current elem : " (`|GetEnumeratorNameAsString` (`self.CurrentElement`))))
      (return))))

(fn `Metal_Update_Skill`
  (bind _asplayer_controller_gameplay (cast `/Game/Blueprints/Gameplay/PlayerController_Gameplay` (`GameplayStatics.GetPlayerController` 0) :!pure true))
  (bind _metal (`/Game/Blueprints/HUD/Player/Compétence/Skill_MainPanel.Metal` (`/Game/Blueprints/Gameplay/PlayerController_Gameplay.HUD Skill` _asplayer_controller_gameplay)))
  (set `/Game/Blueprints/Gameplay/PlayerController_Gameplay.Skill 1` (`/Game/Blueprints/HUD/Player/Compétence/SwitchSkill.Input_1` _metal) _asplayer_controller_gameplay)
  (set `/Game/Blueprints/Gameplay/PlayerController_Gameplay.Skill 2` (`/Game/Blueprints/HUD/Player/Compétence/SwitchSkill.Input_2` _metal) _asplayer_controller_gameplay)
  (set `/Game/Blueprints/Gameplay/PlayerController_Gameplay.Skill 3` (`/Game/Blueprints/HUD/Player/Compétence/SwitchSkill.Input_3` _metal) _asplayer_controller_gameplay))

(fn `Water_Update_Skill`
  (bind _asplayer_controller_gameplay (cast `/Game/Blueprints/Gameplay/PlayerController_Gameplay` (`GameplayStatics.GetPlayerController` 0) :!pure true))
  (bind _water (`/Game/Blueprints/HUD/Player/Compétence/Skill_MainPanel.Water` (`/Game/Blueprints/Gameplay/PlayerController_Gameplay.HUD Skill` _asplayer_controller_gameplay)))
  (set `/Game/Blueprints/Gameplay/PlayerController_Gameplay.Skill 1` (`/Game/Blueprints/HUD/Player/Compétence/SwitchSkill.Input_1` _water) _asplayer_controller_gameplay)
  (set `/Game/Blueprints/Gameplay/PlayerController_Gameplay.Skill 2` (`/Game/Blueprints/HUD/Player/Compétence/SwitchSkill.Input_2` _water) _asplayer_controller_gameplay)
  (set `/Game/Blueprints/Gameplay/PlayerController_Gameplay.Skill 3` (`/Game/Blueprints/HUD/Player/Compétence/SwitchSkill.Input_3` _water) _asplayer_controller_gameplay))