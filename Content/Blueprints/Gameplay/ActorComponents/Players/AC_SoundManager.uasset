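; Player character component that swaps ambient audio for a zone-specific sound while enemies are in the owner's SoundEnemyArray, likely as combat music.
; A looping timer, started only for player 0, polls that array.
; When enemies appear, it picks a DT_Sounds row by type and current zone, fades it in and mutes AmbiantSound.
; When none remain, it fades out and restores ambience; each switch pauses polling for a delay.
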(event `self.ReceiveBeginPlay`
  (if (== (`self.GetOwner`) (`GameplayStatics.GetPlayerCharacter` 0))
    (bind _returnvalue (`KismetSystemLibrary.K2_SetTimerDelegate` (`|CreateDelegate` :!event `CheckEnemyInRange`) (`self.EnemyCheckTime`) true))
    (set `self.EnemyCheckTimer` _returnvalue)))

(event `CheckEnemyInRange`
  (bind _currentsound (`self.CurrentSound`))
  (bind _ascharacter_gameplay (cast `/Game/Blueprints/Gameplay/Character_Gameplay` (`self.GetOwner`)))
  (if (>= (`KismetArrayLibrary.Array_Length` (`/Game/Blueprints/Gameplay/Character_Gameplay.SoundEnemyArray` _ascharacter_gameplay)) 1)
    (if (not (`self.SoundPlaying?`))
      (set `self.SoundPlaying?` true)
      (`KismetSystemLibrary.K2_ClearAndInvalidateTimerHandle` (`self.EnemyCheckTimer`))
      (bind _outrownames (`DataTableFunctionLibrary.GetDataTableRowNames` "/Game/Sounds/DT_Sounds.DT_Sounds"))
      (for _array_element _outrownames
        (bind _returnvalue (`|GetDataTableRow` "/Game/Sounds/DT_Sounds.DT_Sounds" _array_element)
          (:`then`
            (bind (_zonename _soundtype _sound _attenuation) (break `/Game/Sounds/Sound_Structure` _returnvalue))
            (if (and (`|EnumEquality` _soundtype "NewEnumerator0") (`|EnumEquality` _zonename (`self.CurrentZone`)))
              (bind _output_get (set `self.SoundToPlay` _sound))
              (bind _returnvalue_2 (`GameplayStatics.SpawnSoundAtLocation` _output_get (`Actor.K2_GetActorLocation` (`self.GetOwner`)) (struct) 1.0 1.0 0.0 _attenuation null))
              (bind _output_get_2 (set `self.CurrentSound` _returnvalue_2))
              (`AudioComponent.FadeIn` _output_get_2 (`self.Fade in Duration`) 1.0 0.0 "Logarithmic")
              (`AudioComponent.SetVolumeMultiplier` (`/Game/Blueprints/Gameplay/Character_Gameplay.AmbiantSound` (`/Game/Blueprints/Gameplay/Library_Blueprints/FunctionLibrary.Get Player character`)) 0.0)
              (`KismetSystemLibrary.PrintString` "Sound played")
              (`KismetSystemLibrary.RetriggerableDelay` (`self.DelayBeforeCheck`))
              (bind _returnvalue_3 (`KismetSystemLibrary.K2_SetTimerDelegate` (`|CreateDelegate` :!event `CheckEnemyInRange`) (`self.EnemyCheckTime`) true))
              (set `self.EnemyCheckTimer` _returnvalue_3))))))
    (elif (`self.SoundPlaying?`)
      (set `self.SoundPlaying?` false)
      (`KismetSystemLibrary.K2_ClearAndInvalidateTimerHandle` (`self.EnemyCheckTimer`))
      (`/Engine/EditorBlueprintResources/StandardMacros.IsValid` _currentsound
        (:`Is Valid`
          (`AudioComponent.SetVolumeMultiplier` (`/Game/Blueprints/Gameplay/Character_Gameplay.AmbiantSound` (`/Game/Blueprints/Gameplay/Library_Blueprints/FunctionLibrary.Get Player character`)) 1.0)
          (`AudioComponent.FadeOut` _currentsound (`self.Fade Out Duration`) 0.0 "Logarithmic")
          (`KismetSystemLibrary.PrintString` "SoundStopped"))
        (:`Is Not Valid`
          (`KismetSystemLibrary.PrintString` "Current sound is empty")))
      (`KismetSystemLibrary.RetriggerableDelay` (`self.DelayBeforeCheck`))
      (bind _returnvalue_4 (`KismetSystemLibrary.K2_SetTimerDelegate` (`|CreateDelegate` :!event `CheckEnemyInRange`) (`self.EnemyCheckTime`) true))
      (set `self.EnemyCheckTimer` _returnvalue_4))))