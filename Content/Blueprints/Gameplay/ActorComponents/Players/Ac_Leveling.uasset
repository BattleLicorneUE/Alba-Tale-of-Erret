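; Actor component that handles player leveling, experience and skill points for the gameplay character.
; AddExp clamps gained experience to the current maximum and calls AddLevel when full, discarding overflow.
; AddLevel raises the capped level, resets experience, scales the next threshold by a multiplier, grants a skill point and plays the level-up animation on player 0's interface.
; Helper functions check and spend skill points, and AddExp prints debug progress.
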(event `self.ReceiveBeginPlay`
  (bind _ascharacter_gameplay (cast `/Game/Blueprints/Gameplay/Character_Gameplay` (`self.GetOwner`)))
  (set `self.Ref Character Gameplay` _ascharacter_gameplay))

(fn `Add Exp`
  (params (`Add Exp` :type "Float (double-precision)"))
  (bind _output_get (set `self.Exp_Current` (`KismetMathLibrary.FClamp` (+ `Add Exp` (`self.Exp_Current`)) 0.0 (`self.Exp_Max`))))
  (if (>= _output_get (`self.Exp_Max`))
    (`self.Add Level`))
  (`KismetSystemLibrary.PrintString` (`KismetStringLibrary.Concat_StrStr` "Niveau  : " (`KismetStringLibrary.Conv_IntToString` (`self.Level`)) " Exp : " (`KismetStringLibrary.Conv_DoubleToString` (`self.Exp_Current`)))))

(fn `Add Level`
  (bind _interfaceplayer (`/Game/Blueprints/Gameplay/PlayerController_Gameplay.InterfacePlayer` (cast `/Game/Blueprints/Gameplay/PlayerController_Gameplay` (`GameplayStatics.GetPlayerController` 0) :!pure true)))
  (set `self.Level` (`KismetMathLibrary.Clamp` (+ (`self.Level`) 1) 1 (`self.Level_Max`)))
  (set `self.Exp_Current` 0.0)
  (set `self.Exp_Max` (* (`self.Exp_Max`) (`self.Amount Exp`)))
  (set `self.SkillPoints` (+ (`self.SkillPoints`) 1))
  (`UserWidget.PlayAnimation` _interfaceplayer (`/Game/Blueprints/HUD/Player/Interface_Player.DIsplayNiveau` _interfaceplayer) 0.0 1 "Forward" 1.0 false))

(fn `Check if  PT Skill `
  (params (Requis :type Integer))
  (returns (`Can use Skill Point` :type Boolean))
  (return (>= (`self.SkillPoints`) Requis)))

(fn `Use Point Skill`
  (params (`Skill Point Requis` :type Integer))
  (set `self.SkillPoints` (- (`self.SkillPoints`) `Skill Point Requis`)))