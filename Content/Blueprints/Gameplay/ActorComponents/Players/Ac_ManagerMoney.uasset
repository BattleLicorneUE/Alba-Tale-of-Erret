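; Player actor component that manages a gold balance through add, spend and affordability-check functions.
; AddGold clamps the new total between zero and GoldMax and prints it for debugging.
; CheckGold reports whether CurrentGold covers a required amount, while UseGold subtracts without calling that check.
; UseGold clamps with both bounds at zero, so any spend leaves CurrentGold at zero.
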(fn `Add Gold`
  (params (`Add Gold` :type Integer))
  (bind _output_get (set `self.Current Gold` (`KismetMathLibrary.Clamp` (+ (`self.Current Gold`) `Add Gold`) 0 (`self.Gold Max`))))
  (`KismetSystemLibrary.PrintString` (`KismetStringLibrary.Concat_StrStr` "Gold Total : " (`KismetStringLibrary.Conv_IntToString` _output_get))))

(fn `Check Gold`
  (params (`Gold Requis` :type Integer))
  (returns (`Check Gold Requis` :type Boolean))
  (return (>= (`self.Current Gold`) `Gold Requis`)))

(fn `Use Gold`
  (params (`Require Gold` :type Integer))
  (set `self.Current Gold` (`KismetMathLibrary.Clamp` (- (`self.Current Gold`) `Require Gold`))))