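; Player camera component that provides manual and automatic lock-on to enemies for Character_Gameplay.
; Input Lock toggles a lock on the nearest enemy from one externally fed array, while AutoLock picks from a separate auto-lock array.
; A Tick-driven gate eases control rotation toward the target and sets actor yaw directly, resetting when the target becomes invalid.
; Lock changes also apply one-shot eased adjustments to boom offset and FOV.
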(event `self.ReceiveBeginPlay`
  ;[1 1 1] Begin play
  (bind _ascharacter_gameplay (cast `/Game/Blueprints/Gameplay/Character_Gameplay` (`self.GetOwner`)))
  (set `self.Owner` _ascharacter_gameplay))

(event `Add Array Ennemies`
  (params (Character :type "/Game/Blueprints/Gameplay/IntelligenceArticiel/Master/Character_Gameplay_Master_Enemy Object Reference (by ref)"))
  ;[1 1 1] Setup Array Enemies
  (`KismetArrayLibrary.Array_Add` (`self.Array Ennemies`) Character))

(event `Remove Array Ennemies`
  (params (Character :type "/Game/Blueprints/Gameplay/IntelligenceArticiel/Master/Character_Gameplay_Master_Enemy Object Reference (by ref)"))
  ;[1 1 1] Setup Array Enemies
  (if (== Character (`self.Target`))
    (set `self.Target` null))
  (`KismetArrayLibrary.Array_RemoveItem` (`self.Array Ennemies`) Character))

(event `Add Array Ennemies AutoLock`
  (params (Character :type "/Game/Blueprints/Gameplay/IntelligenceArticiel/Master/Character_Gameplay_Master_Enemy Object Reference (by ref)"))
  ;[1 1 1] Setup Array Enemies
  (`KismetArrayLibrary.Array_Add` (`self.Array Ennemies AutoLock`) Character))

(event `Remove Array Ennemies AutoLock`
  (params (Character :type "/Game/Blueprints/Gameplay/IntelligenceArticiel/Master/Character_Gameplay_Master_Enemy Object Reference (by ref)"))
  ;[1 1 1] Setup Array Enemies
  (if (== Character (`self.Target`))
    (set `self.Target` null)
    (`KismetArrayLibrary.Array_RemoveItem` (`self.Array Ennemies AutoLock`) Character)))

(event `self.ReceiveTick`
  (params (DeltaSeconds :type "Float (single-precision)"))
  (`/Engine/EditorBlueprintResources/StandardMacros.Gate` true :!label _label
    (:`Exit`
      (`self.Target`
        (:`then`
          (`Controller.SetControlRotation` (`Pawn.GetController` (`self.Owner`)) (`KismetMathLibrary.MakeRotator` 0.0 (.pitch (`|EaseFunction` "EaseInOut" (`self.CameraSpeed Delta Second` (`self.Camera Speed`)) (`Controller.GetControlRotation` (`Pawn.GetController` (`self.Owner`))) (`self.Look At Target`))) (.yaw (`|EaseFunction` "EaseInOut" (`self.CameraSpeed Delta Second` (`self.Camera Speed`)) (`Controller.GetControlRotation` (`Pawn.GetController` (`self.Owner`))) (`self.Look At Target`)))))
          (`Actor.K2_SetActorRotation` (`self.Owner`) (`KismetMathLibrary.MakeRotator` 0.0 0.0 (.yaw (`self.Look at Target`))) false))
        (:`else`
          (`self.Reset`))))))

(event `AutoLock`
  ;[1 1 1] AutoLock
  (bind _target (`/Game/Blueprints/Gameplay/Library_Blueprints/FunctionLibrary.FindActorsNearest` (`self.Array Ennemies AutoLock`) (`self.Owner`)))
  (bind _output_get (set `self.Target` _target))
  (`/Engine/EditorBlueprintResources/StandardMacros.IsValid` _output_get
    (:`Is Valid`
      (`GameplayStatics.PlaySound2D` "/Game/Sounds/SFX/Target/Target.Target" 1.0 1.0 0.0 null null)
      (set `self.Lock?` true :!label _label_2)
      (set `Pawn.bUseControllerRotationYaw` true (`self.Owner`))
      (`|ExecutionSequence`
        (:`then_0`
          (goto _label :!via `Open`))
        (:`then_1`
          (set `SpringArmComponent.SocketOffset` (`KismetMathLibrary.MakeVector` 0.0 (`|EaseFunction` "EaseIn" (`self.CameraSpeed Delta Second` (`self.Camera Speed`)) (`self.Camere Offset Y Default`) (`self.Camere Offset Y Target`)) 80.0) (`/Game/Blueprints/Gameplay/Character_Gameplay.CameraBoom` (`self.Owner`)))
          (`CameraComponent.SetFieldOfView` (`/Game/Blueprints/Gameplay/Character_Gameplay.Camera` (`self.Owner`)) (`|EaseFunction` "EaseIn" (`self.CameraSpeed Delta Second` (`self.Camera Speed`)) (`self.Field Of View Default`) (`self.Field Of View Target`))))))))

(event `Input Lock`
  (if (`self.Lock?`)
    (set `self.Lock?` false :!label _label_3)
    (set `Pawn.bUseControllerRotationYaw` false (`self.Owner`))
    (`|ExecutionSequence`
      (:`then_0`
        (goto _label :!via `Close`))
      (:`then_1`
        (set `SpringArmComponent.SocketOffset` (`KismetMathLibrary.MakeVector` 0.0 (`|EaseFunction` "EaseInOut" (`self.CameraSpeed Delta Second` (`self.Camera Speed`)) (`self.Camere Offset Y Target`) (`self.Camere Offset Y Default`)) 80.0) (`/Game/Blueprints/Gameplay/Character_Gameplay.CameraBoom` (`self.Owner`)))
        (`CameraComponent.SetFieldOfView` (`/Game/Blueprints/Gameplay/Character_Gameplay.Camera` (`self.Owner`)) (`|EaseFunction` "EaseInOut" (`self.CameraSpeed Delta Second` (`self.Camera Speed`)) (`self.Field Of View Target`) (`self.Field Of View Default`)))))
    (else
      (bind _target (`/Game/Blueprints/Gameplay/Library_Blueprints/FunctionLibrary.FindActorsNearest` (`self.Array Ennemies`) (`self.Owner`)))
      (bind _output_get (set `self.Target` _target))
      (`/Engine/EditorBlueprintResources/StandardMacros.IsValid` _output_get
        (:`Is Valid`
          (`GameplayStatics.PlaySound2D` "/Game/Sounds/SFX/Target/Target.Target" 1.0 1.0 0.0 null null)
          (goto _label_2))))))

(event `Reset`
  (goto _label_3))

(event `Old Camera`
  (set `SpringArmComponent.SocketOffset` (`KismetMathLibrary.MakeVector` 0.0 (`|EaseFunction` "CircularInOut" (`self.CameraSpeed Delta Second` (`self.Camera Speed`)) (`self.Camere Offset Y Default`) (`self.Camere Offset Y Target`)) 80.0) (`/Game/Blueprints/Gameplay/Character_Gameplay.CameraBoom` (`self.Owner`)))
  (`CameraComponent.SetFieldOfView` (`/Game/Blueprints/Gameplay/Character_Gameplay.Camera` (`self.Owner`)) (`|EaseFunction` "CircularInOut" (`self.CameraSpeed Delta Second` (`self.Camera Speed`)) (`self.Field Of View Default`) (`self.Field Of View Target`))))

(event `New Camera`
  (set `SpringArmComponent.SocketOffset` (`KismetMathLibrary.MakeVector` 0.0 (`|EaseFunction` "CircularIn" (`self.CameraSpeed Delta Second` (`self.Camera Speed`)) (`self.Camere Offset Y Target`) (`self.Camere Offset Y Default`)) 80.0) (`/Game/Blueprints/Gameplay/Character_Gameplay.CameraBoom` (`self.Owner`)))
  (`CameraComponent.SetFieldOfView` (`/Game/Blueprints/Gameplay/Character_Gameplay.Camera` (`self.Owner`)) (`|EaseFunction` "CircularIn" (`self.CameraSpeed Delta Second` (`self.Camera Speed`)) (`self.Field Of View Target`) (`self.Field Of View Default`))))

(fn `Look At Target`
  (returns (ReturnValue :type "Rotator Structure"))
  (return (`KismetMathLibrary.FindLookAtRotation` (`Actor.K2_GetActorLocation` (`self.Owner`)) (`Actor.K2_GetActorLocation` (`self.Target`)))))