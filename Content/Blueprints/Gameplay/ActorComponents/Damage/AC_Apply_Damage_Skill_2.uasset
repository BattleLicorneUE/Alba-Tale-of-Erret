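; Actor component that deals radial area damage for a skill, with a chance to land a critical hit.
; ApplyDamage rolls against the SAttack crit chance, then picks a random integer between the rounded min and max damage, multiplied by CoupCritik on a crit.
; Damage is applied with falloff between the given inner and outer radii, never below the minimum, using Pawn as the prevention channel.
; Critical hits also print "Coup Critique".
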(event `Apply Damage`
  (params (Origin :type "Vector Structure (by ref)") (DamageInnerRadius :type "Float (double-precision)") (DamageOuterRadius :type "Float (double-precision)"))
  (bind (_damagemin _damagemax _chancecritik _coupcritik) (break `/Game/Blueprints/Gameplay/Datas/S_Attack` (`self.S_Attack`)))
  (bind _returnvalue (`KismetMathLibrary.Round` _damagemin))
  (bind _returnvalue_2 (`KismetMathLibrary.Round` _damagemin))
  (if (<= (`KismetMathLibrary.RandomFloatInRange` 0.0 100.0) _chancecritik)
    (`GameplayStatics.ApplyRadialDamageWithFalloff` :`BaseDamage` (* (`KismetMathLibrary.Conv_IntToDouble` (`KismetMathLibrary.RandomIntegerInRange` _returnvalue_2 (`KismetMathLibrary.Round` _damagemax))) _coupcritik) :`MinimumDamage` (`KismetMathLibrary.Conv_IntToDouble` _returnvalue_2) :`Origin` Origin :`DamageInnerRadius` DamageInnerRadius :`DamageOuterRadius` DamageOuterRadius :`DamageFalloff` 0.2 :`DamageCauser` null :`InstigatedByController` null :`DamagePreventionChannel` "ECC_Pawn")
    (`KismetSystemLibrary.PrintText` "Coup Critique")
    (else
      (`GameplayStatics.ApplyRadialDamageWithFalloff` :`BaseDamage` (`KismetMathLibrary.Conv_IntToDouble` (`KismetMathLibrary.RandomIntegerInRange` _returnvalue (`KismetMathLibrary.Round` _damagemax))) :`MinimumDamage` (`KismetMathLibrary.Conv_IntToDouble` _returnvalue) :`Origin` Origin :`DamageInnerRadius` DamageInnerRadius :`DamageOuterRadius` DamageOuterRadius :`DamageFalloff` 0.2 :`DamageCauser` null :`InstigatedByController` null :`DamagePreventionChannel` "ECC_Pawn"))))