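; Actor component that applies damage for the first skill when ApplyDamage is called with a target, hit info and direction.
; It rolls a critical chance from the SAttack data, then deals a random integer between its minimum and maximum damage as point damage.
; A critical hit multiplies that damage by the CoupCritik factor and prints a "Coup Critique" message.
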(event `Apply Damage`
  (params (DamagedActor :type "Actor Object Reference") (HitInfo :type "HitResult Structure (by ref)") (HitFromDirection :type "Vector Structure (by ref)"))
  (bind (_damagemin _damagemax _chancecritik _coupcritik) (break `/Game/Blueprints/Gameplay/Datas/S_Attack` (`self.S_Attack`)))
  (if (<= (`KismetMathLibrary.RandomFloatInRange` 0.0 100.0) _chancecritik)
    (`GameplayStatics.ApplyPointDamage` DamagedActor (* (`KismetMathLibrary.Conv_IntToDouble` (`KismetMathLibrary.RandomIntegerInRange` (`KismetMathLibrary.Round` _damagemin) (`KismetMathLibrary.Round` _damagemax))) _coupcritik) HitFromDirection HitInfo)
    (`KismetSystemLibrary.PrintText` "Coup Critique")
    (else
      (`GameplayStatics.ApplyPointDamage` DamagedActor (`KismetMathLibrary.Conv_IntToDouble` (`KismetMathLibrary.RandomIntegerInRange` (`KismetMathLibrary.Round` _damagemin) (`KismetMathLibrary.Round` _damagemax))) HitFromDirection HitInfo))))