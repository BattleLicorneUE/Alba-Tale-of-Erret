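; Base actor component that deals damage for a melee attack and three skills, using stats loaded from a DataTable row at BeginPlay.
; ApplyDamage selects the stat struct for the skill type, and SwitchDamage applies it as point or radial damage.
; Damage is a random integer between min and max.
; The critical check appears inverted: the multiplier applies when the roll exceeds the critical chance.
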(event `self.ReceiveBeginPlay`
  (bind _returnvalue (`|GetDataTableRow` (`self.Data Table`) "Stats_1")
    (:`then`
      (bind (`_mélee` _skill_1 _skill_2 _skill_3) (break `/Game/Blueprints/Gameplay/ActorComponents/Damage/S_Damage_Player` _returnvalue))
      (set `self.S_Attack_Skill_Melee` `_mélee`)
      (set `self.S_Attack_Skill_1` _skill_1)
      (set `self.S_Attack_Skill_2` _skill_2)
      (set `self.S_Attack_Skill_3` _skill_3)
      (set `self.Structure_Attack_Base` (`self.S_Attack_Skill_Melee`)))))

(event `Apply Damage`
  (params (`Type Damage` :type "/Game/Blueprints/Gameplay/ActorComponents/Damage/Type_Damage Enum" :default "NewEnumerator4") (`Type Skill` :type "/Game/Blueprints/Gameplay/ActorComponents/Damage/Type_Skill Enum" :default "NewEnumerator0") (DamagedActor :type "Actor Object Reference") (HitFromDirection :type "Vector Structure (by ref)") (HitInfo :type "HitResult Structure (by ref)") (Origin :type "Vector Structure (by ref)") (DamageRadius :type "Float (double-precision)") (DamageCauser :type "Actor Object Reference"))
  (bind _output_get (set `self.Type Skill` `Type Skill`))
  (switch `/Game/Blueprints/Gameplay/ActorComponents/Damage/Type_Skill` _output_get
    (:`NewEnumerator0`
      (bind _output_get_2 (set `self.Structure_Attack_Base` (`self.S_Attack_Skill_Melee`)))
      (`self.Switch Damage` DamagedActor _output_get_2 `Type Damage` HitFromDirection HitInfo Origin DamageRadius DamageCauser))
    (:`NewEnumerator1`
      (bind _output_get_3 (set `self.Structure_Attack_Base` (`self.S_Attack_Skill_1`)))
      (`self.Switch Damage` DamagedActor _output_get_3 `Type Damage` HitFromDirection HitInfo Origin DamageRadius DamageCauser))
    (:`NewEnumerator2`
      (bind _output_get_4 (set `self.Structure_Attack_Base` (`self.S_Attack_Skill_2`)))
      (`self.Switch Damage` DamagedActor _output_get_4 `Type Damage` HitFromDirection HitInfo Origin DamageRadius DamageCauser))
    (:`NewEnumerator3`
      (bind _output_get_5 (set `self.Structure_Attack_Base` (`self.S_Attack_Skill_3`)))
      (`self.Switch Damage` DamagedActor _output_get_5 `Type Damage` HitFromDirection HitInfo Origin DamageRadius DamageCauser))))

(fn `Switch Damage`
  (params (DamagedActor :type "Actor Object Reference") (Structure_Attack_Base :type "/Game/Blueprints/Gameplay/Datas/S_Attack Structure") (`Type Damage` :type "/Game/Blueprints/Gameplay/ActorComponents/Damage/Type_Damage Enum" :default "NewEnumerator4") (HitFromDirection :type "Vector Structure (by ref)") (HitInfo :type "HitResult Structure (by ref)") (Origin :type "Vector Structure (by ref)") (DamageRadius :type "Float (double-precision)") (DamageCauser :type "Actor Object Reference"))
  (bind (_damagemin _damagemax _chancecritik _coupcritik) (break `/Game/Blueprints/Gameplay/Datas/S_Attack` (`self.Structure_Attack_Base`)))
  (bind _returnvalue (<= (`KismetMathLibrary.RandomFloatInRange` 0.0 100.0) _chancecritik))
  (bind _returnvalue_2 (`KismetMathLibrary.Conv_IntToDouble` (`KismetMathLibrary.RandomIntegerInRange` (`KismetMathLibrary.Round` _damagemin) (`KismetMathLibrary.Round` _damagemax))))
  (bind _returnvalue_3 (* (`KismetMathLibrary.Conv_IntToDouble` (`KismetMathLibrary.RandomIntegerInRange` (`KismetMathLibrary.Round` _damagemin) (`KismetMathLibrary.Round` _damagemax))) _coupcritik))
  (set `self.Structure_Attack_Base` Structure_Attack_Base)
  (bind _output_get (set `self.Type Damage` `Type Damage`))
  (switch `/Game/Blueprints/Gameplay/ActorComponents/Damage/Type_Damage` _output_get
    (:`NewEnumerator4`
      (if _returnvalue
        (`GameplayStatics.ApplyPointDamage` DamagedActor _returnvalue_2 HitFromDirection HitInfo null DamageCauser)
        (else
          (`GameplayStatics.ApplyPointDamage` DamagedActor _returnvalue_3 HitFromDirection HitInfo null DamageCauser))))
    (:`NewEnumerator5`
      (if _returnvalue
        (`GameplayStatics.ApplyRadialDamage` :`BaseDamage` _returnvalue_2 :`Origin` Origin :`DamageRadius` DamageRadius :`DamageCauser` DamageCauser :`InstigatedByController` null :`DamagePreventionChannel` "ECC_Pawn")
        (else
          (`GameplayStatics.ApplyRadialDamage` :`BaseDamage` _returnvalue_3 :`Origin` Origin :`DamageRadius` DamageRadius :`DamageCauser` DamageCauser :`InstigatedByController` null :`DamagePreventionChannel` "ECC_Pawn"))))))