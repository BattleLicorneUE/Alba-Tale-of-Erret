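; Character_Gameplay component that drives a held-input skill through a Skill_Lance_Blob actor.
; Pressing spawns or reuses the blob attached to the owner and opens a Tick gate, which releasing closes.
; While open, a Delay throttles the blob's SpawnActors calls to FireRate, passing the stamina cost.
; A retriggerable delay after each call destroys the blob once firing has been idle for a few seconds.
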(event `self.ReceiveBeginPlay`
  (bind _ascharacter_gameplay (cast `/Game/Blueprints/Gameplay/Character_Gameplay` (`self.GetOwner`)))
  (set `self.Owner` _ascharacter_gameplay))

(event `self.ReceiveTick`
  (params (DeltaSeconds :type "Float (single-precision)"))
  (`/Engine/EditorBlueprintResources/StandardMacros.Gate` true :!label _label
    (:`Exit`
      (`KismetSystemLibrary.Delay` (/ 1.0 (`self.FireRate`)))
      (`/Game/Blueprints/Gameplay/Actors/Skills/Skill_Lance_Blob.Spawn Actors` (`self.Blob`) (`self.Owner`) (`self.Consume Stamina`))
      (`KismetSystemLibrary.RetriggerableDelay` 3.0)
      (`Actor.K2_DestroyActor` (`self.Blob`)))))

(event `Pressed`
  (`self.Spawn Blob `)
  (goto _label :!via `Open`))

(event `Released`
  (goto _label :!via `Close`))

(fn `Spawn Blob `
  (bind _owner (`self.Owner`))
  (`/Engine/EditorBlueprintResources/StandardMacros.IsValid` (`self.Blob`)
    (:`Is Valid`
      _)
    (:`Is Not Valid`
      (bind _returnvalue (`|SpawnActorFromClass` "/Game/Blueprints/Gameplay/Actors/Skills/Skill_Lance_Blob.Skill_Lance_Blob_C" (`KismetMathLibrary.MakeTransform` (`Actor.K2_GetActorLocation` _owner) (`Actor.K2_GetActorRotation` _owner)) "Undefined" "OverrideRootScale" null null null))
      (set `self.Blob` _returnvalue)))
  (`Actor.K2_AttachToActor` (`self.Blob`) (`self.Owner`) "None" "KeepWorld" "KeepWorld" "KeepWorld" true))