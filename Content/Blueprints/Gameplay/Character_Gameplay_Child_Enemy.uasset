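; Enemy character Blueprint that chases a seen Character_Gameplay pawn and attacks it in melee.
; PawnSensing triggers AI MoveTo toward the target, then on success or failure alike it waits a random delay, plays the attack montage and calls ACMelee's Attack.
; Damage reduces Health, and at zero or below it prints a death message, spawns a particle system and destroys the actor.
; Walk speed is applied to CharacterMovement on BeginPlay.
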(event `self.ReceiveBeginPlay`
  (`self.SetSpeed` (`self.Walk Speed`)))

(event `self.ReceiveAnyDamage`
  (params (Damage :type "Float (single-precision)") (DamageType :type "DamageType Object Reference") (InstigatedBy :type "Controller Object Reference") (DamageCauser :type "Actor Object Reference"))
  (bind _output_get (set `self.Health` (- (`self.Health`) Damage)))
  (if (<= _output_get 0.0)
    (`KismetSystemLibrary.PrintString` (`KismetStringLibrary.Concat_StrStr` (`KismetSystemLibrary.GetDisplayName` self) " is Dead"))
    (`NiagaraFunctionLibrary.SpawnSystemAtLocation` (`self.System Template`) (`self.K2_GetActorLocation`))
    (`self.K2_DestroyActor`)))

(event `self.PawnSensing.OnSeePawn`
  (params (Pawn :type "Pawn Object Reference"))
  (bind _ascharacter_gameplay (cast `/Game/Blueprints/Gameplay/Character_Gameplay` Pawn))
  (set `self.Target Character Gameplay` _ascharacter_gameplay)
  (`|AIMoveTo` self (0.0 0.0 0.0) (`self.Target Character Gameplay`) (`self.Acceptance Radius`)
    (:`OnSuccess`
      _)
    (:`OnFail`
      _))
  (`KismetSystemLibrary.Delay` (`KismetMathLibrary.RandomFloatInRange` 1.0 (`self.Delay Before Attack`)))
  (`self.PlayAnimMontage` (`self.Anim Montage Attack`))
  (`/Game/Blueprints/Gameplay/ActorComponents/AC_Melee.Attack` (`self.AC_Melee`)))

(fn `SetSpeed`
  (params (MaxWalkSpeed :type "Float (double-precision)"))
  (set `CharacterMovementComponent.MaxWalkSpeed` MaxWalkSpeed (`self.CharacterMovement`)))

(fn `UserConstructionScript`
  (`parent.UserConstructionScript`))