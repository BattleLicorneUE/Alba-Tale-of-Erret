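; Drinkable potion pickup actor that restores the player's health or stamina, according to its data table potion type.
; BeginPlay loops over all table rows to set mesh, type and amount, so the last row found wins.
; Sphere overlap gates the Use event, which hides the actor and plays a drink montage with the potion in hand.
; Completion applies the restore and destroys the actor, while interruption makes it available again.
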(event `self.ReceiveBeginPlay`
  (bind _datatable (`self.DataTable`))
  (bind _outrownames (`DataTableFunctionLibrary.GetDataTableRowNames` _datatable))
  (for _array_element _outrownames
    (bind _returnvalue (`|GetDataTableRow` _datatable _array_element)
      (:`then`
        (set `self.S_Potion` _returnvalue)
        (bind (_mesh _addconstance) (break `/Game/Blueprints/Gameplay/Datas/Potion/S_Potion` _returnvalue))
        (bind _output_get (set `self.New Mesh` _mesh))
        (`StaticMeshComponent.SetStaticMesh` (`self.Mesh`) _output_get)
        (set `self.Add Constance` _addconstance)))))

(event `self.Sphere.OnComponentBeginOverlap`
  (params (OverlappedComponent :type "PrimitiveComponent Object Reference") (OtherActor :type "Actor Object Reference") (OtherComp :type "PrimitiveComponent Object Reference") (OtherBodyIndex :type Integer) (bFromSweep :type Boolean) (SweepResult :type "HitResult Structure (by ref)"))
  (cast `/Game/Blueprints/Gameplay/Character_Gameplay` OtherActor)
  (set `self.Use?` true))

(event `self.Sphere.OnComponentEndOverlap`
  (params (OverlappedComponent :type "PrimitiveComponent Object Reference") (OtherActor :type "Actor Object Reference") (OtherComp :type "PrimitiveComponent Object Reference") (OtherBodyIndex :type Integer))
  (cast `/Game/Blueprints/Gameplay/Character_Gameplay` OtherActor)
  (set `self.Use?` false))

(event `self.Use`
  (bind _add_constance (`self.Add Constance`))
  (bind _as_character_gameplay (`self.As Character Gameplay`))
  (if (and (`self.CanDrink`) (`self.Use?`))
    (if (not (`SceneComponent.IsVisible` (`self.Sphere`)))
      (set `self.CanDrink` false)
      (`SceneComponent.SetVisibility` (`self.Root`) false true)
      (bind _ascharacter_gameplay (cast `/Game/Blueprints/Gameplay/Character_Gameplay` (`GameplayStatics.GetPlayerCharacter` 0)))
      (bind _output_get (set `self.As Character Gameplay` _ascharacter_gameplay))
      (`|PlayMontage` (`Character.Mesh` _output_get) "/Game/Resources/Animations/Animations_Selected/Animations_Magic/DrinkPotion_Montage.DrinkPotion_Montage" 1.2
        (:`then`
          (bind _ascharacter_gameplay_2 (cast `/Game/Blueprints/Gameplay/Character_Gameplay` (`GameplayStatics.GetPlayerCharacter` 0)))
          (`/Game/Blueprints/Gameplay/Character_Gameplay.Set Drink Potion` _ascharacter_gameplay_2 (`self.New Mesh`)))
        (:`OnCompleted`
          (bind _ascharacter_gameplay_3 (cast `/Game/Blueprints/Gameplay/Character_Gameplay` (`GameplayStatics.GetPlayerCharacter` 0)))
          (`/Game/Blueprints/Gameplay/Character_Gameplay.Clear Object Hand Left` _ascharacter_gameplay_3)
          (switch `/Game/Blueprints/Gameplay/Datas/Potion/Type_Potion` (`.TypePotion_23_E69C65B9433631CDACAD3288DF6E2D57` (break `/Game/Blueprints/Gameplay/Datas/Potion/S_Potion` (`self.S_Potion`)))
            (:`NewEnumerator0`
              (`/Game/Blueprints/Gameplay/ActorComponents/All_Characters/AC_Health.Add Health` (`/Game/Blueprints/Gameplay/Character_Master.AC_Health` _as_character_gameplay) _add_constance))
            (:`NewEnumerator1`
              (`/Game/Blueprints/Gameplay/ActorComponents/Players/AC_Stamina.Add Stamina` (`/Game/Blueprints/Gameplay/Character_Master.AC_Stamina` _as_character_gameplay) _add_constance)))
          (`self.K2_DestroyActor`))
        (:`OnInterrupted`
          (bind _ascharacter_gameplay_4 (cast `/Game/Blueprints/Gameplay/Character_Gameplay` (`GameplayStatics.GetPlayerCharacter` 0)))
          (`/Game/Blueprints/Gameplay/Character_Gameplay.Clear Object Hand Left` _ascharacter_gameplay_4)
          (`SceneComponent.SetVisibility` (`self.Root`) true true)
          (set `self.CanDrink` true)))
      (else
        (`KismetSystemLibrary.PrintString` "Potion Indisponible" :!label _label)))
    (else
      (goto _label))))

(fn `UserConstructionScript`)