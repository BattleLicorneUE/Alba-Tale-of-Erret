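; Trigger actor that marks a border between two sound zones and switches the player's ambient music on crossing.
; When the player character's Sphere enters the TriggerBox, the sound manager's CurrentZone toggles between FirstZoneName and SecondZoneName, defaulting to the first from any other zone.
; AmbiantSound then restarts with the forest or village loop matching the new zone, with debug prints of the changes.
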(event `self.TriggerBox.OnComponentBeginOverlap`
  (params (OverlappedComponent :type "PrimitiveComponent Object Reference") (OtherActor :type "Actor Object Reference") (OtherComp :type "PrimitiveComponent Object Reference") (OtherBodyIndex :type Integer) (bFromSweep :type Boolean) (SweepResult :type "HitResult Structure (by ref)"))
  (bind _returnvalue (`GameplayStatics.GetPlayerCharacter` 0))
  (if (== OtherComp (`/Game/Blueprints/Gameplay/Character_Gameplay.Sphere` (cast `/Game/Blueprints/Gameplay/Character_Gameplay` _returnvalue :!pure true)))
    (bind _ascharacter_gameplay (cast `/Game/Blueprints/Gameplay/Character_Gameplay` _returnvalue))
    (bind _ac_soundmanager (`/Game/Blueprints/Gameplay/Character_Master.AC_SoundManager` _ascharacter_gameplay))
    (bind _currentzone (`/Game/Blueprints/Gameplay/ActorComponents/Players/AC_SoundManager.CurrentZone` _ac_soundmanager))
    (bind _returnvalue_2 (`|EnumEquality` _currentzone (`self.FirstZoneName`)))
    (if (or _returnvalue_2 (`|EnumEquality` _currentzone (`self.SecondZoneName`)))
      (if _returnvalue_2
        (bind _output_get (set `/Game/Blueprints/Gameplay/ActorComponents/Players/AC_SoundManager.CurrentZone` (`self.SecondZoneName`) _ac_soundmanager))
        (`KismetSystemLibrary.PrintString` (`KismetStringLibrary.Concat_StrStr` "The player enters " (`|GetEnumeratorNameAsString` _output_get)))
        (else
          (bind _output_get_2 (set `/Game/Blueprints/Gameplay/ActorComponents/Players/AC_SoundManager.CurrentZone` (`self.FirstZoneName`) _ac_soundmanager :!label _label))
          (`KismetSystemLibrary.PrintString` (`KismetStringLibrary.Concat_StrStr` "The player enters " (`|GetEnumeratorNameAsString` _output_get_2)))))
      (else
        (goto _label)))
    (bind _ambiantsound (`/Game/Blueprints/Gameplay/Character_Gameplay.AmbiantSound` _ascharacter_gameplay))
    (`AudioComponent.Stop` _ambiantsound)
    (switch `/Game/Sounds/E_ZoneNames` (`/Game/Blueprints/Gameplay/ActorComponents/Players/AC_SoundManager.CurrentZone` _ac_soundmanager)
      (:`NewEnumerator0`
        (`AudioComponent.SetSound` _ambiantsound "/Game/Sounds/Music/Music_Forest_Loop.Music_Forest_Loop")
        (bind _returnvalue_3 (`KismetSystemLibrary.GetDisplayName` _ambiantsound))
        (`KismetSystemLibrary.PrintString` _returnvalue_3))
      (:`NewEnumerator1`
        (`AudioComponent.SetSound` _ambiantsound "/Game/Sounds/Music/Music_Village_Loop.Music_Village_Loop")
        (`KismetSystemLibrary.PrintString` _returnvalue_3)))
    (`AudioComponent.Play` _ambiantsound 0.0)))

(fn `UserConstructionScript`)