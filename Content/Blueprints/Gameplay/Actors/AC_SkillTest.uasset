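; AC_SkillTest is a spawned skill actor that performs a delayed melee-style hit in front of its instigator.
; On BeginPlay it plays a random mesh animation, attaches to the instigator's RootSocket, and destroys itself after a delay.
; In parallel, a delayed forward box trace for pawns, ignoring player 0, applies damage, spawns hit Niagara FX and increments the instigator's ACMelee combo.
; The explosion FX spawn is disconnected.
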(event `self.ReceiveBeginPlay`
  (bind _returnvalue (`self.K2_GetActorRotation`))
  (bind _returnvalue_2 (`self.K2_GetActorLocation`))
  (bind _returnvalue_3 (`KismetMathLibrary.GetForwardVector` _returnvalue))
  (`self.Play Animation` (`self.SetRandomAnimation`))
  (`self.K2_AttachToActor` (`self.Instigator`) "RootSocket" "KeepWorld" "SnapToTarget" "KeepRelative")
  (`|ExecutionSequence`
    (:`then_0`
      (`KismetSystemLibrary.Delay` (`self.DelayBeforeDestroy`))
      (`self.K2_DestroyActor`))
    (:`then_1`
      (`KismetSystemLibrary.Delay` (`self.DelayBeforeHit`))
      (bind (_outhit _returnvalue_4) (`KismetSystemLibrary.BoxTraceSingleForObjects` (+ _returnvalue_2 (* _returnvalue_3 (`self.SpellStartOffset`))) (+ _returnvalue_2 (* _returnvalue_3 (`self.SpellEndOffset`))) (`self.SpellHitSize`) _returnvalue (`|MakeArray` "ObjectTypeQuery3" :!type "EObjectTypeQuery Enum") false (`|MakeArray` (`GameplayStatics.GetPlayerCharacter` 0) :!type "Actor Object Reference") "ForDuration"))
      (if _returnvalue_4
        (bind (_bblockinghit _binitialoverlap _time _distance _location _impactpoint _normal _impactnormal _physmat _hitactor) (`GameplayStatics.BreakHitResult` _outhit))
        (`GameplayStatics.ApplyDamage` _hitactor (`self.SpellDamages`))
        (`NiagaraFunctionLibrary.SpawnSystemAtLocation` "/Game/Blueprints/Gameplay/Particles/NA_Hit_System.NA_Hit_System" _impactpoint)
        (`/Game/Blueprints/Gameplay/ActorComponents/AC_Melee.IncrementCombo` (`/Game/Blueprints/Gameplay/Character_Master.AC_Melee` (cast `/Game/Blueprints/Gameplay/Character_Master` (`self.Instigator`) :!pure true)))))))

(fn `SetRandomAnimation`
  (returns (Output :type "AnimSequence Object Reference"))
  (bind _animations (`self.Animations`))
  (return (`|GetArrayItem` _animations (`KismetMathLibrary.RandomInteger` (- (`KismetArrayLibrary.Array_Length` _animations) 1)))))

(fn `UserConstructionScript`)