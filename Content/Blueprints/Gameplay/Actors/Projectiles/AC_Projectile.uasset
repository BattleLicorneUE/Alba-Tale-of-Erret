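; Homing projectile actor that deals fixed damage to any actor overlapping its sphere.
; On spawn, a looping timer polls until Target is valid, then sets the target's mesh as the ProjectileMovement homing component and stops.
; When the projectile stops, it spawns an impact effect and force feedback at the hit location, shakes the first player's camera and destroys itself.
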(event `self.ReceiveBeginPlay`
  (bind _returnvalue (`KismetSystemLibrary.K2_SetTimerDelegate` (delegate `SetHomingTarget`) 0.1 true)))

(event `SetHomingTarget`
  (bind _target (`self.Target`))
  (`/Engine/EditorBlueprintResources/StandardMacros.IsValid` _target
    (:`Is Valid`
      (set `ProjectileMovementComponent.HomingTargetComponent` (`Character.Mesh` _target) (`self.ProjectileMovement`))
      (`KismetSystemLibrary.K2_ClearAndInvalidateTimerHandle` (stale `self.ReceiveBeginPlay` _returnvalue)))))

(event `self.Sphere.OnComponentBeginOverlap`
  (params (OverlappedComponent :type "PrimitiveComponent Object Reference") (OtherActor :type "Actor Object Reference") (OtherComp :type "PrimitiveComponent Object Reference") (OtherBodyIndex :type Integer) (bFromSweep :type Boolean) (SweepResult :type "HitResult Structure (by ref)"))
  (`GameplayStatics.ApplyDamage` OtherActor 50.0))

(event `self.ProjectileMovement.OnProjectileStop`
  (params (ImpactResult :type "HitResult Structure (by ref)"))
  (bind (_bblockinghit _binitialoverlap _time _distance _location _impactpoint) (`GameplayStatics.BreakHitResult` ImpactResult))
  (`NiagaraFunctionLibrary.SpawnSystemAtLocation` "/Game/Blueprints/Gameplay/Particles/Systems/ImpactLight.ImpactLight" _location (`KismetMathLibrary.Conv_VectorToRotator` _impactpoint))
  (`GameplayStatics.SpawnForceFeedbackAtLocation` "/Game/Blueprints/Gameplay/Feelback/Impact.Impact" _location (struct) false 1.0 0.0 null)
  (`PlayerController.ClientStartCameraShake` :`self` (`GameplayStatics.GetPlayerController` 0) :`Shake` "/Game/Blueprints/Gameplay/Feelback/AC_SequenceAnimationCameraShakeImpact_Zone.AC_SequenceAnimationCameraShakeImpact_Zone_C")
  (`self.K2_DestroyActor`))

(fn `UserConstructionScript`)