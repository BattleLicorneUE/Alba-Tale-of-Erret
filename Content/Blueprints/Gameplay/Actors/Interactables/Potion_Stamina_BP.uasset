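; Stamina potion pickup that adds a stamina potion to the player character's inventory when used.
; On BeginPlay it caches the player and loops through every DataTable row, so the last row found sets its mesh and AddConstance value.
; A sphere overlap with the gameplay character toggles a Use flag.
; The Use event checks that flag, adds the potion, plays a 2D sound and destroys the actor after a short delay.
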(event `self.ReceiveBeginPlay`
  (bind _datatable (`self.DataTable`))
  (bind _ascharacter_gameplay (cast `/Game/Blueprints/Gameplay/Character_Gameplay` (`GameplayStatics.GetPlayerCharacter` 0)))
  (set `self.As Character Gameplay` _ascharacter_gameplay)
  (bind _outrownames (`DataTableFunctionLibrary.GetDataTableRowNames` _datatable))
  (for _array_element _outrownames
    (bind _returnvalue (`|GetDataTableRow` _datatable _array_element)
      (:`then`
        (set `self.S_Potion` _returnvalue)
        (bind (_mesh _addconstance) (break `/Game/Blueprints/Gameplay/Datas/Potion/S_Potion` _returnvalue))
        (bind _output_get (set `self.New Mesh` _mesh))
        (`StaticMeshComponent.SetStaticMesh` (`self.Mesh`) _output_get)
        (set `self.Add Constance` _addconstance)))))

(event `self.Sphere.OnComponentBeginOverlap`
  (params (OverlappedComponent :type "PrimitiveComponent Object Reference") (OtherActor :type "Actor Object Reference") (OtherComp :type "PrimitiveComponent Object Reference") (OtherBodyIndex :type Integer) (bFromSweep :type Boolean) (SweepResult :type "HitResult Structure (by ref)"))
  (cast `/Game/Blueprints/Gameplay/Character_Gameplay` OtherActor)
  (set `self.Use?` true))

(event `self.Sphere.OnComponentEndOverlap`
  (params (OverlappedComponent :type "PrimitiveComponent Object Reference") (OtherActor :type "Actor Object Reference") (OtherComp :type "PrimitiveComponent Object Reference") (OtherBodyIndex :type Integer))
  (cast `/Game/Blueprints/Gameplay/Character_Gameplay` OtherActor)
  (set `self.Use?` false))

(event `self.Use`
  (if (`self.Use?`)
    (`/Game/Blueprints/Gameplay/ActorComponents/Players/Ac_Inventory.Add Stamina Potion` (`/Game/Blueprints/Gameplay/Character_Gameplay.Ac_Inventory` (`self.As Character Gameplay`)))
    (`GameplayStatics.PlaySound2D` (`self.Sound Add Potion`) 1.0 1.0 0.0 null null)
    (`KismetSystemLibrary.Delay` 0.1)
    (`self.K2_DestroyActor`)))

(fn `UserConstructionScript`)