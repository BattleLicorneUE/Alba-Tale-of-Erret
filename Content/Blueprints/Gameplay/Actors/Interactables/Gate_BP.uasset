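; Interactable gate that fades the screen out when used and can swing open or closed.
; Use calls the player controller's input toggle with false, holds a camera fade and hides its widget, while a parallel delay leads to no further action.
; OpenDoor and CloseDoor play a timeline forward or in reverse to drive the pivot's yaw.
; ValidQuest is an empty stub.
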(event `self.Use`
  (bind _get_player_controller (`/Game/Blueprints/Gameplay/Library_Blueprints/FunctionLibrary.Get Player Controller`))
  (`|ExecutionSequence`
    (:`then_0`
      (`KismetSystemLibrary.Delay` 2.5))
    (:`then_1`
      (`/Game/Blueprints/Gameplay/PlayerController_Gameplay.Disable or Enable Input` _get_player_controller false)
      (`PlayerCameraManager.StartCameraFade` :`self` (`PlayerController.PlayerCameraManager` _get_player_controller) :`ToAlpha` 1.0 :`Duration` 1.0 :`bHoldWhenFinished` true)
      (`SceneComponent.SetVisibility` (`self.Widget`) false false))))

(event `Open Door`
  (bind (_direction _z) (`Timeline|Play animation` :!via `PlayFromStart` :!label _label)
    (:`Update`
      (`SceneComponent.K2_SetRelativeRotation` (`self.Pivot`) (`KismetMathLibrary.MakeRotator` 0.0 0.0 _z) false false))))

(event `Close Door`
  (goto _label :!via `ReverseFromEnd`))

(fn `UserConstructionScript`
  (`parent.UserConstructionScript`))