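; Interactable gold pickup that grants the player a fixed amount of gold when used.
; Use adds the gold through the player character's money manager component, refreshes the HUD, plays a 2D sound and destroys the actor.
; UpdateGold reaches the interface through the gameplay player controller, makes the gold display visible and triggers its update.
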(event `self.Use`
  (bind _ascharacter_gameplay (cast `/Game/Blueprints/Gameplay/Character_Gameplay` (`GameplayStatics.GetPlayerCharacter` 0)))
  (`/Game/Blueprints/Gameplay/ActorComponents/Players/Ac_ManagerMoney.Add Gold` (`/Game/Blueprints/Gameplay/Character_Gameplay.Ac_ManagerMoney` _ascharacter_gameplay) 30)
  (`self.Update Gold`)
  (`GameplayStatics.PlaySound2D` (`self.Sound Gold `) 1.0 1.0 0.0 null null)
  (`self.K2_DestroyActor`))

(fn `Update Gold`
  (bind _asplayer_controller_gameplay (cast `/Game/Blueprints/Gameplay/PlayerController_Gameplay` (`GameplayStatics.GetPlayerController` 0)))
  (bind _interfaceplayer (`/Game/Blueprints/Gameplay/PlayerController_Gameplay.InterfacePlayer` _asplayer_controller_gameplay))
  (set `/Game/Blueprints/HUD/Player/Interface_Player.Visibity Gold` "Visible" _interfaceplayer)
  (`/Game/Blueprints/HUD/Player/Interface_Player.Play Update Gold` _interfaceplayer))

(fn `UserConstructionScript`
  (`parent.UserConstructionScript`))