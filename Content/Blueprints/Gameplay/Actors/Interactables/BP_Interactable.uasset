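; Interactable actor that shows a prompt while a gameplay character is inside its trigger sphere and fires a one-time interaction on F.
; Overlap toggles the actor's input for that character's controller and adds or removes the message widget, with a DoOnce preventing duplicates.
; The first press sets the Interact flag, readable through HasInteract, and calls EventInteract.
; The construction script applies the configurable trigger radius and mesh.
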(event `self.TriggerZone.OnComponentBeginOverlap`
  (params (OverlappedComponent :type "PrimitiveComponent Object Reference") (OtherActor :type "Actor Object Reference") (OtherComp :type "PrimitiveComponent Object Reference") (OtherBodyIndex :type Integer) (bFromSweep :type Boolean) (SweepResult :type "HitResult Structure (by ref)"))
  (bind _ascharacter_gameplay (cast `/Game/Blueprints/Gameplay/Character_Gameplay` OtherActor))
  (`self.EnableInput` (cast `PlayerController` (`Pawn.GetController` _ascharacter_gameplay) :!pure true))
  (`/Game/Blueprints/Gameplay/Datas/Int_Interactable.OnBeginOverlap`))

(event `self.TriggerZone.OnComponentEndOverlap`
  (params (OverlappedComponent :type "PrimitiveComponent Object Reference") (OtherActor :type "Actor Object Reference") (OtherComp :type "PrimitiveComponent Object Reference") (OtherBodyIndex :type Integer))
  (bind _ascharacter_gameplay (cast `/Game/Blueprints/Gameplay/Character_Gameplay` OtherActor))
  (`self.DisableInput` (cast `PlayerController` (`Pawn.GetController` _ascharacter_gameplay) :!pure true))
  (`/Game/Blueprints/Gameplay/Datas/Int_Interactable.OnEndOverlap`))

(event `Key|F`
  (params (Key :type "Key Structure"))
  (:`Pressed`
    (`/Game/Blueprints/Gameplay/Datas/Int_Interactable.OnInteract`)))

(event `/Game/Blueprints/Gameplay/Datas/Int_Interactable.OnInteract`
  (if (not (`self.Interact?`))
    (set `self.Interact?` true)
    (`self.EventInteract`)))

(event `/Game/Blueprints/Gameplay/Datas/Int_Interactable.OnBeginOverlap`
  (`/Engine/EditorBlueprintResources/StandardMacros.DoOnce` false :!label _label
    (:`Completed`
      (bind _returnvalue (`|CreateWidget` "/Game/Blueprints/HUD/Player/W_InteractMessage.W_InteractMessage_C" (`GameplayStatics.GetPlayerController` 0) (`self.Interact Text`)))
      (bind _output_get (set `self.InteractMessage` _returnvalue))
      (`UserWidget.AddToViewport` _output_get 0))))

(event `/Game/Blueprints/Gameplay/Datas/Int_Interactable.OnEndOverlap`
  (`Widget.RemoveFromParent` (`self.InteractMessage`))
  (goto _label :!via `Reset`))

(fn `HasInteract?`
  (returns (`Interact?` :type Boolean))
  (return (`self.Interact?`)))

(fn `UserConstructionScript`
  (`SphereComponent.SetSphereRadius` (`self.TriggerZone`) (`self.Trigger radius`) true)
  (`StaticMeshComponent.SetStaticMesh` (`self.Mesh`) (`self.Interact Object`)))