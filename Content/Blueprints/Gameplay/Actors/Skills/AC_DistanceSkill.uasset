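; Distance skill actor that attaches to its instigating character, plays an attack montage chosen by that character's distance attack index, and fires a blob projectile.
; A Shoot notify spawns the projectile from the spawn hand, then detaches the actor with a disintegration Niagara effect.
; A Pause notify holds the montage while the character's pause flag is set; a looping timer polls that flag to resume, detach and destroy the actor.
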(event `self.ReceiveBeginPlay`
  (bind _returnvalue (`SkeletalMeshComponent.GetAnimInstance` (`self.SkeletalMesh`)))
  (bind _returnvalue_2 (`KismetSystemLibrary.K2_SetTimerDelegate` (delegate `CheckIsAnimPaused`) 0.3 true))
  (set `self.PauseAnimTimer` _returnvalue_2)
  (`self.K2_AttachToActor` (`self.Instigator`) "None" "KeepWorld" "SnapToTarget" "KeepRelative")
  (bind _notifyname (`|PlayMontage` (`self.SkeletalMesh`) (`|GetArrayItem` (`self.DistSkillAnimations`) (- (`/Game/Blueprints/Gameplay/ActorComponents/AC_Distance.DistAttackIndex` (`/Game/Blueprints/Gameplay/Character_Master.AC_Distance` (cast `/Game/Blueprints/Gameplay/Character_Master` (`self.GetInstigator`) :!pure true))) 1)))
    (:`OnCompleted`
      (`self.Spawn FX `)
      (`self.K2_DestroyActor`))
    (:`OnNotifyBegin`
      (switch `name` _notifyname
        (:`Shoot`
          (`|SpawnActorFromClass` "/Game/Blueprints/Gameplay/Actors/Projectiles/Projectile_Blob.Projectile_Blob_C" (`KismetMathLibrary.MakeTransform` (+ (`SceneComponent.K2_GetComponentLocation` (`self.Spawn Hand`)) (* (`self.GetActorForwardVector`) 10.0)) (`SceneComponent.K2_GetComponentRotation` (`self.DefaultSceneRoot`))) "Undefined" "OverrideRootScale" null (`self.Target`) (`self.Instigator`))
          (`KismetSystemLibrary.K2_ClearAndInvalidateTimerHandle` (`self.PauseAnimTimer`))
          (`self.K2_DetachFromActor` "KeepWorld" "KeepWorld" "KeepWorld")
          (`self.Spawn FX `))
        (:`Pause`
          (if (`/Game/Blueprints/Gameplay/ActorComponents/AC_Distance.bIsAnimPaused` (`/Game/Blueprints/Gameplay/Character_Master.AC_Distance` (cast `/Game/Blueprints/Gameplay/Character_Master` (`self.GetInstigator`) :!pure true)))
            (`AnimInstance.Montage_Pause` _returnvalue (`AnimInstance.GetCurrentActiveMontage` _returnvalue))
            (else
              (`self.K2_DetachFromActor` "KeepWorld" "KeepWorld" "KeepWorld")
              (`self.Spawn FX `))))))))

(event `CheckIsAnimPaused`
  (bind _returnvalue (`SkeletalMeshComponent.GetAnimInstance` (`self.SkeletalMesh`)))
  (if (not (`/Game/Blueprints/Gameplay/ActorComponents/AC_Distance.bIsAnimPaused` (`/Game/Blueprints/Gameplay/Character_Master.AC_Distance` (cast `/Game/Blueprints/Gameplay/Character_Master` (`self.GetInstigator`) :!pure true))))
    (`AnimInstance.Montage_Resume` _returnvalue (`AnimInstance.GetCurrentActiveMontage` _returnvalue))
    (`self.K2_DetachFromActor` "KeepWorld" "KeepWorld" "KeepWorld")
    (`self.Spawn FX `)
    (`KismetSystemLibrary.Delay` 1.0)
    (`self.K2_DestroyActor`)))

(fn `Spawn FX `
  (bind _skeletalmesh (`self.SkeletalMesh`))
  (bind _niagara_spawner (`self.Niagara_Spawner`))
  (`NiagaraFunctionLibrary.SpawnSystemAttached` "/Game/Blueprints/Gameplay/Particles/SkeletonMesh_FX/FX_SketetonMeshDinistegration.FX_SketetonMeshDinistegration" _skeletalmesh "None" (`SceneComponent.K2_GetComponentLocation` _skeletalmesh) (`SceneComponent.K2_GetComponentRotation` _skeletalmesh) "KeepRelativeOffset" true)
  (`/Engine/EditorBlueprintResources/StandardMacros.IsValid` _niagara_spawner
    (:`Is Valid`
      (`ActorComponent.K2_DestroyComponent` _niagara_spawner))))

(fn `UserConstructionScript`)