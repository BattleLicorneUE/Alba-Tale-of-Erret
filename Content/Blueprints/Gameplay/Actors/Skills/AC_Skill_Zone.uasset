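; Zone skill actor that plays an attack montage on its skeletal mesh and fires a Projectile_Zone, then destroys itself after the montage's length.
; On BeginPlay it caches the player character and camera boom, then briefly attaches to the player and detaches, keeping world location and rotation.
; A montage notify runs a debug-drawn path prediction along OriginShoot's right vector and spawns the projectile facing the predicted hit.
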(event `self.ReceiveBeginPlay`
  (bind _ascharacter_gameplay (cast `/Game/Blueprints/Gameplay/Character_Gameplay` (`GameplayStatics.GetPlayerCharacter` 0)))
  (set `self.As Character Gameplay` _ascharacter_gameplay)
  (set `self.camera` (`/Game/Blueprints/Gameplay/Character_Gameplay.CameraBoom` _ascharacter_gameplay))
  (`self.Launch Attack`))

(event `Launch Attack`
  (bind _montage_to_play (`self.Montage to Play`))
  (`self.Attack And Detach Actor`)
  (bind _notifyname (`|PlayMontage` (`self.SkeletalMesh`) _montage_to_play)
    (:`then`
      (`KismetSystemLibrary.Delay` (`AnimSequenceBase.SequenceLength` _montage_to_play))
      (`self.K2_DestroyActor`))
    (:`OnNotifyBegin`
      (switch `name` _notifyname
        (:`Hit`
          (`self.ProjectileCast`))))))

(fn `Attack And Detach Actor`
  (`self.K2_AttachToActor` (`self.As Character Gameplay`) "RootSocket" "KeepWorld" "KeepWorld" "KeepRelative")
  (`self.K2_DetachFromActor` "KeepWorld" "KeepWorld" "KeepWorld"))

(fn `ProjectileCast`
  (bind _originshoot (`self.OriginShoot`))
  (bind _returnvalue (`SceneComponent.K2_GetComponentLocation` (`self.OriginShoot`)))
  (bind _outhit (`GameplayStatics.Blueprint_PredictProjectilePath_ByTraceChannel` (`SceneComponent.K2_GetComponentLocation` _originshoot) (* (`KismetMathLibrary.GetRightVector` (`SceneComponent.K2_GetComponentRotation` _originshoot)) (`self.Launch Velocity`)) true 30.0 "ECC_Visibility" true (`|MakeArray` (`GameplayStatics.GetPlayerCharacter` 0) :!type "Actor Object Reference") "ForDuration" 5.0 1.0))
  (`|SpawnActorFromClass` "/Game/Blueprints/Gameplay/Actors/Skills/Projectile_Zone.Projectile_Zone_C" (`KismetMathLibrary.MakeTransform` _returnvalue (`KismetMathLibrary.FindLookAtRotation` _returnvalue (`.Location` (`GameplayStatics.BreakHitResult` _outhit)))) "AlwaysSpawn" "OverrideRootScale" null null))

(fn `UserConstructionScript`)