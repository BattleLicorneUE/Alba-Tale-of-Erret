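; Short-lived melee skill actor that plays a random animation, snaps to the instigator's RootSocket rotation, then detaches and self-destructs after a delay.
; In parallel, a delayed forward box trace looks for one Pawn, ignoring player 0's character.
; A hit applies point damage, impact VFX, sound, force feedback and camera shake, then increments the instigator's ACMelee combo.
; The random index never selects the last animation in the array.
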(event `self.ReceiveBeginPlay`
  (bind _returnvalue (`self.K2_GetActorRotation`))
  (bind _returnvalue_2 (`self.K2_GetActorLocation`))
  (bind _returnvalue_3 (`KismetMathLibrary.GetForwardVector` _returnvalue))
  (`self.Play Animation` (`self.SetRandomAnimation`))
  (`self.K2_AttachToActor` (`self.Instigator`) "RootSocket" "KeepWorld" "SnapToTarget" "KeepRelative")
  (`self.K2_DetachFromActor` "KeepWorld" "KeepWorld" "KeepWorld")
  (`|ExecutionSequence`
    (:`then_0`
      (`KismetSystemLibrary.Delay` (`self.DelayBeforeDestroy`))
      (`self.K2_DestroyActor`))
    (:`then_1`
      (`KismetSystemLibrary.Delay` (`self.DelayBeforeHit`))
      (bind (_outhit _returnvalue_4) (`KismetSystemLibrary.BoxTraceSingleForObjects` (+ _returnvalue_2 (* _returnvalue_3 (`self.SpellStartOffset`))) (+ _returnvalue_2 (* _returnvalue_3 (`self.SpellEndOffset`))) (`self.SpellHitSize`) _returnvalue (`|MakeArray` "ObjectTypeQuery3" :!type "EObjectTypeQuery Enum") false (`|MakeArray` (`GameplayStatics.GetPlayerCharacter` 0) :!type "Actor Object Reference")))
      (if _returnvalue_4
        (bind (_bblockinghit _binitialoverlap _time _distance _location _impactpoint _normal _impactnormal _physmat _hitactor _hitcomponent _hitbonename _hititem _faceindex _tracestart _traceend) (`GameplayStatics.BreakHitResult` _outhit))
        (`GameplayStatics.ApplyPointDamage` _hitactor (`self.SpellDamages`) _traceend _outhit)
        (`NiagaraFunctionLibrary.SpawnSystemAtLocation` "/Game/Blueprints/Gameplay/Particles/Systems/FX_Impact.FX_Impact" _impactpoint)
        (`GameplayStatics.PlaySoundAtLocation` "/Game/Sounds/SFX/Hits/Hit_Blob.Hit_Blob" _impactpoint (struct) 1.0 1.0 0.0 null null null)
        (`GameplayStatics.SpawnForceFeedbackAtLocation` "/Game/Blueprints/Gameplay/Feelback/Impact.Impact" _impactpoint (struct) false 1.0 0.0 null)
        (`PlayerController.ClientStartCameraShake` :`self` (`GameplayStatics.GetPlayerController` 0) :`Shake` "/Game/Blueprints/Gameplay/Feelback/AC_SequenceAnimationCameraShakeImpact_Light.AC_SequenceAnimationCameraShakeImpact_Light_C")
        (`/Game/Blueprints/Gameplay/ActorComponents/AC_Melee.IncrementCombo` (`/Game/Blueprints/Gameplay/Character_Master.AC_Melee` (cast `/Game/Blueprints/Gameplay/Character_Master` (`self.Instigator`) :!pure true)))))))

(fn `SetRandomAnimation`
  (returns (Output :type "AnimSequence Object Reference"))
  (bind _animations (`self.Animations`))
  (return (`|GetArrayItem` _animations (`KismetMathLibrary.RandomInteger` (- (`KismetArrayLibrary.Array_Length` _animations) 1)))))

(fn `UserConstructionScript`)