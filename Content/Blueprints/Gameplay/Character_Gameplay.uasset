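; Player character Blueprint for an action RPG, tying camera lock-on, stamina, health, quest and dialogue systems together.
; Double-tapped direction keys spend stamina to dash when locked on or roll otherwise.
; Overlap volumes feed enemy lists and interactions, while a timed water trace toggles Flying movement for swimming.
; It also handles dialogue UI, hit flashes, death teleport-respawn, kill-count slow motion, item slots and quest debug keys.
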(event `StartDialog`
  (params (AssetToStart :type "DlgDialogue Object Reference"))
  (bind _returnvalue (`GameplayStatics.GetPlayerController` 0))
  ;[1 1 1] Switch to Dialog mode
  (`KismetSystemLibrary.PrintString` "Start Dialogue")
  (bind _returnvalue_2 (`DlgManager.StartDialogueWithDefaultAttendees` AssetToStart))
  (`/Engine/EditorBlueprintResources/StandardMacros.IsValid` _returnvalue_2
    (:`Is Valid`
      (bind _output_get (set `self.ActiveContext` _returnvalue_2))
      (`/Game/Blueprints/HUD/AI/UI_Dialog.Refresh` (`self.DialogWidget`) _output_get)
      (`WidgetBlueprintLibrary.SetInputMode_GameAndUIEx` _returnvalue null "DoNotLock" false)
      (set `PlayerController.bShowMouseCursor` true _returnvalue)
      (`self.DisableInput` _returnvalue))))

(event `SelectDialogOption`
  (params (OptionIndex :type Integer))
  (bind _returnvalue (`GameplayStatics.GetPlayerController` 0))
  (bind _activecontext (`self.ActiveContext`))
  ;[1 1 1] An option has been selected
  (`/Engine/EditorBlueprintResources/StandardMacros.IsValid` _activecontext
    (:`Is Valid`
      (bind _returnvalue_2 (`DlgContext.ChooseOption` _activecontext OptionIndex))
      (if _returnvalue_2
        ;;[1 1 1] UI has to be Refreshed - dialog still active
        (`/Game/Blueprints/HUD/AI/UI_Dialog.Refresh` (`self.DialogWidget`) (`self.ActiveContext`))
        (else
          ;;[1 1 1] Hide UI when dialog is done and give the game full control back
          (`/Game/Blueprints/HUD/AI/UI_Dialog.Refresh` (`self.DialogWidget`) null)
          (`WidgetBlueprintLibrary.SetInputMode_GameOnly` _returnvalue)
          (set `PlayerController.bShowMouseCursor` false _returnvalue)
          (`self.EnableInput` _returnvalue))))))

(event `self.ReceiveBeginPlay`
  ;[1 1 1] Begin play
  (`|ExecutionSequence`
    (:`then_0`
      ;[1 1 1] Event BeginPlay - Widget Initialisation
      (bind _returnvalue (`|CreateWidget` "/Game/Blueprints/HUD/AI/UI_Dialog.UI_Dialog_C" (`GameplayStatics.GetPlayerController` 0)))
      (bind _output_get (set `self.DialogWidget` _returnvalue))
      (`UserWidget.AddToViewport` _output_get 0)
      (`Widget.SetVisibility` (`self.DialogWidget`) "Collapsed"))
    (:`then_1`
      (`self.Choice animation Begin play`)
      (`self.Init Player Controller`))
    (:`then_2`
      (`KismetSystemLibrary.K2_SetTimer` null "SwimDetector" 0.03 true))))

(event `Key|Z` :consume false
  (params (Key :type "Key Structure"))
  ;[1 1 1] Dash and Roll System
  (:`Pressed`
    (if (not (`self.Rolling?`))
      (bind _doubletap_ (`self.CheckDoubleTapInDirection` "Forward"))
      (if _doubletap_
        (if (`/Game/Blueprints/Gameplay/ActorComponents/Players/AC_Camera.Lock?` (`self.AC_Camera`))
          (bind _returnvalue (`/Game/Blueprints/Gameplay/ActorComponents/Players/AC_Stamina.Check Stamina` (`self.AC_Stamina`) (`self.DashCost`)))
          (if _returnvalue
            (`self.PlayAnimMontage` "/Game/Resources/Animations/Frank_RPG_GreatSword/Animations/IP+RM/Frank_RPG_GreatSword_Step_F_Montage.Frank_RPG_GreatSword_Step_F_Montage")
            (`/Game/Blueprints/Gameplay/ActorComponents/Players/AC_Stamina.Consume Stamina` (`self.AC_Stamina`) (`self.DashCost`))
            (`self.LaunchCharacter` (0.0 1000.0 0.0) true))
          (else
            (bind _returnvalue_2 (`/Game/Blueprints/Gameplay/ActorComponents/Players/AC_Stamina.Check Stamina` (`self.AC_Stamina`) (`self.RollCost`)))
            (if _returnvalue_2
              (set `self.Rolling?` true)
              (bind _returnvalue_3 (`self.PlayAnimMontage` "/Game/Resources/Animations/Frank_RPG_GreatSword/Animations/IP+RM/Frank_RPG_GreatSword_Evade_F_Montage.Frank_RPG_GreatSword_Evade_F_Montage"))
              (`/Game/Blueprints/Gameplay/ActorComponents/Players/AC_Stamina.Consume Stamina` (`self.AC_Stamina`) (`self.RollCost`))
              (`KismetSystemLibrary.RetriggerableDelay` _returnvalue_3)
              (set `self.Rolling?` false))))
        (else
          (`KismetSystemLibrary.Delay` 0.2)
          (set `self.Fint` 0))))))

(event `Key|Q` :consume false
  (params (Key :type "Key Structure"))
  ;[1 1 1] Dash and Roll System
  (:`Pressed`
    (if (not (`self.Rolling?`))
      (bind _doubletap_ (`self.CheckDoubleTapInDirection` "Left"))
      (if _doubletap_
        (if (`/Game/Blueprints/Gameplay/ActorComponents/Players/AC_Camera.Lock?` (`self.AC_Camera`))
          (bind _returnvalue (`/Game/Blueprints/Gameplay/ActorComponents/Players/AC_Stamina.Check Stamina` (`self.AC_Stamina`) (`self.DashCost`)))
          (if _returnvalue
            (`self.PlayAnimMontage` "/Game/Resources/Animations/Frank_RPG_GreatSword/Animations/IP+RM/Frank_RPG_GreatSword_Step_L_Montage.Frank_RPG_GreatSword_Step_L_Montage")
            (`/Game/Blueprints/Gameplay/ActorComponents/Players/AC_Stamina.Consume Stamina` (`self.AC_Stamina`) (`self.DashCost`)))
          (else
            (bind _returnvalue_2 (`/Game/Blueprints/Gameplay/ActorComponents/Players/AC_Stamina.Check Stamina` (`self.AC_Stamina`) (`self.RollCost`)))
            (if _returnvalue_2
              (set `self.Rolling?` true)
              (bind _returnvalue_3 (`self.PlayAnimMontage` "/Game/Resources/Animations/Frank_RPG_GreatSword/Animations/IP+RM/Frank_RPG_GreatSword_Evade_L_Montage.Frank_RPG_GreatSword_Evade_L_Montage"))
              (`/Game/Blueprints/Gameplay/ActorComponents/Players/AC_Stamina.Consume Stamina` (`self.AC_Stamina`) (`self.RollCost`))
              (`KismetSystemLibrary.RetriggerableDelay` _returnvalue_3)
              (set `self.Rolling?` false))))
        (else
          (`KismetSystemLibrary.Delay` 0.2)
          (set `self.Lint` 0))))))

(event `Key|S` :consume false
  (params (Key :type "Key Structure"))
  ;[1 1 1] Dash and Roll System
  (:`Pressed`
    (if (not (`self.Rolling?`))
      (bind _doubletap_ (`self.CheckDoubleTapInDirection` "Backward"))
      (if _doubletap_
        (if (`/Game/Blueprints/Gameplay/ActorComponents/Players/AC_Camera.Lock?` (`self.AC_Camera`))
          (bind _returnvalue (`/Game/Blueprints/Gameplay/ActorComponents/Players/AC_Stamina.Check Stamina` (`self.AC_Stamina`) (`self.DashCost`)))
          (if _returnvalue
            (`self.PlayAnimMontage` "/Game/Resources/Animations/Frank_RPG_GreatSword/Animations/IP+RM/Frank_RPG_GreatSword_Step_B_Montage.Frank_RPG_GreatSword_Step_B_Montage")
            (`/Game/Blueprints/Gameplay/ActorComponents/Players/AC_Stamina.Consume Stamina` (`self.AC_Stamina`) (`self.DashCost`)))
          (else
            (bind _returnvalue_2 (`/Game/Blueprints/Gameplay/ActorComponents/Players/AC_Stamina.Check Stamina` (`self.AC_Stamina`) (`self.RollCost`)))
            (if _returnvalue_2
              (set `self.Rolling?` true)
              (bind _returnvalue_3 (`self.PlayAnimMontage` "/Game/Resources/Animations/Frank_RPG_GreatSword/Animations/IP+RM/Frank_RPG_GreatSword_Evade_B_Montage.Frank_RPG_GreatSword_Evade_B_Montage"))
              (`/Game/Blueprints/Gameplay/ActorComponents/Players/AC_Stamina.Consume Stamina` (`self.AC_Stamina`) (`self.RollCost`))
              (`KismetSystemLibrary.RetriggerableDelay` _returnvalue_3)
              (set `self.Rolling?` false))))
        (else
          (`KismetSystemLibrary.Delay` 0.2)
          (set `self.Bint` 0))))))

(event `Key|D` :consume false
  (params (Key :type "Key Structure"))
  ;[1 1 1] Dash and Roll System
  (:`Pressed`
    (if (not (`self.Rolling?`))
      (bind _doubletap_ (`self.CheckDoubleTapInDirection` "Right"))
      (if _doubletap_
        (if (`/Game/Blueprints/Gameplay/ActorComponents/Players/AC_Camera.Lock?` (`self.AC_Camera`))
          (bind _returnvalue (`/Game/Blueprints/Gameplay/ActorComponents/Players/AC_Stamina.Check Stamina` (`self.AC_Stamina`) (`self.DashCost`)))
          (if _returnvalue
            (`self.PlayAnimMontage` "/Game/Resources/Animations/Frank_RPG_GreatSword/Animations/IP+RM/Frank_RPG_GreatSword_Step_R_Montage.Frank_RPG_GreatSword_Step_R_Montage")
            (`/Game/Blueprints/Gameplay/ActorComponents/Players/AC_Stamina.Consume Stamina` (`self.AC_Stamina`) (`self.DashCost`)))
          (else
            (bind _returnvalue_2 (`/Game/Blueprints/Gameplay/ActorComponents/Players/AC_Stamina.Check Stamina` (`self.AC_Stamina`) (`self.RollCost`)))
            (if _returnvalue_2
              (set `self.Rolling?` true)
              (bind _returnvalue_3 (`self.PlayAnimMontage` "/Game/Resources/Animations/Frank_RPG_GreatSword/Animations/IP+RM/Frank_RPG_GreatSword_Evade_R_Montage.Frank_RPG_GreatSword_Evade_R_Montage"))
              (`/Game/Blueprints/Gameplay/ActorComponents/Players/AC_Stamina.Consume Stamina` (`self.AC_Stamina`) (`self.RollCost`))
              (`KismetSystemLibrary.RetriggerableDelay` _returnvalue_3)
              (set `self.Rolling?` false))))
        (else
          (`KismetSystemLibrary.Delay` 0.2)
          (set `self.Rint` 0))))))

(event `self.Detection_Sound.OnComponentBeginOverlap`
  (params (OverlappedComponent :type "PrimitiveComponent Object Reference") (OtherActor :type "Actor Object Reference") (OtherComp :type "PrimitiveComponent Object Reference") (OtherBodyIndex :type Integer) (bFromSweep :type Boolean) (SweepResult :type "HitResult Structure (by ref)"))
  ;[1 1 1] Detection Sounds
  (`self.AddSoundEnemy` OtherActor))

(event `self.Detection_Sound.OnComponentEndOverlap`
  (params (OverlappedComponent :type "PrimitiveComponent Object Reference") (OtherActor :type "Actor Object Reference") (OtherComp :type "PrimitiveComponent Object Reference") (OtherBodyIndex :type Integer))
  ;[1 1 1] Detection Sounds
  (`self.RemoveSoundEnemy` OtherActor))

(event `self.Detection_AI.OnComponentBeginOverlap`
  (params (OverlappedComponent :type "PrimitiveComponent Object Reference") (OtherActor :type "Actor Object Reference") (OtherComp :type "PrimitiveComponent Object Reference") (OtherBodyIndex :type Integer) (bFromSweep :type Boolean) (SweepResult :type "HitResult Structure (by ref)"))
  ;[1 1 1] Add and Remove Array Enemies
  (bind _ascharacter_gameplay_master_enemy (cast `/Game/Blueprints/Gameplay/IntelligenceArticiel/Master/Character_Gameplay_Master_Enemy` OtherActor))
  (`/Game/Blueprints/Gameplay/ActorComponents/Players/AC_Camera.Add Array Ennemies` (`self.AC_Camera`) _ascharacter_gameplay_master_enemy))

(event `self.Detection_AI.OnComponentEndOverlap`
  (params (OverlappedComponent :type "PrimitiveComponent Object Reference") (OtherActor :type "Actor Object Reference") (OtherComp :type "PrimitiveComponent Object Reference") (OtherBodyIndex :type Integer))
  ;[1 1 1] Add and Remove Array Enemies
  (bind _ascharacter_gameplay_master_enemy (cast `/Game/Blueprints/Gameplay/IntelligenceArticiel/Master/Character_Gameplay_Master_Enemy` OtherActor))
  (`/Game/Blueprints/Gameplay/ActorComponents/Players/AC_Camera.Remove Array Ennemies` (`self.AC_Camera`) _ascharacter_gameplay_master_enemy))

(event `self.Detection AutoLock.OnComponentBeginOverlap`
  (params (OverlappedComponent :type "PrimitiveComponent Object Reference") (OtherActor :type "Actor Object Reference") (OtherComp :type "PrimitiveComponent Object Reference") (OtherBodyIndex :type Integer) (bFromSweep :type Boolean) (SweepResult :type "HitResult Structure (by ref)"))
  ;[1 1 1] Add and Remove Array Enemies
  (bind _ascharacter_gameplay_master_enemy (cast `/Game/Blueprints/Gameplay/IntelligenceArticiel/Master/Character_Gameplay_Master_Enemy` OtherActor))
  (`/Game/Blueprints/Gameplay/ActorComponents/Players/AC_Camera.Add Array Ennemies AutoLock` (`self.AC_Camera`) _ascharacter_gameplay_master_enemy))

(event `self.Detection AutoLock.OnComponentEndOverlap`
  (params (OverlappedComponent :type "PrimitiveComponent Object Reference") (OtherActor :type "Actor Object Reference") (OtherComp :type "PrimitiveComponent Object Reference") (OtherBodyIndex :type Integer))
  ;[1 1 1] Add and Remove Array Enemies
  (bind _ascharacter_gameplay_master_enemy (cast `/Game/Blueprints/Gameplay/IntelligenceArticiel/Master/Character_Gameplay_Master_Enemy` OtherActor))
  (`/Game/Blueprints/Gameplay/ActorComponents/Players/AC_Camera.Remove Array Ennemies AutoLock` (`self.AC_Camera`) _ascharacter_gameplay_master_enemy))

(event `self.InteractionCapsule.OnComponentBeginOverlap`
  (params (OverlappedComponent :type "PrimitiveComponent Object Reference") (OtherActor :type "Actor Object Reference") (OtherComp :type "PrimitiveComponent Object Reference") (OtherBodyIndex :type Integer) (bFromSweep :type Boolean) (SweepResult :type "HitResult Structure (by ref)"))
  ;[1 1 1] Begin/End Overlap interaction
  (if (`KismetSystemLibrary.DoesImplementInterface` OtherActor "/Game/Blueprints/QuestBP/Blueprints/I_Interactable.I_Interactable_C")
    (message `/Game/Blueprints/QuestBP/Blueprints/I_Interactable.OnEnterPlayerRadius` OtherActor self)))

(event `self.InteractionCapsule.OnComponentEndOverlap`
  (params (OverlappedComponent :type "PrimitiveComponent Object Reference") (OtherActor :type "Actor Object Reference") (OtherComp :type "PrimitiveComponent Object Reference") (OtherBodyIndex :type Integer))
  ;[1 1 1] Begin/End Overlap interaction
  (if (`KismetSystemLibrary.DoesImplementInterface` OtherActor "/Game/Blueprints/QuestBP/Blueprints/I_Interactable.I_Interactable_C")
    (message `/Game/Blueprints/QuestBP/Blueprints/I_Interactable.OnLeavePlayerRadius` OtherActor self)))

(event `SwimDetector`
  (bind _returnvalue (`self.K2_GetActorLocation`))
  (bind _isswimming (`self.IsSwimming`))
  (bind _charactermovement (`self.CharacterMovement`))
  (bind _capsulehalfheight (`CapsuleComponent.CapsuleHalfHeight` (`self.CapsuleComponent`)))
  ;[1 1 1] SwimDetection
  (bind (_outhit _returnvalue_2) (`KismetSystemLibrary.LineTraceSingleByProfile` :`Start` (+ _returnvalue (`KismetMathLibrary.MakeVector` 0.0 0.0 _capsulehalfheight)) :`End` (- _returnvalue (`KismetMathLibrary.MakeVector` 0.0 0.0 (* _capsulehalfheight 2.0))) :`ProfileName` "WaterBodyCollision" :`TraceColor` (struct :`R` 0.322837 :`G` 1.0 :`B` 0.990053 :`A` 1.0)))
  (if _returnvalue_2
    (if (<= (`.Distance` (`GameplayStatics.BreakHitResult` _outhit)) _capsulehalfheight)
      (if (not _isswimming)
        (set `self.IsSwimming` true)
        (`CharacterMovementComponent.SetMovementMode` _charactermovement "MOVE_Flying" 0))
      (elif _isswimming
        (set `self.IsSwimming` false)
        (`CharacterMovementComponent.SetMovementMode` _charactermovement "MOVE_Walking" 0)))))

(event `Key|O`
  (params (Key :type "Key Structure"))
  (:`Pressed`
    (`/Game/Blueprints/QuestBP/Blueprints/QuestSystem/Actors/AC_QuestManager.AddNewQuest` (`self.AC_QuestManager`) "/Game/Blueprints/QuestBP/Blueprints/QuestSystem/Actors/QuestActor/Quest_Test_03.Quest_Test_03_C" false)))

(event `Key|LeftAlt`
  (params (Key :type "Key Structure"))
  (bind _returnvalue (`GameplayStatics.GetPlayerController` 0))
  (bind _journal (`/Game/Blueprints/QuestBP/Blueprints/QuestSystem/Widgets/W_MainWidget.Journal` (`/Game/Blueprints/QuestBP/Blueprints/QuestSystem/Actors/AC_QuestManager.MainWidget` (`self.AC_QuestManager`))))
  (:`Pressed`
    (bind _isa (`/Engine/EditorBlueprintResources/StandardMacros.FlipFlop`)
      (:`A`
        _)
      (:`B`
        _))
    (`Widget.SetVisibility` _journal (select `bool` _isa :`false` "Collapsed" :`true` "Visible" :!type "ESlateVisibility Enum"))
    (bind _output_get (set `PlayerController.bShowMouseCursor` _isa _returnvalue))
    (if _output_get
      (`WidgetBlueprintLibrary.SetInputMode_GameAndUIEx` _returnvalue _journal "DoNotLock" false)
      (`/Game/Blueprints/QuestBP/Blueprints/QuestSystem/Actors/AC_QuestManager.OnAction` (`self.AC_QuestManager`) "NewEnumerator9")
      (else
        (`WidgetBlueprintLibrary.SetInputMode_GameOnly` _returnvalue)))))

(event `Key|G`
  (params (Key :type "Key Structure"))
  ;[1 1 1] Debug quest system
  ;;[1 1 1] G to add a quest
  (:`Pressed`
    (`/Game/Blueprints/QuestBP/Blueprints/QuestSystem/Actors/AC_QuestManager.AddNewQuest` (`self.AC_QuestManager`) "/Game/Blueprints/QuestBP/Blueprints/QuestSystem/Actors/QuestActor/Quest_test_01.Quest_test_01_C" true)))

(event `Key|H`
  (params (Key :type "Key Structure"))
  ;[1 1 1] Debug quest system
  ;;[1 1 1] H to add second quest
  (:`Pressed`
    (`/Game/Blueprints/QuestBP/Blueprints/QuestSystem/Actors/AC_QuestManager.AddNewQuest` (`self.AC_QuestManager`) "/Game/Blueprints/QuestBP/Blueprints/QuestSystem/Actors/QuestActor/Quest_Test_02.Quest_Test_02_C" false)))

(event `Key|L`
  (params (Key :type "Key Structure"))
  (bind _mainwidget (`/Game/Blueprints/QuestBP/Blueprints/QuestSystem/Actors/AC_QuestManager.MainWidget` (`self.AC_QuestManager`)))
  (bind _slideout (`/Game/Blueprints/QuestBP/Blueprints/QuestSystem/Widgets/W_MainWidget.SlideOut` _mainwidget))
  ;[1 1 1] Press L to slide in/out quest widget
  (:`Pressed`
    (if (>= (`KismetArrayLibrary.Array_Length` (`/Game/Blueprints/QuestBP/Blueprints/QuestSystem/Widgets/W_MainWidget.QuestWidgets` _mainwidget)) 1)
      (if (`UserWidget.IsAnimationPlaying` _mainwidget _slideout)
        (`UserWidget.ReverseAnimation` _mainwidget _slideout)
        (else
          (`UserWidget.PlayAnimation` _mainwidget (`/Game/Blueprints/QuestBP/Blueprints/QuestSystem/Widgets/W_MainWidget.SlideOut` _mainwidget) 0.0 1 (select `bool` (`/Game/Blueprints/QuestBP/Blueprints/QuestSystem/Widgets/W_MainWidget.SlideOut?` _mainwidget) :`false` "Forward" :`true` "Reverse" :!type "EUMGSequencePlayMode Enum") 1.0 false)))
      (bind _output_get (set `/Game/Blueprints/QuestBP/Blueprints/QuestSystem/Widgets/W_MainWidget.SlideOut?` (not (`/Game/Blueprints/QuestBP/Blueprints/QuestSystem/Widgets/W_MainWidget.SlideOut?` _mainwidget)) _mainwidget))
      (`KismetSystemLibrary.PrintString` (select `bool` _output_get :`false` "not out" :`true` "out")))))

(event `Key|J`
  (params (Key :type "Key Structure"))
  (bind _currentquest (`/Game/Blueprints/QuestBP/Blueprints/QuestSystem/Actors/AC_QuestManager.CurrentQuest` (`self.AC_QuestManager`)))
  ;[1 1 1] Debug Complete/fail sub Goal
  (:`Pressed`
    (`/Engine/EditorBlueprintResources/StandardMacros.IsValid` _currentquest
      (:`Is Valid`
        (`/Game/Blueprints/QuestBP/Blueprints/QuestSystem/Actors/QuestActor/BP_MasterQuest.CompleteSubGoal` _currentquest (`/Game/Blueprints/QuestBP/Blueprints/QuestSystem/Actors/QuestActor/BP_MasterQuest.SelectedSubGoalIndex` _currentquest) false)))))

(event `Key|B`
  (params (Key :type "Key Structure"))
  (bind _currentquest (`/Game/Blueprints/QuestBP/Blueprints/QuestSystem/Actors/AC_QuestManager.CurrentQuest` (`self.AC_QuestManager`)))
  ;[1 1 1] Debug Complete/fail sub Goal
  (:`Pressed`
    (`/Engine/EditorBlueprintResources/StandardMacros.IsValid` _currentquest
      (:`Is Valid`
        (`/Game/Blueprints/QuestBP/Blueprints/QuestSystem/Actors/QuestActor/BP_MasterQuest.CompleteSubGoal` _currentquest (`/Game/Blueprints/QuestBP/Blueprints/QuestSystem/Actors/QuestActor/BP_MasterQuest.SelectedSubGoalIndex` _currentquest) true)))))

(event `Key|T`
  (params (Key :type "Key Structure"))
  (bind _currentquest (`/Game/Blueprints/QuestBP/Blueprints/QuestSystem/Actors/AC_QuestManager.CurrentQuest` (`self.AC_QuestManager`)))
  (bind _questwidget (`/Game/Blueprints/QuestBP/Blueprints/QuestSystem/Actors/QuestActor/BP_MasterQuest.QuestWidget` _currentquest))
  (bind _subgoalwidget (`/Game/Blueprints/QuestBP/Blueprints/QuestSystem/Widgets/W_QuestWidget.SubGoalWidget` _questwidget))
  (bind _returnvalue (`KismetArrayLibrary.Array_Find` _subgoalwidget (`/Game/Blueprints/QuestBP/Blueprints/QuestSystem/Widgets/W_QuestWidget.SelectedSubGoal` _questwidget)))
  ;[1 1 1] PressTToSwitchSubGoals
  (:`Pressed`
    (`/Engine/EditorBlueprintResources/StandardMacros.IsValid` _currentquest
      (:`Is Valid`
        (if (> (`KismetArrayLibrary.Array_Length` _subgoalwidget) 1)
          (`/Game/Blueprints/QuestBP/Blueprints/QuestSystem/Widgets/W_QuestWidget.SelectSubGoal` _questwidget (`|GetArrayItem` _subgoalwidget (select `bool` (< _returnvalue (`KismetArrayLibrary.Array_LastIndex` _subgoalwidget)) :`true` (+ _returnvalue 1)))))))))

(event `self.ReceiveAnyDamage`
  (params (Damage :type "Float (single-precision)") (DamageType :type "DamageType Object Reference") (InstigatedBy :type "Controller Object Reference") (DamageCauser :type "Actor Object Reference"))
  (bind _ac_health (`self.AC_Health`))
  (`|ExecutionSequence`
    (:`then_0`
      (`/Game/Blueprints/Gameplay/ActorComponents/All_Characters/AC_Health.Apply Damage Simple` _ac_health Damage)
      (if (<= (`/Game/Blueprints/Gameplay/ActorComponents/All_Characters/AC_Health.Health_Current` _ac_health) 0.0)
        (set `self.InputEnabled?` false)
        (`/Game/Blueprints/Gameplay/ActorComponents/Players/AC_Camera.Reset` (`self.AC_Camera`))
        (`self.K2_TeleportTo` (1490.0 -830.0 112.0) (struct :`Yaw` -180.0))
        (`/Game/Blueprints/Gameplay/ActorComponents/All_Characters/AC_Health.Reset Health` (`self.AC_Health`))
        (bind _returnvalue (`self.PlayAnimMontage` "/Game/Resources/Animations/Animations_Selected/Animations_Phases/LevelStart_Montage1.LevelStart_Montage1"))
        (`KismetSystemLibrary.Delay` _returnvalue)
        (set `self.InputEnabled?` true)))
    (:`then_1`
      (`self.SwitchColor`))))

(event `Interaction`
  ;[1 1 1] Character intraction To Actor
  (`|ExecutionSequence`
    (:`then_0`
      (bind (_returnvalue _hitactor) (`self.Raycast to Camera`))
      (bind _asinteract_actor_bp (cast `/Game/Blueprints/Gameplay/Actors/Interactables/Interact_Actor_BP` _hitactor)
        (:`then`
          (`/Game/Blueprints/Gameplay/Actors/Interactables/Interact_Actor_BP.Interact` _asinteract_actor_bp))
        (:`CastFailed`
          (bind _asnpc_villages (cast `/Game/Blueprints/Gameplay/IntelligenceArticiel/NPC_Dialogue/NPC_Villages` _hitactor))
          (`/Game/Blueprints/Gameplay/IntelligenceArticiel/NPC_Dialogue/NPC_Villages.Interact to Dialog` _asnpc_villages))))
    (:`then_1`
      (for _array_element (`PrimitiveComponent.GetOverlappingActors` (`self.InteractionCapsule`) null)
        (if (`KismetSystemLibrary.DoesImplementInterface` _array_element "/Game/Blueprints/QuestBP/Blueprints/I_Interactable.I_Interactable_C")
          (message `/Game/Blueprints/QuestBP/Blueprints/I_Interactable.OnInteract` _array_element self)
          (break))))))

(event `Show Sword`
  (bind _swordvfx (`self.SwordVFX`))
  ;[1 1 1] Show and Hidden VFX Sword
  (`|ExecutionSequence`
    (:`then_0`
      (`/Engine/EditorBlueprintResources/StandardMacros.DoOnce` false :!label _label
        (:`Completed`
          (`ActorComponent.SetActive` _swordvfx true false)
          (`KismetSystemLibrary.Delay` 4.9)
          (`NiagaraComponent.SetPaused` _swordvfx true))))
    (:`then_1`
      (`KismetSystemLibrary.RetriggerableDelay` 5.0)
      (`NiagaraComponent.SetPaused` _swordvfx false)
      (`ActorComponent.SetActive` (`self.SwordVFX1`) true false)
      (goto _label :!via `Reset`))))

(event `Set Drink Potion`
  (params (NewMesh :type "StaticMesh Object Reference"))
  ;[1 1 1] Show and Hidden potion
  (`StaticMeshComponent.SetStaticMesh` (`self.DrinkPotion`) NewMesh))

(event `Clear Object Hand Left`
  ;[1 1 1] Show and Hidden potion
  (`StaticMeshComponent.SetStaticMesh` (`self.DrinkPotion`) null))

(event `Cancel Animation Beginplay`
  ;[1 1 1] Cancel animation begin play
  (if (not (`self.GameStarted?`))
    (`self.StopAnimMontage` "/Game/Resources/Animations/Animations_Selected/Animations_NPCs/Anim_Body_Stretch_1_Montage.Anim_Body_Stretch_1_Montage")
    (set `self.GameStarted?` true)
    (set `self.InputEnabled?` true)))

(event `Choice animation Begin play`
  ;[1 1 1] Choice animation Begin play
  (if (`self.GameStarted?`)
    (set `self.InputEnabled?` false)
    (bind _returnvalue (`self.PlayAnimMontage` "/Game/Resources/Animations/Animations_Selected/Animations_Phases/LevelStart_Montage1.LevelStart_Montage1"))
    (`KismetSystemLibrary.Delay` _returnvalue)
    (set `self.InputEnabled?` true)
    (else
      (set `self.InputEnabled?` false)
      (bind _returnvalue_2 (`self.PlayAnimMontage` "/Game/Resources/Animations/Animations_Selected/Animations_NPCs/Anim_Body_Stretch_1_Montage.Anim_Body_Stretch_1_Montage"))
      (`KismetSystemLibrary.Delay` _returnvalue_2)
      (set `self.GameStarted?` true)
      (set `self.InputEnabled?` true))))

(event `Check SlowMotion`
  ;[1 1 1] Play Slow motion
  (bind _result (`/Engine/EditorBlueprintResources/StandardMacros.IncrementInt` (`self.MobKill`))
    (:`  `
      (if (>= _result (`KismetMathLibrary.RandomIntegerInRange` 5 8))
        (`GameplayStatics.SetGlobalTimeDilation` 0.3)
        (`KismetSystemLibrary.Delay` 0.15)
        (`GameplayStatics.SetGlobalTimeDilation` 1.0)
        (set `self.MobKill` 0)))))

(event `Use Slot 1`
  ;[1 1 1] Use Slot
  (`/Game/Blueprints/HUD/Player/Shortcut_Player.Use Slot 1` (`/Game/Blueprints/HUD/Player/Interface_Player.Shortcut_Player` (`/Game/Blueprints/Gameplay/PlayerController_Gameplay.InterfacePlayer` (`self.As Player Controller Gameplay`)))))

(event `Use Slot 2`
  ;[1 1 1] Use Slot
  (`/Game/Blueprints/HUD/Player/Shortcut_Player.Use Slot 2` (`/Game/Blueprints/HUD/Player/Interface_Player.Shortcut_Player` (`/Game/Blueprints/Gameplay/PlayerController_Gameplay.InterfacePlayer` (`self.As Player Controller Gameplay`)))))

(event `Use Slot 3`
  ;[1 1 1] Use Slot
  (`/Game/Blueprints/HUD/Player/Shortcut_Player.Use Slot 3` (`/Game/Blueprints/HUD/Player/Interface_Player.Shortcut_Player` (`/Game/Blueprints/Gameplay/PlayerController_Gameplay.InterfacePlayer` (`self.As Player Controller Gameplay`)))))

(event `Use Slot 4`
  ;[1 1 1] Use Slot
  (`/Game/Blueprints/HUD/Player/Shortcut_Player.Use Slot 4` (`/Game/Blueprints/HUD/Player/Interface_Player.Shortcut_Player` (`/Game/Blueprints/Gameplay/PlayerController_Gameplay.InterfacePlayer` (`self.As Player Controller Gameplay`)))))

(fn `AddSoundEnemy`
  (params (A :type "Actor Object Reference"))
  (if (!= A self)
    (bind _ascharacter_gameplay_master_enemy (cast `/Game/Blueprints/Gameplay/IntelligenceArticiel/Master/Character_Gameplay_Master_Enemy` A))
    (`KismetArrayLibrary.Array_Add` (`self.SoundEnemyArray`) _ascharacter_gameplay_master_enemy)))

(fn `CheckCondition`
  (params (Context :type "DlgContext Object Reference") (ConditionName :type Name))
  (returns (ReturnValue :type Boolean))
  (return false))

(fn `CheckDoubleTapInDirection`
  (params (Direction :type String))
  (returns (`DoubleTap?` :type Boolean))
  (switch `string` Direction
    (:`Forward`
      (set `self.Bint` 0)
      (set `self.Rint` 0)
      (set `self.Lint` 0)
      (bind _result (`/Engine/EditorBlueprintResources/StandardMacros.IncrementInt` (`self.Fint`))
        (:`  `
          (if (>= _result 2)
            (set `self.Fint` 0)
            (return true)
            (else
              (return false))))))
    (:`Backward`
      (set `self.Fint` 0)
      (set `self.Rint` 0)
      (set `self.Lint` 0)
      (bind _result_2 (`/Engine/EditorBlueprintResources/StandardMacros.IncrementInt` (`self.Bint`))
        (:`  `
          (if (>= _result_2 2)
            (set `self.Bint` 0)
            (return true)
            (else
              (return false))))))
    (:`Left`
      (set `self.Fint` 0)
      (set `self.Bint` 0)
      (set `self.Rint` 0)
      (bind _result_3 (`/Engine/EditorBlueprintResources/StandardMacros.IncrementInt` (`self.Lint`))
        (:`  `
          (if (>= _result_3 2)
            (set `self.Lint` 0)
            (return true)
            (else
              (return false))))))
    (:`Right`
      (set `self.Lint` 0)
      (set `self.Bint` 0)
      (set `self.Fint` 0)
      (bind _result_4 (`/Engine/EditorBlueprintResources/StandardMacros.IncrementInt` (`self.Rint`))
        (:`  `
          (if (>= _result_4 2)
            (set `self.Rint` 0)
            (return true)
            (else
              (return false))))))))

(fn `GetAttendeeDisplayName`
  (params (ActiveSpeaker :type Name))
  (returns (ReturnValue :type Text))
  (return "Tiava"))

(fn `GetAttendeeGender`
  (returns (ReturnValue :type "ETextGender Enum"))
  (return "Masculine"))

(fn `GetAttendeeIcon`
  (params (ActiveSpeaker :type Name) (ActiveSpeakerState :type Name))
  (returns (ReturnValue :type "Texture2D Object Reference"))
  (return "/Game/Blueprints/HUD/Texture_HUD/Character.Character"))

(fn `GetAttendeeName`
  (returns (ReturnValue :type Name))
  (return "Player"))

(fn `GetBoolValue`
  (params (ValueName :type Name))
  (returns (ReturnValue :type Boolean))
  (return false))

(fn `GetFloatValue`
  (params (ValueName :type Name))
  (returns (ReturnValue :type "Float (double-precision)"))
  (return 0.0))

(fn `GetIntValue`
  (params (ValueName :type Name))
  (returns (ReturnValue :type Integer))
  (return 0))

(fn `GetNameValue`
  (params (ValueName :type Name))
  (returns (ReturnValue :type Name))
  (return "None"))

(fn `Init Player Controller`
  (bind _asplayer_controller_gameplay (cast `/Game/Blueprints/Gameplay/PlayerController_Gameplay` (`GameplayStatics.GetPlayerController` 0)))
  (set `self.As Player Controller Gameplay` _asplayer_controller_gameplay))

(fn `ModifyBoolValue`
  (params (ValueName :type Name) (bNewValue :type Boolean))
  (returns (ReturnValue :type Boolean))
  (return false))

(fn `ModifyFloatValue`
  (params (ValueName :type Name) (bDelta :type Boolean) (Value :type "Float (double-precision)"))
  (returns (ReturnValue :type Boolean))
  (return false))

(fn `ModifyIntValue`
  (params (ValueName :type Name) (bDelta :type Boolean) (Value :type Integer))
  (returns (ReturnValue :type Boolean))
  (return false))

(fn `ModifyNameValue`
  (params (ValueName :type Name) (NameValue :type Name))
  (returns (ReturnValue :type Boolean))
  (return false))

(fn `OnDialogueEvent`
  (params (Context :type "DlgContext Object Reference") (EventName :type Name))
  (returns (ReturnValue :type Boolean))
  (return false))

(fn `Raycast to Camera`
  (returns (ReturnValue :type Boolean) (HitActor :type "Actor Object Reference") (Location :type "Vector Structure"))
  (bind _camera (`self.Camera`))
  (bind _returnvalue (`SceneComponent.K2_GetComponentLocation` _camera))
  (bind (_outhit _returnvalue_2) (`KismetSystemLibrary.LineTraceSingleForObjects` _returnvalue (+ (* (`SceneComponent.GetForwardVector` _camera) 2000.0) _returnvalue) (`|MakeArray` "ObjectTypeQuery2" "ObjectTypeQuery1" "ObjectTypeQuery3" "ObjectTypeQuery6" :!type "EObjectTypeQuery Enum")))
  (bind (_bblockinghit _binitialoverlap _time _distance _location _impactpoint _normal _impactnormal _physmat _hitactor) (`GameplayStatics.BreakHitResult` _outhit))
  (return _returnvalue_2 _hitactor _location))

(fn `RemoveSoundEnemy`
  (params (B :type "Actor Object Reference"))
  (if (!= self B)
    (bind _ascharacter_gameplay_master_enemy (cast `/Game/Blueprints/Gameplay/IntelligenceArticiel/Master/Character_Gameplay_Master_Enemy` B))
    (`KismetArrayLibrary.Array_RemoveItem` (`self.SoundEnemyArray`) _ascharacter_gameplay_master_enemy)))

(fn `UpdateVFX_SwitchElement`
  (bind _vfx_switch_element (`self.VFX_Switch_Element`))
  (`ActorComponent.SetActive` _vfx_switch_element true false)
  (`NiagaraComponent.SetAsset` _vfx_switch_element "/Game/Particles/Systems/Systems_SwitchElements/VFX_SwtichElement.VFX_SwtichElement")
  (`NiagaraComponent.SetVariableLinearColor` _vfx_switch_element "Color_Elements" (`self.In Value`))
  (`NiagaraComponent.ResetSystem` _vfx_switch_element)
  (`self.PlayAnimMontage` "/Game/Resources/Animations/Animations_Selected/Animations_Magic/MG_Buff_Montage.MG_Buff_Montage")
  (`KismetSystemLibrary.PrintString` "Switch Elements" true false (struct :`R` 0.075611 :`G` 1.0 :`A` 1.0) 1.0))

(fn `UserConstructionScript`
  (`SphereComponent.SetSphereRadius` (`self.Detection_Sound`) (`self.SoundDetectionValue`) true))