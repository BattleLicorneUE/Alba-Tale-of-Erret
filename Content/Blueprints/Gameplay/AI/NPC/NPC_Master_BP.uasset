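; Base NPC actor that shows a dialogue widget to a gameplay character inside its detection area.
; Overlap stores the character, fills the widget with name and current line from StructNPC, then shows it; leaving hides it and resets the index.
; InteracttoNPC cycles through the lines, wrapping to the first, while a target is valid.
; A look-at-player function and saved starting rotation exist but are unused in this graph.
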(event `self.ReceiveBeginPlay`
  (set `self.Rotation Origin` (`self.K2_GetActorRotation`)))

(event `Interact to NPC`
  (`/Engine/EditorBlueprintResources/StandardMacros.IsValid` (`self.Target To Interact`)
    (:`Is Valid`
      (`self.Check Last Index Dialogue`)
      (`self.Update Dialogue`))))

(event `self.Detection_PlayerCharacters.OnComponentBeginOverlap`
  (params (OverlappedComponent :type "PrimitiveComponent Object Reference") (OtherActor :type "Actor Object Reference") (OtherComp :type "PrimitiveComponent Object Reference") (OtherBodyIndex :type Integer) (bFromSweep :type Boolean) (SweepResult :type "HitResult Structure (by ref)"))
  (bind _ascharacter_gameplay (cast `/Game/Blueprints/Gameplay/Character_Gameplay` OtherActor))
  (set `self.Target To Interact` _ascharacter_gameplay)
  (`self.Update Dialogue`)
  (`self.Display Dialogue Screen`))

(event `self.Detection_PlayerCharacters.OnComponentEndOverlap`
  (params (OverlappedComponent :type "PrimitiveComponent Object Reference") (OtherActor :type "Actor Object Reference") (OtherComp :type "PrimitiveComponent Object Reference") (OtherBodyIndex :type Integer))
  (cast `/Game/Blueprints/Gameplay/Character_Gameplay` OtherActor)
  (set `self.Target To Interact` null)
  (`self.Hidden Dialogue Screen`)
  (`self.Reset Dialogue`))

(fn `Cast to Widgets Interact`
  (returns (`AsWidgets Interact NPC` :type "/Game/Blueprints/Gameplay/AI/NPC/Widgets_Interact_NPC Object Reference"))
  (bind _aswidgets_interact_npc (cast `/Game/Blueprints/Gameplay/AI/NPC/Widgets_Interact_NPC` (`WidgetComponent.GetUserWidgetObject` (`self.Widget`))))
  (return _aswidgets_interact_npc))

(fn `Check Last Index Dialogue`
  (if (== (`self.Index Dialogue`) (`KismetArrayLibrary.Array_LastIndex` (`.SetTextDialogue_10_83967C1848DF33A8517203B15E604737` (break `/Game/Blueprints/Gameplay/AI/NPC/S_NPC` (`self.Struct NPC`)))))
    (set `self.Index Dialogue` 0)
    (else
      (`/Engine/EditorBlueprintResources/StandardMacros.IncrementInt` (`self.Index Dialogue`)))))

(fn `Display Dialogue Screen`
  (`SceneComponent.SetVisibility` (`self.Widget`) true false))

(fn `Hidden Dialogue Screen`
  (`SceneComponent.SetVisibility` (`self.Widget`) false false))

(fn `LookAt To Player`
  (`self.K2_SetActorRotation` (`KismetMathLibrary.FindLookAtRotation` (`self.K2_GetActorLocation`) (`self.K2_GetActorLocation` (`GameplayStatics.GetPlayerCharacter` 0)))))

(fn `Reset Dialogue`
  (set `self.Index Dialogue` 0))

(fn `Update Dialogue`
  (bind (_namenpc _staticorpatrol _settextdialogue) (break `/Game/Blueprints/Gameplay/AI/NPC/S_NPC` (`self.Struct NPC`)))
  (bind _aswidgets_interact_npc (`self.Cast to Widgets Interact`))
  (set `/Game/Blueprints/Gameplay/AI/NPC/Widgets_Interact_NPC.Name` (`KismetTextLibrary.Conv_NameToText` _namenpc) _aswidgets_interact_npc)
  (set `/Game/Blueprints/Gameplay/AI/NPC/Widgets_Interact_NPC.Dialogue` (`|GetArrayItem` _settextdialogue (`self.Index Dialogue`)) _aswidgets_interact_npc))

(fn `UserConstructionScript`)