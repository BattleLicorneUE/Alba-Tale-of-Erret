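; Actor component for AI mobs that computes outgoing damage and defensive damage reduction from damage and defense stat structs.
; ApplyDamage rolls a critical chance, then deals random damage within the min-max range to the target, multiplied by the critical factor on a crit.
; ReductionDamage is a separate function that returns incoming damage lowered by the base defense percentage.
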(event `Apply Damage`
  (params (DamagedActor :type "Actor Object Reference"))
  (bind (_damagemin _damagemax _chancecritik _coupcritik) (break `/Game/Blueprints/Gameplay/AI/S_Attack_Mob` (`self.S_Stats Damage`)))
  (bind _returnvalue (`KismetMathLibrary.RandomFloatInRange` _damagemin _damagemax))
  (if (<= (`KismetMathLibrary.RandomFloat`) (/ _chancecritik 100.0))
    (`GameplayStatics.ApplyDamage` DamagedActor (* _returnvalue _coupcritik))
    (else
      (`GameplayStatics.ApplyDamage` DamagedActor _returnvalue))))

(fn `Reduction Damage`
  (params (Damage :type "Float (double-precision)"))
  (returns (`Damage Before Reduction` :type "Float (double-precision)"))
  (return (- Damage (* Damage (/ (`.Defensebase_19_0831040944DA062C0297638B4A45CAF9` (break `/Game/Blueprints/Gameplay/AI/S_Defense_Mob` (`self.S_Stats Defense`))) 100.0)))))