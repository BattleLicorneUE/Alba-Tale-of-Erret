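; Master character Blueprint that maps player inputs to attacks handled by separate melee, zone and distance components.
; NormalAttack triggers the melee attack after caching the actor's location and rotation, while Skill_1 fires the zone attack.
; Skill_3 fires the distance attack, and a hardcoded E key starts a ray attack on the distance component on press and ends it on release.
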(event `InputAction|NormalAttack`
  (params (Key :type "Key Structure"))
  (:`Pressed`
    (set `self.C_Location` (`self.K2_GetActorLocation` self))
    (set `self.C_Rotation` (`self.K2_GetActorRotation` self))
    (`/Game/Blueprints/Gameplay/ActorComponents/AC_Melee.Attack` (`self.AC_Melee`))))

(event `InputAction|Skill_1`
  (params (Key :type "Key Structure"))
  (:`Pressed`
    (`/Game/Blueprints/Gameplay/ActorComponents/AC_Zone.Attack` (`self.AC_Zone`))))

(event `InputAction|Skill_3`
  (params (Key :type "Key Structure"))
  (:`Pressed`
    (`/Game/Blueprints/Gameplay/ActorComponents/AC_Distance.DistanceAttack` (`self.AC_Distance`))))

(event `Key|E`
  (params (Key :type "Key Structure"))
  (bind _ac_distance (`self.AC_Distance`))
  (:`Pressed`
    (`/Game/Blueprints/Gameplay/ActorComponents/AC_Distance.StartRayAttack` _ac_distance))
  (:`Released`
    (`/Game/Blueprints/Gameplay/ActorComponents/AC_Distance.EndRayAttack` _ac_distance)))

(fn `UserConstructionScript`)