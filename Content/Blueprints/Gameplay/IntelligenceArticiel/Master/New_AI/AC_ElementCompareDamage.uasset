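; Actor component that provides elemental damage helpers for enemy AI.
; CompareElementDamage casts a damage object to DamageType_Master and has the player character's CompareElements check its element against the enemy structure's element.
; CalculeReductionDamage takes a boolean condition, dividing initial damage by the enemy's SystemDefense resistance when true and doubling it when false.
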(fn `Calcule Reduction Damage`
  (params (`Damage Init` :type "Float (double-precision)") (Condition :type Boolean) (Structure_Enemy_AI :type "/Game/Blueprints/Gameplay/IntelligenceArticiel/StructureAI/Structure_Enemy_AI Structure (by ref)"))
  (returns (`New Damage` :type "Float (double-precision)"))
  (if Condition
    (return (/ `Damage Init` (`KismetMathLibrary.Conv_IntToDouble` (`.Resistance_60_FCF7D810435489E431CF85B6D95054FD` (break `/Game/Blueprints/Gameplay/IntelligenceArticiel/StructureAI/Structure_Enemy_Defense` (`.SystemDefense_50_4E1F7EFB4745E6C4212E649AB4A9E771` (break `/Game/Blueprints/Gameplay/IntelligenceArticiel/StructureAI/Structure_Enemy_AI` Structure_Enemy_AI)))))))
    (else
      (return (* `Damage Init` 2.0)))))

(fn `Compare Element Damage`
  (params (Object :type "Object Object Reference") (Structure_Enemy_AI :type "/Game/Blueprints/Gameplay/IntelligenceArticiel/StructureAI/Structure_Enemy_AI Structure (by ref)"))
  (returns (`Resist?` :type Boolean))
  (bind _asdamage_type_master (cast `/Game/Blueprints/Gameplay/Datas/DamageTypes/DamageType_Master` Object :!pure true))
  (`/Engine/EditorBlueprintResources/StandardMacros.IsValid` _asdamage_type_master
    (:`Is Valid`
      (bind _resist_ (`/Game/Blueprints/Gameplay/Character_Gameplay.CompareElements` (`/Game/Blueprints/Gameplay/Library_Blueprints/FunctionLibrary.Get Player character`) (`/Game/Blueprints/Gameplay/Datas/DamageTypes/DamageType_Master.Element` _asdamage_type_master) (`.Element_71_B5E3B1604135E1D4D2FD6B99507A3EB4` (break `/Game/Blueprints/Gameplay/IntelligenceArticiel/StructureAI/Structure_Enemy_AI` Structure_Enemy_AI))))
      (return _resist_))))