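; BP_Quest_03 defines the forest quest "La forêt", an ordered chain of reach-location objectives that takes the player from catching up with a man to waiting for the village chief's return.
; It constructs an order-required root objective collection and fills it with four BP_objReachLocation objectives, each tied to its own destination.
; The final objective's completion event is bound, and the QuestEnd function opens Level_Arene.
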(fn `ConstructRootObjectiveCollection`
  (returns (RootObjCollection :type "/Game/Blueprints/Gameplay/QuestSystem/Objectives/BP_objCollection Object Reference"))
  (bind _returnvalue (`|GenericCreateObject` "/Game/Blueprints/Gameplay/QuestSystem/Objectives/BP_objCollection.BP_objCollection_C" self true "La forêt"))
  (return _returnvalue))

(fn `PopulateObjectives`
  (params (RootObjCollection :type "/Game/Blueprints/Gameplay/QuestSystem/Objectives/BP_objCollection Object Reference"))
  (bind _returnvalue (`|GenericCreateObject` "/Game/Blueprints/Gameplay/QuestSystem/Objectives/BP_objReachLocation.BP_objReachLocation_C" self (`self.DestinationHomme`) "Rattraper l'homme"))
  (`/Game/Blueprints/Gameplay/QuestSystem/Objectives/BP_objCollection.AddObjective` RootObjCollection _returnvalue)
  (bind _returnvalue_2 (`|GenericCreateObject` "/Game/Blueprints/Gameplay/QuestSystem/Objectives/BP_objReachLocation.BP_objReachLocation_C" self (`self.DestinationVista`) "Voir la vista"))
  (`/Game/Blueprints/Gameplay/QuestSystem/Objectives/BP_objCollection.AddObjective` RootObjCollection _returnvalue_2)
  (bind _returnvalue_3 (`|GenericCreateObject` "/Game/Blueprints/Gameplay/QuestSystem/Objectives/BP_objReachLocation.BP_objReachLocation_C" self (`self.DestinationVillage`) "Aller au village"))
  (`/Game/Blueprints/Gameplay/QuestSystem/Objectives/BP_objCollection.AddObjective` RootObjCollection _returnvalue_3)
  (bind _returnvalue_4 (`|GenericCreateObject` "/Game/Blueprints/Gameplay/QuestSystem/Objectives/BP_objReachLocation.BP_objReachLocation_C" self (`self.DestinationChef`) "Attendre le retour du chef"))
  (add `/Game/Blueprints/Gameplay/QuestSystem/Objectives/BP_Objective.OnCompleted` _returnvalue_4 (`|CreateDelegate` :!event `QuestEnd`))
  (`/Game/Blueprints/Gameplay/QuestSystem/Objectives/BP_objCollection.AddObjective` RootObjCollection _returnvalue_4))

(fn `QuestEnd`
  (params (Objective :type "/Game/Blueprints/Gameplay/QuestSystem/Objectives/BP_Objective Object Reference"))
  (`GameplayStatics.OpenLevel` "Level_Arene"))

(fn `UserConstructionScript`
  (`parent.UserConstructionScript`))