(fn `ConstructRootObjectiveCollection`
  (returns (RootObjCollection :type "/Game/Blueprints/Gameplay/QuestSystem/Objectives/BP_objCollection Object Reference"))
  (bind _returnvalue (`|GenericCreateObject` "/Game/Blueprints/Gameplay/QuestSystem/Objectives/BP_objCollection.BP_objCollection_C" self true "Niveau 1 : Terre"))
  (return _returnvalue))

(fn `PopulateObjectives`
  (params (RootObjCollection :type "/Game/Blueprints/Gameplay/QuestSystem/Objectives/BP_objCollection Object Reference"))
  (locals (ObjectifRanger :type "/Game/Blueprints/Gameplay/QuestSystem/Objectives/BP_objCollection Object Reference"))
  (bind _bag_object (`self.Bag object`))
  (`|ExecutionSequence`
    (:`then_0`
      (bind _returnvalue (`|GenericCreateObject` "/Game/Blueprints/Gameplay/QuestSystem/Objectives/BP_objCollection.BP_objCollection_C" self true "Range ta chambre"))
      (bind _output_get (set `local.ObjectifRanger` _returnvalue))
      (`/Game/Blueprints/Gameplay/QuestSystem/Objectives/BP_objCollection.AddObjective` (`local.RootObjCollection`) _output_get))
    (:`then_1`
      (bind _returnvalue_2 (`|GenericCreateObject` "/Game/Blueprints/Gameplay/QuestSystem/Objectives/BP_objInteract.BP_objInteract_C" self _bag_object (`/Game/Blueprints/Gameplay/Actors/Interactables/BP_Interactable.ObjectiveText` _bag_object)))
      (`/Game/Blueprints/Gameplay/QuestSystem/Objectives/BP_objCollection.AddObjective` (`local.ObjectifRanger`) _returnvalue_2)
      (bind _returnvalue_3 (`|GenericCreateObject` "/Game/Blueprints/Gameplay/QuestSystem/Objectives/BP_objReachLocation.BP_objReachLocation_C" self (`self.Door Trigger`) "Ouvre a ton jumeau"))
      (`/Game/Blueprints/Gameplay/QuestSystem/Objectives/BP_objCollection.AddObjective` (`local.ObjectifRanger`) _returnvalue_3))))

(fn `UserConstructionScript`
  (`parent.UserConstructionScript`))