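; BP_Quest_02 defines the "L'école" (school) quest in the quest system, with objectives to rejoin friends and survive a fight.
; It builds an order-required root objective collection and fills it with two reach-location objectives, so even the combat step completes by reaching a destination.
; The second objective binds a completion event, and the FinDuCombat handler prints a sky-glow message and opens the Village_Hannathan_P level.
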(fn `ConstructRootObjectiveCollection`
  (returns (RootObjCollection :type "/Game/Blueprints/Gameplay/QuestSystem/Objectives/BP_objCollection Object Reference"))
  (bind _returnvalue (`|GenericCreateObject` "/Game/Blueprints/Gameplay/QuestSystem/Objectives/BP_objCollection.BP_objCollection_C" self true "L'école"))
  (return _returnvalue))

(fn `FinDuCombat`
  (params (Objective :type "/Game/Blueprints/Gameplay/QuestSystem/Objectives/BP_Objective Object Reference"))
  (`KismetSystemLibrary.PrintString` "Une immense lueur dans le ciel")
  (`GameplayStatics.OpenLevel` "Village_Hannathan_P"))

(fn `PopulateObjectives`
  (params (RootObjCollection :type "/Game/Blueprints/Gameplay/QuestSystem/Objectives/BP_objCollection Object Reference"))
  (bind _returnvalue (`|GenericCreateObject` "/Game/Blueprints/Gameplay/QuestSystem/Objectives/BP_objReachLocation.BP_objReachLocation_C" self (`self.Destination01`) "Rejoins tes amis"))
  (`/Game/Blueprints/Gameplay/QuestSystem/Objectives/BP_objCollection.AddObjective` RootObjCollection _returnvalue)
  (bind _returnvalue_2 (`|GenericCreateObject` "/Game/Blueprints/Gameplay/QuestSystem/Objectives/BP_objReachLocation.BP_objReachLocation_C" self (`self.Destination02`) "Survis au combat"))
  (add `/Game/Blueprints/Gameplay/QuestSystem/Objectives/BP_Objective.OnCompleted` _returnvalue_2 (`|CreateDelegate` :!event `FinDuCombat`))
  (`/Game/Blueprints/Gameplay/QuestSystem/Objectives/BP_objCollection.AddObjective` RootObjCollection _returnvalue_2))

(fn `UserConstructionScript`
  (`parent.UserConstructionScript`))