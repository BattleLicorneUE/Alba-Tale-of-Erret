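; Quest objective Blueprint that completes when the player interacts with a designated InteractObject.
; On activation it runs the parent logic and binds to the object's interact event.
; The first interaction unbinds the listener and fires the completion callback with itself.
; Completion checks read the object's HasInteract state directly rather than storing a separate flag.
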(event `self.ActivateObjective`
  (`parent.ActivateObjective`)
  (add `/Game/Blueprints/Gameplay/Actors/Interactables/BP_Interactable.EventInteract` (`self.InteractObject`) (delegate `Interact`)))

(event `Interact`
  (remove `/Game/Blueprints/Gameplay/Actors/Interactables/BP_Interactable.EventInteract` (`self.InteractObject`) (delegate `Interact`))
  (`self.OnCompleted` self))

(fn `GetIsComplete`
  (returns (IsComplete :type Boolean))
  (return (`/Game/Blueprints/Gameplay/Actors/Interactables/BP_Interactable.HasInteract?` (`self.InteractObject`))))