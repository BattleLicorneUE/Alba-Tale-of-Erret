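; SerializeDlg_BP is a save-game folder Blueprint with stubbed dialogue participant functions and a DialogHistory variable, apparently intended for serializing dialogue history.
; Every condition, value, attendee and event function returns a fixed default or empty result, with no real logic.
; The only EventGraph logic copies GetDialogueHistory into DialogHistory, but it never runs because no event triggers it.
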(fn `CheckCondition`
  (params (Context :type "DlgContext Object Reference") (ConditionName :type Name))
  (returns (ReturnValue :type Boolean))
  (return false))

(fn `GetAttendeeDisplayName`
  (params (ActiveSpeaker :type Name))
  (returns (ReturnValue :type Text))
  (return ""))

(fn `GetAttendeeGender`
  (returns (ReturnValue :type "ETextGender Enum"))
  (return "Masculine"))

(fn `GetAttendeeIcon`
  (params (ActiveSpeaker :type Name) (ActiveSpeakerState :type Name))
  (returns (ReturnValue :type "Texture2D Object Reference"))
  (return null))

(fn `GetAttendeeName`
  (returns (ReturnValue :type Name))
  (return "None"))

(fn `GetBoolValue`
  (params (ValueName :type Name))
  (returns (ReturnValue :type Boolean))
  (return false))

(fn `GetFloatValue`
  (params (ValueName :type Name))
  (returns (ReturnValue :type "Float (double-precision)"))
  (return 0.0))

(fn `GetIntValue`
  (params (ValueName :type Name))
  (returns (ReturnValue :type Integer))
  (return 0))

(fn `GetNameValue`
  (params (ValueName :type Name))
  (returns (ReturnValue :type Name))
  (return "None"))

(fn `ModifyBoolValue`
  (params (ValueName :type Name) (bNewValue :type Boolean))
  (returns (ReturnValue :type Boolean))
  (return false))

(fn `ModifyFloatValue`
  (params (ValueName :type Name) (bDelta :type Boolean) (Value :type "Float (double-precision)"))
  (returns (ReturnValue :type Boolean))
  (return false))

(fn `ModifyIntValue`
  (params (ValueName :type Name) (bDelta :type Boolean) (Value :type Integer))
  (returns (ReturnValue :type Boolean))
  (return false))

(fn `ModifyNameValue`
  (params (ValueName :type Name) (NameValue :type Name))
  (returns (ReturnValue :type Boolean))
  (return false))

(fn `OnDialogueEvent`
  (params (Context :type "DlgContext Object Reference") (EventName :type Name))
  (returns (ReturnValue :type Boolean))
  (return false))