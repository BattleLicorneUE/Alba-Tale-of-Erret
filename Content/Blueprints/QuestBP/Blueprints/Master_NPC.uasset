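; Master NPC Blueprint for an interactable character that shows a name prompt and gives the player a quest.
; On BeginPlay it writes its Name into the InteractMessage widget, which is shown or hidden as the player enters or leaves its radius.
; On interact it adds the hard-coded Quest_test_01 to the character's quest manager without directly starting it, unless that quest is already present.
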(event `self.ReceiveBeginPlay`
  (bind _asw_interact_message (cast `/Game/Blueprints/QuestBP/Blueprints/W_InteractMessage` (`WidgetComponent.GetUserWidgetObject` (`self.InteractMessage`))))
  (`TextBlock.SetText` (`/Game/Blueprints/QuestBP/Blueprints/W_InteractMessage.Name` _asw_interact_message) (`self.Name`)))

(event `self.OnEnterPlayerRadius`
  (params (Character :type "/Game/Blueprints/Gameplay/Character_Gameplay Object Reference"))
  (`SceneComponent.SetVisibility` (`self.InteractMessage`) true false))

(event `self.OnLeavePlayerRadius`
  (params (Character :type "/Game/Blueprints/Gameplay/Character_Gameplay Object Reference"))
  (`SceneComponent.SetVisibility` (`self.InteractMessage`) false false))

(event `self.OnInteract`
  (params (Character :type "/Game/Blueprints/Gameplay/Character_Gameplay Object Reference"))
  (bind _ac_questmanager (`/Game/Blueprints/Gameplay/Character_Gameplay.AC_QuestManager` Character))
  (if (not (`KismetArrayLibrary.Array_Contains` (`/Game/Blueprints/QuestBP/Blueprints/QuestSystem/Actors/AC_QuestManager.AllQuestClasses` _ac_questmanager) "/Game/Blueprints/QuestBP/Blueprints/QuestSystem/Actors/QuestActor/Quest_test_01.Quest_test_01_C"))
    (`/Game/Blueprints/QuestBP/Blueprints/QuestSystem/Actors/AC_QuestManager.AddNewQuest` _ac_questmanager "/Game/Blueprints/QuestBP/Blueprints/QuestSystem/Actors/QuestActor/Quest_test_01.Quest_test_01_C" false)))

(fn `UserConstructionScript`)