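; Quest manager component on the player character that tracks active, completed and failed quest actors and drives the quest HUD and journal.
; Gameplay events like kills, pickups, talks and key presses advance matching subgoals, deferring quest-completing ones until iteration ends.
; It spawns a goal marker for the selected subgoal and grants XP and gold on completion.
; LoadQuest rebuilds quests and NPC state from saved character data, then notifies NPCs and objects.
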(event `OnAction`
  (params (NewParam :type "/Game/Blueprints/QuestBP/Blueprints/QuestSystem/Enums/E_ActionTypes Enum" :default "NewEnumerator0"))
  ;[1 1 1] OnAction
  (`KismetArrayLibrary.Array_Clear` (`self.IndicesToCompleteLater`))
  (for _array_element (`self.CurrentQuestActors`)
    (for (_array_element_2 _array_index) (`/Game/Blueprints/QuestBP/Blueprints/QuestSystem/Actors/QuestActor/BP_MasterQuest.CurrentGoals` _array_element)
      (bind (_type _customgoal_ _goaltext _additionnalname _amounttohunt _goalclass _keytopress _actiontodo _goalid _goallocation _updatequestdescription _updateddescription _followingsubgoalindices _failmeansquestfailed_ _completequest_) (break `/Game/Blueprints/QuestBP/Blueprints/QuestSystem/Structures/S_GoalInfo` _array_element_2))
      (if (and (`|EnumEquality` _type "NewEnumerator6") (`|EnumEquality` _actiontodo NewParam))
        (if _completequest_
          (bind _output (`|GetArrayItem` (`/Game/Blueprints/QuestBP/Blueprints/QuestSystem/Actors/QuestActor/BP_MasterQuest.CurrentGoalIndices` _array_element) _array_index))
          (`KismetArrayLibrary.Array_Add` (`self.IndicesToCompleteLater`) (make `/Game/Blueprints/QuestBP/Blueprints/QuestSystem/Structures/s_IndexToComplete` _array_element _output))
          (else
            (`/Game/Blueprints/QuestBP/Blueprints/QuestSystem/Actors/QuestActor/BP_MasterQuest.CompleteSubGoal` _array_element _output false))))))
  (`self.CompleteGoals`))

(event `OnKeyPressed`
  (params (KeyPressed :type "Key Structure" :default "None"))
  ;[1 1 1] OnKeyPressed
  (`KismetArrayLibrary.Array_Clear` (`self.IndicesToCompleteLater`))
  (for _array_element (`self.CurrentQuestActors`)
    (for (_array_element_2 _array_index) (`/Game/Blueprints/QuestBP/Blueprints/QuestSystem/Actors/QuestActor/BP_MasterQuest.CurrentGoals` _array_element)
      (bind (_type _customgoal_ _goaltext _additionnalname _amounttohunt _goalclass _keytopress _actiontodo _goalid _goallocation _updatequestdescription _updateddescription _followingsubgoalindices _failmeansquestfailed_ _completequest_) (break `/Game/Blueprints/QuestBP/Blueprints/QuestSystem/Structures/S_GoalInfo` _array_element_2))
      (if (and (`|EnumEquality` _type "NewEnumerator5") (== _keytopress KeyPressed))
        (if _completequest_
          (bind _output (`|GetArrayItem` (`/Game/Blueprints/QuestBP/Blueprints/QuestSystem/Actors/QuestActor/BP_MasterQuest.CurrentGoalIndices` _array_element) _array_index))
          (`KismetArrayLibrary.Array_Add` (`self.IndicesToCompleteLater`) (make `/Game/Blueprints/QuestBP/Blueprints/QuestSystem/Structures/s_IndexToComplete` _array_element _output))
          (else
            (`/Game/Blueprints/QuestBP/Blueprints/QuestSystem/Actors/QuestActor/BP_MasterQuest.CompleteSubGoal` _array_element _output false))))))
  (`self.CompleteGoals`))

(event `OnGoToReached`
  (params (TriggerActor :type "Actor Object Reference"))
  ;[1 1 1] OnGoToReached
  (`KismetArrayLibrary.Array_Clear` (`self.IndicesToCompleteLater`))
  (for _array_element (`self.CurrentQuestActors`)
    (for (_array_element_2 _array_index) (`/Game/Blueprints/QuestBP/Blueprints/QuestSystem/Actors/QuestActor/BP_MasterQuest.CurrentGoals` _array_element)
      (bind (_type _customgoal_ _goaltext _additionnalname _amounttohunt _goalclass _keytopress _actiontodo _goalid _goallocation _updatequestdescription _updateddescription _followingsubgoalindices _failmeansquestfailed_ _completequest_) (break `/Game/Blueprints/QuestBP/Blueprints/QuestSystem/Structures/S_GoalInfo` _array_element_2))
      (if (and (`|EnumEquality` _type "NewEnumerator4") (== (`.Location_4_4E9D284C4B75330CD687E483CD1A5E50` (break `/Game/Blueprints/QuestBP/Blueprints/QuestSystem/Structures/S_GoalLocation` _goallocation)) (`Actor.K2_GetActorLocation` TriggerActor)))
        (if _completequest_
          (bind _output (`|GetArrayItem` (`/Game/Blueprints/QuestBP/Blueprints/QuestSystem/Actors/QuestActor/BP_MasterQuest.CurrentGoalIndices` _array_element) _array_index))
          (`KismetArrayLibrary.Array_Add` (`self.IndicesToCompleteLater`) (make `/Game/Blueprints/QuestBP/Blueprints/QuestSystem/Structures/s_IndexToComplete` _array_element _output))
          (else
            (`/Game/Blueprints/QuestBP/Blueprints/QuestSystem/Actors/QuestActor/BP_MasterQuest.CompleteSubGoal` _array_element _output false))))))
  (`self.CompleteGoals`))

(event `OnTalkedToNpc`
  (params (`NPC Class` :type "/Game/Blueprints/Gameplay/IntelligenceArticiel/NPC_Dialogue/NPC_Villages Class Reference") (`NPC Id` :type Integer))
  ;[1 1 1] OnTalkToNpc
  (`KismetArrayLibrary.Array_Clear` (`self.IndicesToCompleteLater`))
  (for _array_element (`self.CurrentQuestActors`)
    (for (_array_element_2 _array_index) (`/Game/Blueprints/QuestBP/Blueprints/QuestSystem/Actors/QuestActor/BP_MasterQuest.CurrentGoals` _array_element)
      (bind (_type _customgoal_ _goaltext _additionnalname _amounttohunt _goalclass _keytopress _actiontodo _goalid _goallocation _updatequestdescription _updateddescription _followingsubgoalindices _failmeansquestfailed_ _completequest_) (break `/Game/Blueprints/QuestBP/Blueprints/QuestSystem/Structures/S_GoalInfo` _array_element_2))
      (if (and (`|EnumEquality` _type "NewEnumerator3") (== _goalclass `NPC Class`) (== _goalid `NPC Id`))
        (if _completequest_
          (bind _output (`|GetArrayItem` (`/Game/Blueprints/QuestBP/Blueprints/QuestSystem/Actors/QuestActor/BP_MasterQuest.CurrentGoalIndices` _array_element) _array_index))
          (`KismetArrayLibrary.Array_Add` (`self.IndicesToCompleteLater`) (make `/Game/Blueprints/QuestBP/Blueprints/QuestSystem/Structures/s_IndexToComplete` _array_element _output))
          (else
            (`/Game/Blueprints/QuestBP/Blueprints/QuestSystem/Actors/QuestActor/BP_MasterQuest.CompleteSubGoal` _array_element _output false))))))
  (`self.CompleteGoals`))

(event `OnInteract`
  (params (InteractObject :type "/Game/Blueprints/QuestBP/Blueprints/QuestSystem/Actors/Interactables/BP_Master_InteractActor Class Reference"))
  ;[1 1 1] OnInteract
  (`KismetArrayLibrary.Array_Clear` (`self.IndicesToCompleteLater`))
  (set `self.InteractObject` InteractObject)
  (for _array_element (`self.CurrentQuestActors`)
    (for (_array_element_2 _array_index) (`/Game/Blueprints/QuestBP/Blueprints/QuestSystem/Actors/QuestActor/BP_MasterQuest.CurrentGoals` _array_element)
      (bind (_type _customgoal_ _goaltext _additionnalname _amounttohunt _goalclass _keytopress _actiontodo _goalid _goallocation _updatequestdescription _updateddescription _followingsubgoalindices _failmeansquestfailed_ _completequest_) (break `/Game/Blueprints/QuestBP/Blueprints/QuestSystem/Structures/S_GoalInfo` _array_element_2))
      (if (and (`|EnumEquality` _type "NewEnumerator7") (== _goalclass (`self.InteractObject`)))
        (if _completequest_
          (bind _output (`|GetArrayItem` (`/Game/Blueprints/QuestBP/Blueprints/QuestSystem/Actors/QuestActor/BP_MasterQuest.CurrentGoalIndices` _array_element) _array_index))
          (`KismetArrayLibrary.Array_Add` (`self.IndicesToCompleteLater`) (make `/Game/Blueprints/QuestBP/Blueprints/QuestSystem/Structures/s_IndexToComplete` _array_element _output))
          (else
            (`/Game/Blueprints/QuestBP/Blueprints/QuestSystem/Actors/QuestActor/BP_MasterQuest.CompleteSubGoal` _array_element _output false))))))
  (`self.CompleteGoals`))

(event `CheckObtainedObjects`
  (bind _currentsubgoal (`self.currentSubGoal`))
  (bind _currentquest (`self.CurrentQuest`))
  (for _array_element (`/Game/Blueprints/Gameplay/Character_Gameplay.ObtainedObjects` (`/Game/Blueprints/Gameplay/Library_Blueprints/FunctionLibrary.Get Player character`))
    (if (== (`.GoalClass_30_FDB48288437F2E4A20AE20930E5D650E` (break `/Game/Blueprints/QuestBP/Blueprints/QuestSystem/Structures/S_GoalInfo` _currentsubgoal)) _array_element)
      (`/Game/Blueprints/QuestBP/Blueprints/QuestSystem/Actors/QuestActor/BP_MasterQuest.PlayQuestEvent` _currentquest (`KismetArrayLibrary.Array_Find` (`.SubGoals_24_6AFC3586495CE67033B84C93ADD70970` (break `/Game/Blueprints/QuestBP/Blueprints/QuestSystem/Structures/S_QuestInfo` (`/Game/Blueprints/QuestBP/Blueprints/QuestSystem/Actors/QuestActor/BP_MasterQuest.QuestInfo` _currentquest))) _currentsubgoal) false))))

(event `OnObjectFound`
  (params (FoundObject :type "/Game/Blueprints/QuestBP/Blueprints/QuestSystem/Actors/Objects/Master_Object Class Reference"))
  ;[1 1 1] OnObjectFound
  (`KismetArrayLibrary.Array_Clear` (`self.IndicesToCompleteLater`))
  (set `self.Found Object` FoundObject)
  (for _array_element (`self.CurrentQuestActors`)
    (for (_array_element_2 _array_index) (`/Game/Blueprints/QuestBP/Blueprints/QuestSystem/Actors/QuestActor/BP_MasterQuest.CurrentGoals` _array_element)
      (bind (_type _customgoal_ _goaltext _additionnalname _amounttohunt _goalclass _keytopress _actiontodo _goalid _goallocation _updatequestdescription _updateddescription _followingsubgoalindices _failmeansquestfailed_ _completequest_) (break `/Game/Blueprints/QuestBP/Blueprints/QuestSystem/Structures/S_GoalInfo` _array_element_2))
      (if (and (`|EnumEquality` _type "NewEnumerator2") (== _goalclass (`self.Found Object`)))
        (bind _returnvalue (+ (`|GetArrayItem` (`/Game/Blueprints/QuestBP/Blueprints/QuestSystem/Actors/QuestActor/BP_MasterQuest.CurrentHuntedAmounts` _array_element) _array_index) 1))
        (if (>= _returnvalue _amounttohunt)
          (if _completequest_
            (bind _output (`|GetArrayItem` (`/Game/Blueprints/QuestBP/Blueprints/QuestSystem/Actors/QuestActor/BP_MasterQuest.CurrentGoalIndices` _array_element) _array_index))
            (`KismetArrayLibrary.Array_Add` (`self.IndicesToCompleteLater`) (make `/Game/Blueprints/QuestBP/Blueprints/QuestSystem/Structures/s_IndexToComplete` _array_element _output))
            (else
              (`/Game/Blueprints/QuestBP/Blueprints/QuestSystem/Actors/QuestActor/BP_MasterQuest.CompleteSubGoal` _array_element _output false)))
          (else
            (`KismetArrayLibrary.Array_Set` (`/Game/Blueprints/QuestBP/Blueprints/QuestSystem/Actors/QuestActor/BP_MasterQuest.CurrentHuntedAmounts` _array_element) _array_index _returnvalue)
            (`/Game/Blueprints/QuestBP/Blueprints/QuestSystem/Widgets/W_SubGoalWidget.Update` (`|GetArrayItem` (`/Game/Blueprints/QuestBP/Blueprints/QuestSystem/Widgets/W_QuestWidget.SubGoalWidget` (`/Game/Blueprints/QuestBP/Blueprints/QuestSystem/Actors/QuestActor/BP_MasterQuest.QuestWidget` _array_element)) _array_index))
            (if (`/Game/Blueprints/QuestBP/Blueprints/QuestSystem/Actors/QuestActor/BP_MasterQuest.SelectedInJournal?` _array_element)
              (`/Game/Blueprints/QuestBP/Blueprints/QuestSystem/Widgets/W_QuestJounal.GenerateSubGoals` (`/Game/Blueprints/QuestBP/Blueprints/QuestSystem/Widgets/W_MainWidget.Journal` (`self.MainWidget`)))))))))
  (`self.CompleteGoals`))

(event `OnEnemyKilled`
  (params (EnemyClass :type "/Game/Blueprints/Gameplay/IntelligenceArticiel/Master/Character_Gameplay_Master_Enemy Class Reference"))
  ;[1 1 1] OnEnemyKilled (quest update)
  (`KismetArrayLibrary.Array_Clear` (`self.IndicesToCompleteLater`))
  (set `self.KilledEnemy` EnemyClass)
  (for _array_element (`self.CurrentQuestActors`)
    (for (_array_element_2 _array_index) (`/Game/Blueprints/QuestBP/Blueprints/QuestSystem/Actors/QuestActor/BP_MasterQuest.CurrentGoals` _array_element)
      (bind (_type _customgoal_ _goaltext _additionnalname _amounttohunt _goalclass _keytopress _actiontodo _goalid _goallocation _updatequestdescription _updateddescription _followingsubgoalindices _failmeansquestfailed_ _completequest_) (break `/Game/Blueprints/QuestBP/Blueprints/QuestSystem/Structures/S_GoalInfo` _array_element_2))
      (if (and (`|EnumEquality` _type "NewEnumerator1") (== _goalclass (`self.KilledEnemy`)))
        (bind _returnvalue (+ (`|GetArrayItem` (`/Game/Blueprints/QuestBP/Blueprints/QuestSystem/Actors/QuestActor/BP_MasterQuest.CurrentHuntedAmounts` _array_element) _array_index) 1))
        (if (>= _returnvalue _amounttohunt)
          (if _completequest_
            (bind _output (`|GetArrayItem` (`/Game/Blueprints/QuestBP/Blueprints/QuestSystem/Actors/QuestActor/BP_MasterQuest.CurrentGoalIndices` _array_element) _array_index))
            (`KismetArrayLibrary.Array_Add` (`self.IndicesToCompleteLater`) (make `/Game/Blueprints/QuestBP/Blueprints/QuestSystem/Structures/s_IndexToComplete` _array_element _output))
            (else
              (`/Game/Blueprints/QuestBP/Blueprints/QuestSystem/Actors/QuestActor/BP_MasterQuest.CompleteSubGoal` _array_element _output false)))
          (else
            (`KismetArrayLibrary.Array_Set` (`/Game/Blueprints/QuestBP/Blueprints/QuestSystem/Actors/QuestActor/BP_MasterQuest.CurrentHuntedAmounts` _array_element) _array_index _returnvalue)
            (`/Game/Blueprints/QuestBP/Blueprints/QuestSystem/Widgets/W_SubGoalWidget.Update` (`|GetArrayItem` (`/Game/Blueprints/QuestBP/Blueprints/QuestSystem/Widgets/W_QuestWidget.SubGoalWidget` (`/Game/Blueprints/QuestBP/Blueprints/QuestSystem/Actors/QuestActor/BP_MasterQuest.QuestWidget` _array_element)) _array_index))
            (if (`/Game/Blueprints/QuestBP/Blueprints/QuestSystem/Actors/QuestActor/BP_MasterQuest.SelectedInJournal?` _array_element)
              (`/Game/Blueprints/QuestBP/Blueprints/QuestSystem/Widgets/W_QuestJounal.GenerateSubGoals` (`/Game/Blueprints/QuestBP/Blueprints/QuestSystem/Widgets/W_MainWidget.Journal` (`self.MainWidget`)))))))))
  (`self.CompleteGoals`))

(event `self.ReceiveBeginPlay`
  ;[1 1 1] BeginPlay
  (`self.GetAllNpcs`)
  (`self.GetAllObjects`))

(event `StartQuestManager`
  (bind _returnvalue (`|CreateWidget` "/Game/Blueprints/QuestBP/Blueprints/QuestSystem/Widgets/W_MainWidget.W_MainWidget_C" (`GameplayStatics.GetPlayerController` 0) self))
  (bind _output_get (set `self.MainWidget` _returnvalue))
  (`UserWidget.AddToViewport` _output_get 0)
  (set `self.CharRef` (cast `/Game/Blueprints/Gameplay/Character_Gameplay` (`self.GetOwner`) :!pure true))
  (`/Game/Blueprints/QuestBP/Blueprints/QuestSystem/Widgets/W_QuestJounal.Initialize` (`/Game/Blueprints/QuestBP/Blueprints/QuestSystem/Widgets/W_MainWidget.Journal` (`self.MainWidget`)) self))

(event `OnSwitchSubQuest`
  (bind _currentgoalactor (`self.CurrentGoalActor`))
  (bind _currentquest (`self.CurrentQuest`))
  (`/Engine/EditorBlueprintResources/StandardMacros.IsValid` _currentgoalactor
    (:`Is Valid`
      (`Actor.K2_DestroyActor` _currentgoalactor))
    (:`Is Not Valid`
      _))
  (bind _output_get (set `self.currentSubGoal` (`|GetArrayItem` (`.SubGoals_24_6AFC3586495CE67033B84C93ADD70970` (break `/Game/Blueprints/QuestBP/Blueprints/QuestSystem/Structures/S_QuestInfo` (`/Game/Blueprints/QuestBP/Blueprints/QuestSystem/Actors/QuestActor/BP_MasterQuest.QuestInfo` _currentquest))) (`/Game/Blueprints/QuestBP/Blueprints/QuestSystem/Actors/QuestActor/BP_MasterQuest.SelectedSubGoalIndex` _currentquest))))
  (bind (_haslocation_ _location) (break `/Game/Blueprints/QuestBP/Blueprints/QuestSystem/Structures/S_GoalLocation` (`.GoalLocation_16_74DE8E224F2CE570D3A824B60E6FED8E` (break `/Game/Blueprints/QuestBP/Blueprints/QuestSystem/Structures/S_GoalInfo` _output_get))))
  (if _haslocation_
    (bind _returnvalue (`|SpawnActorFromClass` "/Game/Blueprints/QuestBP/Blueprints/QuestSystem/Actors/BP_GoalActor.BP_GoalActor_C" (`KismetMathLibrary.MakeTransform` _location) "AlwaysSpawn" "OverrideRootScale" null null))
    (set `self.CurrentGoalActor` _returnvalue)
    (set `self.Distance` (`self.DistanceToGoal`))
    (else
      (set `self.CurrentGoalActor` null))))

(event `LoadQuest`
  (bind _loadedquest (`self.LoadedQuest`))
  (bind _loadedquest_2 (`self.LoadedQuest`))
  (bind _loadedquest_3 (`self.LoadedQuest`))
  (bind _loadedquest_4 (`self.LoadedQuest`))
  (bind _mainwidget (`self.MainWidget`))
  (bind _charref (`self.CharRef`))
  (bind _currentstate (`/Game/Blueprints/QuestBP/Blueprints/QuestSystem/Actors/QuestActor/BP_MasterQuest.CurrentState` _loadedquest_2))
  (for _array_element (`/Game/Blueprints/Gameplay/Character_Gameplay.LoadedQuest` _charref)
    (bind (_questclass _currentlyactiv_ _currentgoalindices _huntamounts _selectedgoalindex _currentgoals _completedgoals _currentstate_2 _currentdescription) (break `/Game/Blueprints/QuestBP/Blueprints/QuestSystem/Structures/s_SavedQuest` _array_element))
    (`KismetArrayLibrary.Array_Add` (`self.AllQuestClasses`) _questclass)
    (bind _returnvalue (`|SpawnActorFromClass` _questclass (`KismetMathLibrary.MakeTransform` (0.0 0.0 0.0)) "AlwaysSpawn" "OverrideRootScale" null self null))
    (set `self.LoadedQuest` _returnvalue)
    (set `/Game/Blueprints/QuestBP/Blueprints/QuestSystem/Actors/QuestActor/BP_MasterQuest.CurrentGoalIndices` _currentgoalindices _loadedquest)
    (set `/Game/Blueprints/QuestBP/Blueprints/QuestSystem/Actors/QuestActor/BP_MasterQuest.CurrentHuntedAmounts` _huntamounts _loadedquest)
    (set `/Game/Blueprints/QuestBP/Blueprints/QuestSystem/Actors/QuestActor/BP_MasterQuest.SelectedSubGoalIndex` _selectedgoalindex _loadedquest)
    (set `/Game/Blueprints/QuestBP/Blueprints/QuestSystem/Actors/QuestActor/BP_MasterQuest.CurrentGoals` _currentgoals _loadedquest)
    (set `/Game/Blueprints/QuestBP/Blueprints/QuestSystem/Actors/QuestActor/BP_MasterQuest.CompletedSubGoals` _completedgoals _loadedquest)
    (set `/Game/Blueprints/QuestBP/Blueprints/QuestSystem/Actors/QuestActor/BP_MasterQuest.CurrentState` _currentstate_2 _loadedquest)
    (set `/Game/Blueprints/QuestBP/Blueprints/QuestSystem/Actors/QuestActor/BP_MasterQuest.CurrentDescription` _currentdescription _loadedquest)
    (`KismetArrayLibrary.Array_Add` (select `/Game/Blueprints/QuestBP/Blueprints/QuestSystem/Enums/E_QuestStates` _currentstate :`NewEnumerator0` (`self.CurrentQuestActors`) :`NewEnumerator1` (`self.CompletedQuestActors`) :`NewEnumerator2` (`self.FailedQuestActors`)) _loadedquest_2)
    (`/Game/Blueprints/QuestBP/Blueprints/QuestSystem/Widgets/W_QuestJounal.AddEntry` (`/Game/Blueprints/QuestBP/Blueprints/QuestSystem/Widgets/W_MainWidget.Journal` (`self.MainWidget`)) (`self.LoadedQuest`))
    (if (`|EnumEquality` _currentstate "NewEnumerator0")
      (bind _widget (`/Game/Blueprints/QuestBP/Blueprints/QuestSystem/Widgets/W_MainWidget.AddQuestToList` (`self.MainWidget`) _loadedquest_3))
      (bind _output_get (set `/Game/Blueprints/QuestBP/Blueprints/QuestSystem/Actors/QuestActor/BP_MasterQuest.QuestWidget` _widget _loadedquest_3))
      (`/Game/Blueprints/QuestBP/Blueprints/QuestSystem/Widgets/W_QuestWidget.UpdateQuest` _output_get)
      (if _currentlyactiv_
        (`self.SelectNewQuest` _loadedquest_4 (`|GetArrayItem` (`/Game/Blueprints/QuestBP/Blueprints/QuestSystem/Widgets/W_QuestWidget.SubGoalWidget` _widget) (`KismetArrayLibrary.Array_Find` (`/Game/Blueprints/QuestBP/Blueprints/QuestSystem/Actors/QuestActor/BP_MasterQuest.CurrentGoalIndices` _loadedquest_4) (`/Game/Blueprints/QuestBP/Blueprints/QuestSystem/Actors/QuestActor/BP_MasterQuest.SelectedSubGoalIndex` _loadedquest_4))) true)
        (if (`/Game/Blueprints/QuestBP/Blueprints/QuestSystem/Widgets/W_MainWidget.SlideOut?` _mainwidget)
          (`UserWidget.PlayAnimation` _mainwidget (`/Game/Blueprints/QuestBP/Blueprints/QuestSystem/Widgets/W_MainWidget.SlideOut` _mainwidget) 0.0 1 "Reverse" 1.0 false)
          (set `/Game/Blueprints/QuestBP/Blueprints/QuestSystem/Widgets/W_MainWidget.SlideOut?` false _mainwidget)))))
  (for _array_element_2 (`/Game/Blueprints/Gameplay/Character_Gameplay.LoadedNpcs` _charref)
    (bind (_npcclass _location _alreadytalkedto_ _questdone_ _nomoretosay _patrolindex) (break `/Game/Blueprints/QuestBP/Blueprints/QuestSystem/Structures/s_SavedNpc` _array_element_2))
    (bind _returnvalue_2 (`GameplayStatics.GetActorOfClass` _npcclass))
    (`Actor.K2_SetActorLocation` _returnvalue_2 _location false false)
    (set `/Game/Blueprints/Gameplay/IntelligenceArticiel/NPC_Dialogue/NPC_Villages.AlreadyTalkedTo?` _alreadytalkedto_ _returnvalue_2)
    (set `/Game/Blueprints/Gameplay/IntelligenceArticiel/NPC_Dialogue/NPC_Villages.QuestDone?` _questdone_ _returnvalue_2)
    (set `/Game/Blueprints/Gameplay/IntelligenceArticiel/NPC_Dialogue/NPC_Villages.NoMoreToSay?` _nomoretosay _returnvalue_2)
    (set `/Game/Blueprints/Gameplay/IntelligenceArticiel/NPC_Dialogue/NPC_Villages.Index` _patrolindex _returnvalue_2))
  (for _array_element_3 (`self.AllNpcsInWorld`)
    (`/Game/Blueprints/Gameplay/IntelligenceArticiel/NPC_Dialogue/NPC_Villages.OnQuestsLoaded` _array_element_3 self))
  (for _array_element_4 (`self.AllObjectsWorld`)
    (`/Game/Blueprints/QuestBP/Blueprints/QuestSystem/Actors/Objects/Master_Object.OnGameLoaded` _array_element_4 self)))

(fn `AddNewQuest`
  (params (QuestClass :type "/Game/Blueprints/QuestBP/Blueprints/QuestSystem/Actors/QuestActor/BP_MasterQuest Class Reference") (`DirectlyStart?` :type Boolean))
  (returns (Success :type Boolean))
  (locals (LocalClass :type "/Game/Blueprints/QuestBP/Blueprints/QuestSystem/Actors/QuestActor/BP_MasterQuest Class Reference") (LocalStart :type Boolean) (LocalQuestActor :type "/Game/Blueprints/QuestBP/Blueprints/QuestSystem/Actors/QuestActor/BP_MasterQuest Object Reference"))
  (bind _mainwidget (`self.MainWidget`))
  (bind _localquestactor (`local.LocalQuestActor`))
  (bind _localquestactor_2 (`local.LocalQuestActor`))
  (set `local.LocalClass` QuestClass)
  (set `local.LocalStart` `DirectlyStart?`)
  (if (and (`KismetSystemLibrary.IsValidClass` QuestClass) (not (`KismetArrayLibrary.Array_Contains` (`self.AllQuestClasses`) QuestClass)))
    (`KismetArrayLibrary.Array_Add` (`self.AllQuestClasses`) (`local.LocalClass`))
    (bind _returnvalue (`|SpawnActorFromClass` (`local.LocalClass`) (`KismetMathLibrary.MakeTransform` (0.0 0.0 0.0)) "AlwaysSpawn" "OverrideRootScale" null self null))
    (bind _output_get (set `local.LocalQuestActor` _returnvalue))
    (`KismetArrayLibrary.Array_Add` (`self.CurrentQuestActors`) _localquestactor)
    (bind _widget (`/Game/Blueprints/QuestBP/Blueprints/QuestSystem/Widgets/W_MainWidget.AddQuestToList` (`self.MainWidget`) _localquestactor))
    (bind _output_get_2 (set `/Game/Blueprints/QuestBP/Blueprints/QuestSystem/Actors/QuestActor/BP_MasterQuest.QuestWidget` _widget _localquestactor))
    (`/Game/Blueprints/QuestBP/Blueprints/QuestSystem/Actors/QuestActor/BP_MasterQuest.SetupStartingGoals` _output_get)
    (`/Game/Blueprints/QuestBP/Blueprints/QuestSystem/Actors/QuestActor/BP_MasterQuest.SetupStartingGoals` _localquestactor)
    (`/Game/Blueprints/QuestBP/Blueprints/QuestSystem/Widgets/W_QuestWidget.UpdateQuest` _output_get_2)
    (`/Game/Blueprints/QuestBP/Blueprints/QuestSystem/Widgets/W_QuestJounal.AddEntry` (`/Game/Blueprints/QuestBP/Blueprints/QuestSystem/Widgets/W_MainWidget.Journal` (`self.MainWidget`)) (`local.LocalQuestActor`))
    (if true
      (`self.SelectNewQuest` _localquestactor_2 (`|GetArrayItem` (`/Game/Blueprints/QuestBP/Blueprints/QuestSystem/Widgets/W_QuestWidget.SubGoalWidget` (`/Game/Blueprints/QuestBP/Blueprints/QuestSystem/Actors/QuestActor/BP_MasterQuest.QuestWidget` _localquestactor_2)))))
    (if (`/Game/Blueprints/QuestBP/Blueprints/QuestSystem/Widgets/W_MainWidget.SlideOut?` (`self.MainWidget`))
      (`UserWidget.PlayAnimation` _mainwidget (`/Game/Blueprints/QuestBP/Blueprints/QuestSystem/Widgets/W_MainWidget.SlideOut` _mainwidget) 0.0 1 "Reverse" 1.0 false)
      (set `/Game/Blueprints/QuestBP/Blueprints/QuestSystem/Widgets/W_MainWidget.SlideOut?` false _mainwidget)
      (return true)
      (else
        (return true)))
    (else
      (return false))))

(fn `CompleteGoals`
  (for _array_element (`self.IndicesToCompleteLater`)
    (bind (_quest _index) (break `/Game/Blueprints/QuestBP/Blueprints/QuestSystem/Structures/s_IndexToComplete` _array_element))
    (`/Game/Blueprints/QuestBP/Blueprints/QuestSystem/Actors/QuestActor/BP_MasterQuest.CompleteSubGoal` _quest _index false)))

(fn `DistanceToGoal`
  (returns (Distance :type Integer))
  (return (`KismetMathLibrary.Round` (/ (`KismetMathLibrary.VSize` (- (`Actor.K2_GetActorLocation` (cast `/Game/Blueprints/Gameplay/Character_Gameplay` (`GameplayStatics.GetPlayerCharacter` 0) :!pure true)) (`Actor.K2_GetActorLocation` (`self.CurrentGoalActor`)))) 100.0))))

(fn `EndQuest`
  (params (Quest :type "/Game/Blueprints/QuestBP/Blueprints/QuestSystem/Actors/QuestActor/BP_MasterQuest Object Reference"))
  (locals (LocalQuest :type "/Game/Blueprints/QuestBP/Blueprints/QuestSystem/Actors/QuestActor/BP_MasterQuest Object Reference"))
  (bind _currentgoalactor (`self.CurrentGoalActor`))
  (bind _localquest (`local.LocalQuest`))
  (bind _charref (`self.CharRef`))
  (bind _output (`|GetArrayItem` (`self.CurrentQuestActors`)))
  (bind (_experience _prestige _gold) (break `/Game/Blueprints/QuestBP/Blueprints/QuestSystem/Structures/S_QuestReward` (`.CompletionReward_14_313D09584A2E6A68DA6AA3B70C3AD819` (break `/Game/Blueprints/QuestBP/Blueprints/QuestSystem/Structures/S_QuestInfo` (`/Game/Blueprints/QuestBP/Blueprints/QuestSystem/Actors/QuestActor/BP_MasterQuest.QuestInfo` _localquest)))))
  (bind _output_get (set `local.LocalQuest` Quest))
  (`KismetArrayLibrary.Array_RemoveItem` (`self.CurrentQuestActors`) _output_get)
  (`KismetArrayLibrary.Array_Add` (select `/Game/Blueprints/QuestBP/Blueprints/QuestSystem/Enums/E_QuestStates` (`/Game/Blueprints/QuestBP/Blueprints/QuestSystem/Actors/QuestActor/BP_MasterQuest.CurrentState` (`local.LocalQuest`)) :`NewEnumerator0` (`self.CurrentQuestActors`) :`NewEnumerator1` (`self.CompletedQuestActors`) :`NewEnumerator2` (`self.FailedQuestActors`)) (`local.LocalQuest`))
  (`/Game/Blueprints/QuestBP/Blueprints/QuestSystem/Widgets/W_QuestJounal.AddEntry` (`/Game/Blueprints/QuestBP/Blueprints/QuestSystem/Widgets/W_MainWidget.Journal` (`self.MainWidget`)) (`local.LocalQuest`))
  (if (== (`local.LocalQuest`) (`self.CurrentQuest`))
    (set `self.CurrentQuest` null)
    (`/Engine/EditorBlueprintResources/StandardMacros.IsValid` _currentgoalactor
      (:`Is Valid`
        (`Actor.K2_DestroyActor` _currentgoalactor))
      (:`Is Not Valid`
        _))
    (`/Engine/EditorBlueprintResources/StandardMacros.IsValid` _output
      (:`Is Valid`
        (`self.SelectNewQuest` _output (`|GetArrayItem` (`/Game/Blueprints/QuestBP/Blueprints/QuestSystem/Widgets/W_QuestWidget.SubGoalWidget` (`/Game/Blueprints/QuestBP/Blueprints/QuestSystem/Actors/QuestActor/BP_MasterQuest.QuestWidget` _output)))))
      (:`Is Not Valid`
        _)))
  (if (`/Game/Blueprints/QuestBP/Blueprints/QuestSystem/Actors/QuestActor/BP_MasterQuest.SelectedInJournal?` (`local.LocalQuest`))
    (`/Game/Blueprints/QuestBP/Blueprints/QuestSystem/Widgets/W_QuestJounal.OnQuestClicked` (`/Game/Blueprints/QuestBP/Blueprints/QuestSystem/Widgets/W_MainWidget.Journal` (`self.MainWidget`)) null))
  (if (`|EnumEquality` (`/Game/Blueprints/QuestBP/Blueprints/QuestSystem/Actors/QuestActor/BP_MasterQuest.CurrentState` _localquest) "NewEnumerator1")
    (`/Game/Blueprints/Gameplay/ActorComponents/Players/Ac_Leveling.Add Exp` (`/Game/Blueprints/Gameplay/Character_Gameplay.Ac_Leveling` _charref) (`KismetMathLibrary.Conv_IntToDouble` _experience))
    (`/Game/Blueprints/Gameplay/ActorComponents/Players/Ac_ManagerMoney.Add Gold` (`/Game/Blueprints/Gameplay/Character_Gameplay.Ac_ManagerMoney` _charref) _gold)
    (return)
    (else
      (return))))

(fn `GetAllNpcs`
  (bind _outactors (`GameplayStatics.GetAllActorsOfClass` "/Game/Blueprints/Gameplay/IntelligenceArticiel/NPC_Dialogue/NPC_Villages.NPC_Villages_C"))
  (set `self.AllNpcsInWorld` _outactors)
  (return))

(fn `GetAllObjects`
  (bind _outactors (`GameplayStatics.GetAllActorsOfClass` "/Game/Blueprints/QuestBP/Blueprints/QuestSystem/Actors/Objects/Master_Object.Master_Object_C"))
  (set `self.AllObjectsWorld` _outactors)
  (return))

(fn `HasCurrentQuest?`
  (params (QuestClass :type "/Game/Blueprints/QuestBP/Blueprints/QuestSystem/Actors/QuestActor/BP_MasterQuest Class Reference"))
  (returns (`Out?` :type Boolean) (QuestActor :type "/Game/Blueprints/QuestBP/Blueprints/QuestSystem/Actors/QuestActor/BP_MasterQuest Object Reference"))
  (locals (FoundQuest :type "/Game/Blueprints/QuestBP/Blueprints/QuestSystem/Actors/QuestActor/BP_MasterQuest Object Reference"))
  (bind _foundquest (`local.FoundQuest`))
  (for _array_element (`self.CurrentQuestActors`)
    (if (== (`GameplayStatics.GetObjectClass` _array_element) QuestClass)
      (set `local.FoundQuest` _array_element)
      (break)))
  (`/Engine/EditorBlueprintResources/StandardMacros.IsValid` _foundquest
    (:`Is Valid`
      (return true _foundquest))
    (:`Is Not Valid`
      (return false null))))

(fn `SelectNewQuest`
  (params (Quest :type "/Game/Blueprints/QuestBP/Blueprints/QuestSystem/Actors/QuestActor/BP_MasterQuest Object Reference") (SubGoal :type "/Game/Blueprints/QuestBP/Blueprints/QuestSystem/Widgets/W_SubGoalWidget Object Reference") (`Loaded?` :type Boolean))
  (bind _currentquest (`self.CurrentQuest`))
  (bind _questwidget (`/Game/Blueprints/QuestBP/Blueprints/QuestSystem/Actors/QuestActor/BP_MasterQuest.QuestWidget` _currentquest))
  (`/Engine/EditorBlueprintResources/StandardMacros.IsValid` _currentquest
    (:`Is Valid`
      (`Widget.SetIsEnabled` (`/Game/Blueprints/QuestBP/Blueprints/QuestSystem/Widgets/W_QuestWidget.QuestName` _questwidget) false)
      (`/Game/Blueprints/QuestBP/Blueprints/QuestSystem/Widgets/W_QuestWidget.SelectSubGoal` _questwidget null false))
    (:`Is Not Valid`
      _))
  (bind _output_get (set `self.CurrentQuest` Quest))
  (`/Game/Blueprints/QuestBP/Blueprints/QuestSystem/Widgets/W_QuestWidget.OnQuestSelected` (`/Game/Blueprints/QuestBP/Blueprints/QuestSystem/Actors/QuestActor/BP_MasterQuest.QuestWidget` _output_get) SubGoal `Loaded?`)
  (return))