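; BP_Master_InteractActor is the base interactable actor for the quest system, with a name prompt widget.
; On BeginPlay it writes its Name into the W_InteractMessage widget.
; Enter and leave player-radius events show and hide that widget.
; On interaction, it passes its own class to the interacting character's ACQuestManager, so the quest manager identifies interactions by actor class.
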(event `self.ReceiveBeginPlay`
  (bind _asw_interact_message (cast `/Game/Blueprints/QuestBP/Blueprints/W_InteractMessage` (`WidgetComponent.GetUserWidgetObject` (`self.Widget`))))
  (`TextBlock.SetText` (`/Game/Blueprints/QuestBP/Blueprints/W_InteractMessage.Name` _asw_interact_message) (`self.Name`)))

(event `/Game/Blueprints/QuestBP/Blueprints/I_Interactable.OnEnterPlayerRadius`
  (params (Character :type "/Game/Blueprints/Gameplay/Character_Gameplay Object Reference"))
  (`SceneComponent.SetVisibility` (`self.Widget`) true false))

(event `/Game/Blueprints/QuestBP/Blueprints/I_Interactable.OnLeavePlayerRadius`
  (params (Character :type "/Game/Blueprints/Gameplay/Character_Gameplay Object Reference"))
  (`SceneComponent.SetVisibility` (`self.Widget`) false false))

(event `/Game/Blueprints/QuestBP/Blueprints/I_Interactable.OnInteract`
  (params (Character :type "/Game/Blueprints/Gameplay/Character_Gameplay Object Reference"))
  (`/Game/Blueprints/QuestBP/Blueprints/QuestSystem/Actors/AC_QuestManager.OnInteract` (`/Game/Blueprints/Gameplay/Character_Gameplay.AC_QuestManager` Character) (`GameplayStatics.GetObjectClass` self)))

(fn `UserConstructionScript`)